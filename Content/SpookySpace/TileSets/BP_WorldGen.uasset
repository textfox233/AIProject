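; Procedural world generator that assembles a level from tile-set Data Table rooms, using a seeded random stream for most picks.
; It spawns a drop ship and dock, then attaches random rooms at open exits, destroying and retrying overlapping ones.
; Accepted rooms add exits, vents and doors; once the room budget runs out, it places objectives and caps remaining exits.
; A looping watchdog timer reloads the test level if generation is unfinished at 15 seconds.
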(event `Start World Gen Timer`
  (bind _returnvalue (`KismetSystemLibrary.K2_SetTimerDelegate` (delegate `Check Completion`) 0.2 true))
  (set `self.Timer Handle` _returnvalue))

(event `Check Completion`
  (`KismetSystemLibrary.PrintString` "Checking")
  (if (>= (`KismetSystemLibrary.GetGameTimeInSeconds`) 15.0)
    (`KismetSystemLibrary.PrintString` "Restarting")
    (`GameplayStatics.OpenLevel` "L_Mikey_TestLevel")))

(event `self.ReceiveBeginPlay`
  (`self.Set Seed`)
  ;[0 0.05944 1] Sets All Desired Gen Values
  (set `self.Number of Objectives` (`KismetMathLibrary.Clamp` (`self.Number of Objectives`) 1 2))
  (set `self.Room Amount` (`KismetMathLibrary.Clamp` (`self.Room Amount`) 10 50))
  ;[0 0.3969 1] Sets All Asset Data
  (bind _returnvalue (`|GetDataTableRow` (`self.Tile Set`) "1")
    (:`then`
      (bind (_dt_name_cid _dt_name_end _dt_name_o _dt_name_e _replacevent _ventsytle _doorstyle _widedoorstyle) (break `/Game/SpookySpace/TileSets/S_DT_List_Ref` _returnvalue))
      (set `self.Room List` _dt_name_cid)
      (set `self.Close List` _dt_name_end)
      (set `self.Objective List` _dt_name_o)
      (set `self.Dock List` _dt_name_e)
      (set `self.Close Wall Holes` _replacevent)
      (set `self.Vents` _ventsytle)
      (set `self.Doors` _doorstyle)
      (set `self.Wide Door Style` _widedoorstyle)
      (bind _outrownames (`DataTableFunctionLibrary.GetDataTableRowNames` (`self.Room List`)))
      (set `self.Room List Row Names` _outrownames)
      (bind _outrownames_2 (`DataTableFunctionLibrary.GetDataTableRowNames` (`self.Close List`)))
      (set `self.Close List Row Name` _outrownames_2)
      (bind _outrownames_3 (`DataTableFunctionLibrary.GetDataTableRowNames` (`self.Objective List`)))
      (set `self.Objective List Row Name` _outrownames_3)
      (bind _outrownames_4 (`DataTableFunctionLibrary.GetDataTableRowNames` (`self.Dock List`)))
      (set `self.Dock List Row Names` _outrownames_4)
      (`self.Generate_DropShip`)
      (`self.Start World Gen Timer`)
      (`self.Generate_Dock`)
      (`self.Repeat`))))

(event `Repeat`
  (bind _type_of_tile_typeoftiles (break `/Game/SpookySpace/TileSets/S_SpawnIntoList` (`self.Type Of Tile`)))
  (`KismetSystemLibrary.Delay` 0.0)
  (switch `/Game/SpookySpace/TileSets/E_TileSets` (`KismetArrayLibrary.Array_RandomFromStream` _type_of_tile_typeoftiles (`self.Stream`))
    (:`NewEnumerator2`
      (`self.Genereate_Rooms` :!label _label))
    (:`NewEnumerator3`
      (goto _label))
    (:`NewEnumerator4`
      (`self.Generate_Objective`))
    (:`NewEnumerator5`
      (goto _label))))

(event `Set Seed`
  (bind _stream (`self.Stream`))
  (bind _seed (`self.Seed`))
  ;[0 0.1883 1] Optinal Seed Ref or have each Load Random -1 on seed = Random
  (if (== _seed -1)
    (`KismetMathLibrary.SeedRandomStream` _stream)
    (else
      (`KismetMathLibrary.SetRandomStreamSeed` _stream _seed))))

(fn `Close off Open Spaces`
  (bind _stream (`self.Stream`))
  (set `self.DE Complete` true)
  (bind _output_get (set `self.Selected Exit` (`KismetArrayLibrary.Array_RandomFromStream` (`self.Exit List`) _stream)))
  (bind _returnvalue (`|GetDataTableRow` (`self.Close List`) (`KismetArrayLibrary.Array_RandomFromStream` (`self.Close List Row Name`) _stream))
    (:`then`
      (bind _returnvalue_2 (`|SpawnActorFromClass` (`KismetArrayLibrary.Array_RandomFromStream` (`|MakeArray` (`.BP_Room_7_9D01BA1747B9AA39F81C078894BB71C6` (break `/Game/SpookySpace/TileSets/S_Room_Gen_Refs` _returnvalue))) _stream) (`SceneComponent.K2_GetComponentToWorld` _output_get) "AlwaysSpawn" "MultiplyWithRoot" null true null))
      (set `self.Last Room` _returnvalue_2)
      (`self.OverLap Check`))))

(fn `Close off Vent Holes`
  (for _array_element (`self.Vent List`)
    (`|SpawnActorFromClass` (`self.Close Wall Holes`) (`SceneComponent.K2_GetComponentToWorld` _array_element) "AlwaysSpawn" "MultiplyWithRoot" null true null))
  (`KismetArrayLibrary.Array_Clear` (`self.Vent List`)))

(fn `Close off Wide Doors`
  (bind _wide_doors_list (`self.Wide Doors List`))
  (for _array_element _wide_doors_list
    (`|SpawnActorFromClass` (`self.Wide Door Style`) (`SceneComponent.K2_GetComponentToWorld` _array_element) "AlwaysSpawn" "MultiplyWithRoot" null true null))
  (`KismetArrayLibrary.Array_Clear` _wide_doors_list))

(fn `Generate_Dock`
  (bind _exit_list (`self.Exit List`))
  (bind _stream (`self.Stream`))
  (bind _output_get (set `self.Selected Exit` (`KismetArrayLibrary.Array_RandomFromStream` _exit_list _stream)))
  (`KismetArrayLibrary.Array_Clear` _exit_list)
  (bind _returnvalue (`|GetDataTableRow` (`self.Dock List`) (`KismetArrayLibrary.Array_RandomFromStream` (`self.Dock List Row Names`) _stream))
    (:`then`
      (bind _returnvalue_2 (`|SpawnActorFromClass` (`KismetArrayLibrary.Array_RandomFromStream` (`|MakeArray` (`.BP_Room_7_9D01BA1747B9AA39F81C078894BB71C6` (break `/Game/SpookySpace/TileSets/S_Room_Gen_Refs` _returnvalue))) _stream) (`SceneComponent.K2_GetComponentToWorld` _output_get) "AlwaysSpawn" "MultiplyWithRoot" null true null))
      (`KismetArrayLibrary.Array_Append` (`self.Exit List`) (`SceneComponent.GetChildrenComponents` (`/Game/SpookySpace/TileSets/BP_MasterRef.Exit Folder` _returnvalue_2) false))
      (set `self.Type Of Tile` (`/Game/SpookySpace/TileSets/BP_MasterRef.Type to spawn` _returnvalue_2))
      (`KismetArrayLibrary.Array_Append` (`self.Door List`) (`SceneComponent.GetChildrenComponents` (`/Game/SpookySpace/TileSets/BP_MasterRef.Door Folder` _returnvalue_2) false))
      (return))))

(fn `Generate_Doors`
  (returns (ReturnValue :type Boolean))
  (bind _door_list (`self.Door List`))
  (for _array_element _door_list
    (`|SpawnActorFromClass` (`self.Doors`) (`SceneComponent.K2_GetComponentToWorld` _array_element) "AlwaysSpawn" "MultiplyWithRoot" null false null))
  (`KismetArrayLibrary.Array_Clear` _door_list)
  (return (`KismetArrayLibrary.Array_IsEmpty` _door_list)))

(fn `Generate_DropShip`
  (bind _returnvalue (`|SpawnActorFromClass` "/Game/SpookySpace/TileSets/BP_S_DropShip.BP_S_DropShip_C" (`SceneComponent.K2_GetComponentToWorld` (`self.DefaultSceneRoot`)) "AlwaysSpawn" "MultiplyWithRoot" null true null))
  (`KismetArrayLibrary.Array_Append` (`self.Exit List`) (`SceneComponent.GetChildrenComponents` (`/Game/SpookySpace/TileSets/BP_MasterRef.Exit Folder` _returnvalue) false))
  (return))

(fn `Generate_Objective`
  (bind _stream (`self.Stream`))
  (bind _output_get (set `self.Selected Exit` (`KismetArrayLibrary.Array_RandomFromStream` (`self.Exit List`) _stream)))
  (bind _returnvalue (`|GetDataTableRow` (`self.Objective List`) (`KismetArrayLibrary.Array_RandomFromStream` (`self.Objective List Row Name`) _stream))
    (:`then`
      (bind _returnvalue_2 (`|SpawnActorFromClass` (`KismetArrayLibrary.Array_RandomFromStream` (`|MakeArray` (`.BP_Room_7_9D01BA1747B9AA39F81C078894BB71C6` (break `/Game/SpookySpace/TileSets/S_Room_Gen_Refs` _returnvalue))) _stream) (`SceneComponent.K2_GetComponentToWorld` _output_get) "AlwaysSpawn" "MultiplyWithRoot" null true null))
      (bind _output_get_2 (set `self.Last Room` _returnvalue_2))
      (set `self.Type Of Tile` (`/Game/SpookySpace/TileSets/BP_MasterRef.Type to spawn` _output_get_2))
      (`self.OverLap Check`))))

(fn `Generate_Stairs`
  (set `self.Selected Exit` (`KismetArrayLibrary.Array_Random` (`self.Exit List`)))
  (bind _returnvalue (`|GetDataTableRow` (`self.Objective List`) (`KismetArrayLibrary.Array_Random` (`self.Objective List Row Name`)))
    (:`then`
      (bind _returnvalue_2 (`|SpawnActorFromClass` (`KismetArrayLibrary.Array_Random` (`|MakeArray` (`.BP_Room_7_9D01BA1747B9AA39F81C078894BB71C6` (break `/Game/SpookySpace/TileSets/S_Room_Gen_Refs` _returnvalue)))) (`SceneComponent.K2_GetComponentToWorld` (`self.Selected Exit`)) "AlwaysSpawn" "MultiplyWithRoot" null true null))
      (bind _output_get (set `self.Last Room` _returnvalue_2))
      (set `self.Type Of Tile` (`/Game/SpookySpace/TileSets/BP_MasterRef.Type to spawn` _output_get))
      (`self.OverLap Check`))))

(fn `Genereate_Rooms`
  (bind _stream (`self.Stream`))
  (bind _output_get (set `self.Selected Exit` (`KismetArrayLibrary.Array_RandomFromStream` (`self.Exit List`) _stream)))
  (bind _returnvalue (`|GetDataTableRow` (`self.Room List`) (`KismetArrayLibrary.Array_RandomFromStream` (`self.Room List Row Names`) _stream))
    (:`then`
      (bind _returnvalue_2 (`|SpawnActorFromClass` (`KismetArrayLibrary.Array_RandomFromStream` (`|MakeArray` (`.BP_Room_7_9D01BA1747B9AA39F81C078894BB71C6` (break `/Game/SpookySpace/TileSets/S_Room_Gen_Refs` _returnvalue))) _stream) (`SceneComponent.K2_GetComponentToWorld` _output_get) "AlwaysSpawn" "MultiplyWithRoot" null true null))
      (bind _output_get_2 (set `self.Last Room` _returnvalue_2))
      (set `self.Type Of Tile` (`/Game/SpookySpace/TileSets/BP_MasterRef.Type to spawn` _output_get_2))
      (`self.OverLap Check`))))

(fn `OverLap Check`
  (bind _last_room (`self.Last Room`))
  (bind _vent_list (`self.Vent List`))
  (bind _number_of_objectives (`self.Number of Objectives`))
  (bind _wide_doors_list (`self.Wide Doors List`))
  (bind _max_stair_spawns (`self.Max Stair spawns`))
  (bind _last_room_2 (`self.Last Room`))
  ;[1 0 0.01675] OverLapped?
  (for _array_element (`SceneComponent.GetChildrenComponents` (`/Game/SpookySpace/TileSets/BP_MasterRef.Overlap Folder` (`self.Last Room`)) false)
    (bind _asbox_collision (cast `BoxComponent` _array_element))
    (`KismetArrayLibrary.Array_Append` (`self.Overlapped List`) (`PrimitiveComponent.GetOverlappingComponents` _asbox_collision))
    (if (`KismetArrayLibrary.Array_IsNotEmpty` (`self.Overlapped List`))
      (`KismetArrayLibrary.Array_Clear` (`self.Overlapped List`))
      (`self.K2_DestroyActor` (`self.Last Room`) :!label _label)
      (if (`self.DE Complete`)
        (`self.Close off Open Spaces`)
        (elif (`self.Objective Complete`)
          (`self.Generate_Objective`)
          (else
            (`self.Genereate_Rooms`))))
      (else
        (`KismetArrayLibrary.Array_Clear` (`self.Overlapped List`))
        (if (`/Game/SpookySpace/TileSets/BP_MasterRef.isStair?` _last_room)
          (if (> _max_stair_spawns 0)
            (bind _result (`/Engine/EditorBlueprintResources/StandardMacros.DecrementInt` _max_stair_spawns)
              (:`  `
                (set `self.Max Stair spawns` _result)))
            (else
              (goto _label))))
        (switch `/Game/SpookySpace/TileSets/E_TileSets` (`/Game/SpookySpace/TileSets/BP_MasterRef.Type of tile` _last_room)
          (:`NewEnumerator0`
            _)
          (:`NewEnumerator1`
            _)
          (:`NewEnumerator2`
            _)
          (:`NewEnumerator3`
            _)
          (:`NewEnumerator4`
            (if (> _number_of_objectives 0)
              (bind _result_2 (`/Engine/EditorBlueprintResources/StandardMacros.DecrementInt` _number_of_objectives)
                (:`  `
                  (set `self.Number of Objectives` _result_2)
                  (set `self.Objective Complete` false)))
              (else
                (goto _label))))
          (:`NewEnumerator5`
            _))
        (set `self.DE Complete` false)
        (bind _result_3 (`/Engine/EditorBlueprintResources/StandardMacros.DecrementInt` (`self.Room Amount`))
          (:`  `
            (set `self.Room Amount` _result_3)
            ;[0 0.5488 1] Cleanup
            (`KismetArrayLibrary.Array_RemoveItem` (`self.Exit List`) (`self.Selected Exit`))
            (`KismetArrayLibrary.Array_Append` (`self.Exit List`) (`SceneComponent.GetChildrenComponents` (`/Game/SpookySpace/TileSets/BP_MasterRef.Exit Folder` _last_room_2) false))
            (`KismetArrayLibrary.Array_Append` _wide_doors_list (`SceneComponent.GetChildrenComponents` (`/Game/SpookySpace/TileSets/BP_MasterRef.Wide Door Folder` _last_room_2) false))
            (if (not (`KismetArrayLibrary.Array_IsEmpty` _wide_doors_list))
              (`self.Close off Wide Doors`))
            (`KismetArrayLibrary.Array_Append` _vent_list (`SceneComponent.GetChildrenComponents` (`/Game/SpookySpace/TileSets/BP_MasterRef.Vent Folder` _last_room_2) false))
            (if (not (`KismetArrayLibrary.Array_IsEmpty` _vent_list))
              (`self.Spawn Vents`))
            (`KismetArrayLibrary.Array_Append` (`self.Door List`) (`SceneComponent.GetChildrenComponents` (`/Game/SpookySpace/TileSets/BP_MasterRef.Door Folder` _last_room_2) false))
            (if (> (`self.Room Amount`) 0)
              (`self.Repeat`)
              (else
                ;[1 0 0.03719] End World Gen
                (if (`KismetArrayLibrary.Array_IsEmpty` (`self.Exit List`))
                  (bind _returnvalue (`self.Generate_Doors`))
                  (if _returnvalue
                    (set `self.WorldGen Complete` true)
                    (`KismetSystemLibrary.K2_ClearAndInvalidateTimerHandle` (`self.Timer Handle`))
                    (`KismetSystemLibrary.PrintString` "World GEN Finished"))
                  (elif (> (`self.Number of Objectives`) 0)
                    (`self.Generate_Objective`)
                    (else
                      (`self.Close off Open Spaces`))))))))))))

(fn `Spawn Vents`
  (bind _vent_list (`self.Vent List`))
  (bind _selected_vent (`self.Selected Vent`))
  (set `self.Selected Vent` (`KismetArrayLibrary.Array_RandomFromStream` _vent_list (`self.Stream`)))
  (`KismetArrayLibrary.Array_RemoveItem` _vent_list _selected_vent)
  (`|SpawnActorFromClass` (`self.Vents`) (`SceneComponent.K2_GetComponentToWorld` _selected_vent) "AlwaysSpawn" "MultiplyWithRoot" null true null)
  (`self.Close off Vent Holes`))

(fn `UserConstructionScript`)