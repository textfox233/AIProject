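; Animation notify state that marks the span of an attack in an AIProjectCharacter's animation.
; On begin, it casts the mesh owner to Pawn and then AIProjectCharacter, sets the action state to Attacking, and calls CheckActionState.
; On end, it does the same but resets the action state to Unoccupied.
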(fn `Received_NotifyBegin`
  (params (MeshComp :type "SkeletalMeshComponent Object Reference") (Animation :type "AnimSequenceBase Object Reference") (TotalDuration :type "Float (single-precision)") (EventReference :type "AnimNotifyEventReference Structure (by ref)"))
  (returns (ReturnValue :type Boolean))
  (bind _aspawn (cast `Pawn` (`ActorComponent.GetOwner` MeshComp)))
  (bind _asaiproject_character (cast `AIProjectCharacter` _aspawn))
  (`AIProjectCharacter.SetActionState` _asaiproject_character "EAS_Attacking")
  (`AIProjectCharacter.CheckActionState` _asaiproject_character)
  (return false))

(fn `Received_NotifyEnd`
  (params (MeshComp :type "SkeletalMeshComponent Object Reference") (Animation :type "AnimSequenceBase Object Reference") (EventReference :type "AnimNotifyEventReference Structure (by ref)"))
  (returns (ReturnValue :type Boolean))
  (bind _aspawn (cast `Pawn` (`ActorComponent.GetOwner` MeshComp)))
  (bind _asaiproject_character (cast `AIProjectCharacter` _aspawn))
  (`AIProjectCharacter.SetActionState` _asaiproject_character "EAS_Unoccupied")
  (`AIProjectCharacter.CheckActionState` _asaiproject_character)
  (return false))