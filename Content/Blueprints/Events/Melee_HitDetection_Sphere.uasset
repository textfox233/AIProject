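; Anim notify state that marks the melee hit detection window (Sphere, per its name) within an attack animation.
; On begin and end, it looks up the MeleeComponent on the mesh's owner and calls StartHitDetection and EndHitDetection respectively, leaving detection itself to that component.
; If the component is missing, both events print an error, and the end event's message mislabels itself as NotifyBegin.
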(fn `Received_NotifyBegin`
  (params (MeshComp :type "SkeletalMeshComponent Object Reference") (Animation :type "AnimSequenceBase Object Reference") (TotalDuration :type "Float (single-precision)") (EventReference :type "AnimNotifyEventReference Structure (by ref)"))
  (returns (ReturnValue :type Boolean))
  (bind _returnvalue (`Actor.GetComponentByClass` (`ActorComponent.GetOwner` MeshComp) "/Script/AIProject.MeleeComponent"))
  ;[1 1 1] Trigger Melee Hit Detection (Sphere)
  (`/Engine/EditorBlueprintResources/StandardMacros.IsValid` _returnvalue
    (:`Is Valid`
      (`MeleeComponent.StartHitDetection` _returnvalue)
      (return false))
    (:`Is Not Valid`
      ;[1 1 1] Debug Messages
      (`KismetSystemLibrary.PrintString` null "ERROR in MeleeEvent::NotifyBegin - Target has no Melee Component"))))

(fn `Received_NotifyEnd`
  (params (MeshComp :type "SkeletalMeshComponent Object Reference") (Animation :type "AnimSequenceBase Object Reference") (EventReference :type "AnimNotifyEventReference Structure (by ref)"))
  (returns (ReturnValue :type Boolean))
  (bind _returnvalue (`Actor.GetComponentByClass` (`ActorComponent.GetOwner` MeshComp) "/Script/AIProject.MeleeComponent"))
  ;[1 1 1] Stop Trigger Melee Event
  (`/Engine/EditorBlueprintResources/StandardMacros.IsValid` _returnvalue
    (:`Is Valid`
      (`MeleeComponent.EndHitDetection` _returnvalue)
      (return false))
    (:`Is Not Valid`
      ;[1 1 1] Debug Messages
      (`KismetSystemLibrary.PrintString` null "ERROR in MeleeEvent::NotifyBegin - Target has no Melee Component"))))