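; Actor component that marks its owner as an interactive object, driving client-side view and overview markers and an input tip.
; The interaction system's toggle events set each state, and a retriggerable delay switches it off unless refreshed within the update period.
; Paired DoOnce gates fire show or hide only on state changes, on widget components found by tag; overview and interact handle only Pickup.
; Server and multicast events update the CanBeInteract flag.
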(event `ClientToggleViewObj`
  (params (ToggleOn :type Boolean))
  ;[1 1 1] TOGGLE VIEW OBJ
  ;;[1 0.1179 0] INPUT FROM INTERACTION OBJ SYSTEM
  (if ToggleOn
    (set `self.ToggleOnView` true)
    (`self.ClientHandleViewState`)
    (`KismetSystemLibrary.RetriggerableDelay` (`self.InteractiveUpdatePeriodTime`))
    (set `self.ToggleOnView` false)
    (`self.ClientHandleViewState`)
    (else
      (set `self.ToggleOnView` false)
      (`self.ClientHandleViewState`))))

(event `ServerUpdateCanBeInteract`
  (params (CanBeInteract :type Boolean))
  ;[1 1 1] UPDATE CAN BE INTERACT
  ;;[1 0.1179 0] INPUT FROM OWNER
  (set `self.CanBeInteract` CanBeInteract))

(event `MulticastUpdateCanBeInteract`
  (params (CanBeInteract :type Boolean))
  ;[1 1 1] UPDATE CAN BE INTERACT
  (set `self.CanBeInteract` CanBeInteract))

(event `ClientToggleOverviewObj`
  (params (ToggleOn :type Boolean))
  ;[1 1 1] TOGGLE OVERVIEW OBJ
  ;;[1 0.1179 0] INPUT FROM INTERACTION OBJ SYSTEM
  (if ToggleOn
    (set `self.ToggleOnOverview` true)
    (`self.ClientHandleOverviewState`)
    (`KismetSystemLibrary.RetriggerableDelay` (`self.InteractiveUpdatePeriodTime`))
    (set `self.ToggleOnOverview` false)
    (`self.ClientHandleOverviewState`)
    (else
      (set `self.ToggleOnOverview` false)
      (`self.ClientHandleOverviewState`))))

(event `ClientToggleInteractObj`
  (params (ToggleOn :type Boolean))
  ;[1 1 1] TOGGLE INTERACT OBJ
  ;;[1 0.1179 0] INPUT FROM INTERACTION OBJ SYSTEM
  (if ToggleOn
    (set `self.ToggleOnInteract` true)
    (`self.ClientHandleInteractState`)
    (`KismetSystemLibrary.RetriggerableDelay` (`self.InteractiveUpdatePeriodTime`))
    (set `self.ToggleOnInteract` false)
    (`self.ClientHandleInteractState`)
    (else
      (set `self.ToggleOnInteract` false)
      (`self.ClientHandleInteractState`))))

(event `ClientHandleViewState`
  ;[1 1 1] HANDLE VIEW STATE
  ;;[1 0.2552 0.2552] CHECK: Owner is valid
  (`/Engine/EditorBlueprintResources/StandardMacros.IsValid` (`self.GetOwner`)
    (:`Is Valid`
      ;;[1 0.2552 0.2552] CHECK: ToggleOnView
      (if (`self.ToggleOnView`)
        (`|ExecutionSequence`
          (:`then_0`
            (`/Engine/EditorBlueprintResources/StandardMacros.DoOnce` false :!label _label
              (:`Completed`
                ;;[1 1 1] Show view marker
                ;;;[1 0.2552 0.2552] CHECK: Widget is valid
                (`/Engine/EditorBlueprintResources/StandardMacros.IsValid` (`WidgetComponent.GetWidget` (`|GetArrayItem` (`Actor.GetComponentsByTag` (`self.GetOwner`) "/Script/UMG.WidgetComponent" (`self.TagInteractiveObjectMarkerView`))))
                  (:`Is Valid`
                    ;;;[1 0.6824 0] TO WBP_InteractiveObjectMarkerView
                    (bind _aswbp_interactive_object_marker_view (cast `/Game/CHARACTER_SYSTEM_V2/Blueprints/PlayerHUD/InteractiveObject/WBP_InteractiveObjectMarkerView` (`WidgetComponent.GetWidget` (`|GetArrayItem` (`Actor.GetComponentsByTag` (`self.GetOwner`) "/Script/UMG.WidgetComponent" (`self.TagInteractiveObjectMarkerView`))))))
                    (`/Game/CHARACTER_SYSTEM_V2/Blueprints/PlayerHUD/InteractiveObject/WBP_InteractiveObjectMarkerView.ShowMarker` _aswbp_interactive_object_marker_view))))))
          (:`then_1`
            (goto _label_2 :!via `Reset`)))
        (else
          (`|ExecutionSequence`
            (:`then_0`
              (`/Engine/EditorBlueprintResources/StandardMacros.DoOnce` false :!label _label_2
                (:`Completed`
                  ;;[1 1 1] Hide view marker
                  ;;;[1 0.2552 0.2552] CHECK: Widget is valid
                  (`/Engine/EditorBlueprintResources/StandardMacros.IsValid` (`WidgetComponent.GetWidget` (`|GetArrayItem` (`Actor.GetComponentsByTag` (`self.GetOwner`) "/Script/UMG.WidgetComponent" (`self.TagInteractiveObjectMarkerView`))))
                    (:`Is Valid`
                      ;;;[1 0.6824 0] TO WBP_InteractiveObjectMarkerView
                      (bind _aswbp_interactive_object_marker_view_2 (cast `/Game/CHARACTER_SYSTEM_V2/Blueprints/PlayerHUD/InteractiveObject/WBP_InteractiveObjectMarkerView` (`WidgetComponent.GetWidget` (`|GetArrayItem` (`Actor.GetComponentsByTag` (`self.GetOwner`) "/Script/UMG.WidgetComponent" (`self.TagInteractiveObjectMarkerView`))))))
                      (`/Game/CHARACTER_SYSTEM_V2/Blueprints/PlayerHUD/InteractiveObject/WBP_InteractiveObjectMarkerView.HideMarker` _aswbp_interactive_object_marker_view_2))))))
            (:`then_1`
              (goto _label :!via `Reset`))))))))

(event `ClientHandleOverviewState`
  ;[1 1 1] HANDLE OVERVIEW STATE
  ;;[1 0.2552 0.2552] CHECK: Owner is valid
  (`/Engine/EditorBlueprintResources/StandardMacros.IsValid` (`self.GetOwner`)
    (:`Is Valid`
      ;;[1 0.2552 0.2552] CHECK: InteractiveObjType
      (switch `/Game/CHARACTER_SYSTEM_V2/Blueprints/DATA/E/InteractiveObj/E_InteractiveObjType` (`self.InteractiveObjType`)
        (:`NewEnumerator0`
          (`self.ClientHandleOverviewStatePickup`))))))

(event `ClientHandleOverviewStatePickup`
  ;[1 1 1] HANDLE OVERVIEW STATE PICKUP
  ;;[1 0.2552 0.2552] CHECK: ToggleOnOverview
  (if (`self.ToggleOnOverview`)
    (`|ExecutionSequence`
      (:`then_0`
        (`/Engine/EditorBlueprintResources/StandardMacros.DoOnce` false :!label _label_3
          (:`Completed`
            ;;[1 1 1] Show overview marker
            ;;;[1 0.2552 0.2552] CHECK: Widget is valid
            (`/Engine/EditorBlueprintResources/StandardMacros.IsValid` (`WidgetComponent.GetWidget` (`|GetArrayItem` (`Actor.GetComponentsByTag` (`self.GetOwner`) "/Script/UMG.WidgetComponent" (`self.TagInteractiveObjectMarkerOverviewPickup`))))
              (:`Is Valid`
                ;;;[1 0.6824 0] TO WBP_InteractiveObjectMarkerView
                (bind _aswbp_interactive_object_marker_overview_pickup (cast `/Game/CHARACTER_SYSTEM_V2/Blueprints/PlayerHUD/InteractiveObject/WBP_InteractiveObjectMarkerOverviewPickup` (`WidgetComponent.GetWidget` (`|GetArrayItem` (`Actor.GetComponentsByTag` (`self.GetOwner`) "/Script/UMG.WidgetComponent" (`self.TagInteractiveObjectMarkerOverviewPickup`))))))
                (`/Game/CHARACTER_SYSTEM_V2/Blueprints/PlayerHUD/InteractiveObject/WBP_InteractiveObjectMarkerOverviewPickup.ShowMarker` _aswbp_interactive_object_marker_overview_pickup))))))
      (:`then_1`
        (goto _label_4 :!via `Reset`)))
    (else
      (`|ExecutionSequence`
        (:`then_0`
          (`/Engine/EditorBlueprintResources/StandardMacros.DoOnce` false :!label _label_4
            (:`Completed`
              ;;[1 1 1] Hide overview marker
              ;;;[1 0.2552 0.2552] CHECK: Widget is valid
              (`/Engine/EditorBlueprintResources/StandardMacros.IsValid` (`WidgetComponent.GetWidget` (`|GetArrayItem` (`Actor.GetComponentsByTag` (`self.GetOwner`) "/Script/UMG.WidgetComponent" (`self.TagInteractiveObjectMarkerOverviewPickup`))))
                (:`Is Valid`
                  ;;;[1 0.6824 0] TO WBP_InteractiveObjectMarkerView
                  (bind _aswbp_interactive_object_marker_overview_pickup_2 (cast `/Game/CHARACTER_SYSTEM_V2/Blueprints/PlayerHUD/InteractiveObject/WBP_InteractiveObjectMarkerOverviewPickup` (`WidgetComponent.GetWidget` (`|GetArrayItem` (`Actor.GetComponentsByTag` (`self.GetOwner`) "/Script/UMG.WidgetComponent" (`self.TagInteractiveObjectMarkerOverviewPickup`))))))
                  (`/Game/CHARACTER_SYSTEM_V2/Blueprints/PlayerHUD/InteractiveObject/WBP_InteractiveObjectMarkerOverviewPickup.HideMarker` _aswbp_interactive_object_marker_overview_pickup_2))))))
        (:`then_1`
          (goto _label_3 :!via `Reset`))))))

(event `ClientHandleInteractState`
  ;[1 1 1] HANDLE INTERACT STATE
  ;;[1 0.2552 0.2552] CHECK: Owner is valid
  (`/Engine/EditorBlueprintResources/StandardMacros.IsValid` (`self.GetOwner`)
    (:`Is Valid`
      ;;[1 0.2552 0.2552] CHECK: InteractiveObjType
      (switch `/Game/CHARACTER_SYSTEM_V2/Blueprints/DATA/E/InteractiveObj/E_InteractiveObjType` (`self.InteractiveObjType`)
        (:`NewEnumerator0`
          (`self.ClientHandleInteractStatePickup`))))))

(event `ClientHandleInteractStatePickup`
  ;[1 1 1] HANDLE INTERACT STATE PICKUP
  ;;[1 0.2552 0.2552] CHECK: ToggleOnOverview
  (if (`self.ToggleOnInteract`)
    (`|ExecutionSequence`
      (:`then_0`
        (`/Engine/EditorBlueprintResources/StandardMacros.DoOnce` false :!label _label_5
          (:`Completed`
            ;;[1 1 1] Show overview marker
            ;;;[1 0.2552 0.2552] CHECK: Widget is valid
            (`/Engine/EditorBlueprintResources/StandardMacros.IsValid` (`WidgetComponent.GetWidget` (`|GetArrayItem` (`Actor.GetComponentsByTag` (`self.GetOwner`) "/Script/UMG.WidgetComponent" (`self.TagInteractiveObjectMarkerOverviewPickup`))))
              (:`Is Valid`
                ;;;[1 0.6824 0] TO WBP_InteractiveObjectMarkerView
                (bind _aswbp_interactive_object_marker_overview_pickup (cast `/Game/CHARACTER_SYSTEM_V2/Blueprints/PlayerHUD/InteractiveObject/WBP_InteractiveObjectMarkerOverviewPickup` (`WidgetComponent.GetWidget` (`|GetArrayItem` (`Actor.GetComponentsByTag` (`self.GetOwner`) "/Script/UMG.WidgetComponent" (`self.TagInteractiveObjectMarkerOverviewPickup`))))))
                (`/Game/CHARACTER_SYSTEM_V2/Blueprints/PlayerHUD/InteractiveObject/WBP_InteractiveObjectMarkerOverviewPickup.ShowInputTip` _aswbp_interactive_object_marker_overview_pickup))))))
      (:`then_1`
        (goto _label_6 :!via `Reset`)))
    (else
      (`|ExecutionSequence`
        (:`then_0`
          (`/Engine/EditorBlueprintResources/StandardMacros.DoOnce` false :!label _label_6
            (:`Completed`
              ;;[1 1 1] Hide overview marker
              ;;;[1 0.2552 0.2552] CHECK: Widget is valid
              (`/Engine/EditorBlueprintResources/StandardMacros.IsValid` (`WidgetComponent.GetWidget` (`|GetArrayItem` (`Actor.GetComponentsByTag` (`self.GetOwner`) "/Script/UMG.WidgetComponent" (`self.TagInteractiveObjectMarkerOverviewPickup`))))
                (:`Is Valid`
                  ;;;[1 0.6824 0] TO WBP_InteractiveObjectMarkerView
                  (bind _aswbp_interactive_object_marker_overview_pickup_2 (cast `/Game/CHARACTER_SYSTEM_V2/Blueprints/PlayerHUD/InteractiveObject/WBP_InteractiveObjectMarkerOverviewPickup` (`WidgetComponent.GetWidget` (`|GetArrayItem` (`Actor.GetComponentsByTag` (`self.GetOwner`) "/Script/UMG.WidgetComponent" (`self.TagInteractiveObjectMarkerOverviewPickup`))))))
                  (`/Game/CHARACTER_SYSTEM_V2/Blueprints/PlayerHUD/InteractiveObject/WBP_InteractiveObjectMarkerOverviewPickup.HideInputTip` _aswbp_interactive_object_marker_overview_pickup_2))))))
        (:`then_1`
          (goto _label_5 :!via `Reset`))))))

(fn `GetCanBeInteract`
  (returns (CanBeInteract :type Boolean))
  (return (`self.CanBeInteract`)))

(fn `GetInteractiveObjType`
  (returns (InteractiveObjType :type "/Game/CHARACTER_SYSTEM_V2/Blueprints/DATA/E/InteractiveObj/E_InteractiveObjType Enum"))
  (return (`self.InteractiveObjType`)))