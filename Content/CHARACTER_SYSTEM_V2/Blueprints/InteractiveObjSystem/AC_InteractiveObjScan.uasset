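; Character component that periodically scans for tagged interactive objects and picks the best one to interact with.
; A looping timer, started only in standalone or on the server, sphere-traces around the owner, enabling view, overview and interact candidacy by distance.
; A camera sphere trace prioritises aimed-at candidates, falling back to all in range, and the nearest wins.
; Results go to server events and BP_CharacterCommon; vehicles limit scanning to view toggling.
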(event `self.ReceiveBeginPlay`
  ;[1 1 1] EVENT BEGIN PLAY
  ;;[1 1 1] Delay
  (`KismetSystemLibrary.Delay` 3.0)
  ;;[1 1 1] Start scaning
  (if (`KismetSystemLibrary.IsStandalone`)
    (`KismetSystemLibrary.K2_SetTimer` null "ClientScanInteractiveObjects" (`self.CheckFrequency`) true :!label _label)
    (elif (`KismetSystemLibrary.IsServer`)
      (goto _label))))

(event `ClientScanInteractiveObjects`
  (bind _returnvalue (`Actor.K2_GetActorLocation` (`self.GetOwner`)))
  ;[1 1 1] SCAN INTERACTIVE OBJECTS
  ;;[1 1 1] Clear array for scan
  (`KismetArrayLibrary.Array_Clear` (`self.IntObjArrayFinalCommon`))
  (`KismetArrayLibrary.Array_Clear` (`self.IntObjArrayFromScan`))
  (`KismetArrayLibrary.Array_Clear` (`self.IntObjArrayForInteract`))
  ;;[1 1 1] Multi sphere trace
  (bind _outhits (`KismetSystemLibrary.SphereTraceMultiForObjects` _returnvalue _returnvalue (`self.MinDistanceView`) (`self.ObjectTypesForScan`) true (`|MakeArray` (`self.GetOwner`)) (select `bool` (`self.DrawDebug`) :`true` "ForDuration" :!type "EDrawDebugTrace Enum") true (struct :`R` 1.0 :`A` 1.0) (struct :`G` 1.0 :`A` 1.0) (`self.CheckFrequency`)))
  ;;[1 1 1] Toggle view & Toggle overview state by main scan around character
  ;;;[1 1 1] For each loop of hits by scan trace
  (for _array_element _outhits
    (bind (_bblockinghit _binitialoverlap _time _distance _location _impactpoint _normal _impactnormal _physmat _hitactor) (`GameplayStatics.BreakHitResult` _array_element))
    ;;;[1 0.2552 0.2552] CHECK: Tag = InteractiveObject
    (if (`Actor.ActorHasTag` _hitactor (`self.InteractiveObjectTag`))
      ;;;[1 1 1] Init checked actor
      (set `self.CheckedActor` _hitactor)
      ;;;[1 0.2552 0.2552] CHECK: InteractionObjTarget = valid
      (`/Engine/EditorBlueprintResources/StandardMacros.IsValid` (`Actor.GetComponentByClass` (`self.CheckedActor`) "/Game/CHARACTER_SYSTEM_V2/Blueprints/InteractiveObjSystem/AC_InteractiveObjTarget.AC_InteractiveObjTarget_C")
        (:`Is Valid`
          ;;;[1 0.2552 0.2552] CHECK: CanBeInteract = 1
          (if (`/Game/CHARACTER_SYSTEM_V2/Blueprints/InteractiveObjSystem/AC_InteractiveObjTarget.GetCanBeInteract` (`Actor.GetComponentByClass` (`self.CheckedActor`) "/Game/CHARACTER_SYSTEM_V2/Blueprints/InteractiveObjSystem/AC_InteractiveObjTarget.AC_InteractiveObjTarget_C"))
            ;;;[1 0.6824 0] TO INTERACTIVE OBJ TARGET
            (`/Game/CHARACTER_SYSTEM_V2/Blueprints/InteractiveObjSystem/AC_InteractiveObjTarget.ClientToggleViewObj` (`Actor.GetComponentByClass` (`self.CheckedActor`) "/Game/CHARACTER_SYSTEM_V2/Blueprints/InteractiveObjSystem/AC_InteractiveObjTarget.AC_InteractiveObjTarget_C") true)
            ;;;[1 1 1] Initialize CheckedActorFirstPoint
            (bind (_outhits_2 _returnvalue_2) (`KismetSystemLibrary.SphereTraceMultiForObjects` (`Actor.K2_GetActorLocation` (`self.GetOwner`)) (`Actor.K2_GetActorLocation` (`self.CheckedActor`)) 50.0 (`self.ObjectTypesForScan`) false (`|MakeArray` (`self.GetOwner`)) (select `bool` (`self.DrawDebug`) :`true` "ForDuration" :!type "EDrawDebugTrace Enum") true (struct :`R` 1.0 :`A` 1.0) (struct :`G` 1.0 :`A` 1.0) (`self.CheckFrequency`)))
            (if _returnvalue_2
              (for _array_element_2 _outhits_2
                (bind (_bblockinghit_2 _binitialoverlap_2 _time_2 _distance_2 _location_2 _impactpoint_2 _normal_2 _impactnormal_2 _physmat_2 _hitactor_2) (`GameplayStatics.BreakHitResult` _array_element_2))
                (if (== _hitactor_2 (`self.CheckedActor`))
                  (set `self.CheckedActorFirstPoint` _location_2)
                  ;;;[1 0.2552 0.2552] CHECK: Character state for interact with objects
                  (if (not (`/Game/CHARACTER_SYSTEM_V2/Blueprints/CharacterCommon/BP_CharacterCommon.GetInVehicle` (`self.GetCharacterCommon`)))
                    ;;;[1 0.2552 0.2552] CHECK: Min distance for toggle on of overview
                    (if (<= (`KismetMathLibrary.Vector_Distance` (`self.CheckedActorFirstPoint`) (`Actor.K2_GetActorLocation` (`self.GetOwner`))) (`self.MinDistanceOverview`))
                      ;;;[1 0.6824 0] TO INTERACTIVE OBJ TARGET
                      (`/Game/CHARACTER_SYSTEM_V2/Blueprints/InteractiveObjSystem/AC_InteractiveObjTarget.ClientToggleOverviewObj` (`Actor.GetComponentByClass` (`self.CheckedActor`) "/Game/CHARACTER_SYSTEM_V2/Blueprints/InteractiveObjSystem/AC_InteractiveObjTarget.AC_InteractiveObjTarget_C") true)
                      ;;;[1 0.2552 0.2552] CHECK: Min distance for toggle of interact with one object
                      (if (<= (`KismetMathLibrary.Vector_Distance` (`self.CheckedActorFirstPoint`) (`Actor.K2_GetActorLocation` (`self.GetOwner`))) (`self.MinDistanceInteract`))
                        ;;;[1 1 1] Form array of object in interact distance
                        (`KismetArrayLibrary.Array_AddUnique` (`self.IntObjArrayForInteract`) (`self.CheckedActor`)))))))))))))
  ;;[1 1 1] Find int object in scan
  ;;;[1 0.2552 0.2552] CHECK: Character state for interact with objects
  (if (not (`/Game/CHARACTER_SYSTEM_V2/Blueprints/CharacterCommon/BP_CharacterCommon.GetInVehicle` (`self.GetCharacterCommon`)))
    ;;;[1 1 1] Multi Trace from camera
    (bind _outhits_3 (`KismetSystemLibrary.SphereTraceMultiForObjects` (`SceneComponent.K2_GetComponentLocation` (`self.GetMainPlayerCamera`)) (+ (`SceneComponent.K2_GetComponentLocation` (`self.GetMainPlayerCamera`)) (* (`KismetMathLibrary.GetForwardVector` (`SceneComponent.K2_GetComponentRotation` (`self.GetMainPlayerCamera`))) (`self.ScanDistanceOverview`))) (`self.ScanRadiusOverview`) (`self.ObjectTypesForScan`) true (`|MakeArray` (`self.GetOwner`)) (select `bool` (`self.DrawDebug`) :`true` "ForDuration" :!type "EDrawDebugTrace Enum") true (struct :`R` 0.177803 :`B` 1.0 :`A` 1.0) (struct :`R` 1.0 :`B` 0.143681 :`A` 1.0) (`self.CheckFrequency`)))
    ;;;[1 1 1] For each loop by scan trace
    (for _array_element_3 _outhits_3
      (bind (_bblockinghit_3 _binitialoverlap_3 _time_3 _distance_3 _location_3 _impactpoint_3 _normal_3 _impactnormal_3 _physmat_3 _hitactor_3) (`GameplayStatics.BreakHitResult` _array_element_3))
      ;;;[1 0.2552 0.2552] CHECK: Tag = InteractiveObject
      (if (`Actor.ActorHasTag` _hitactor_3 (`self.InteractiveObjectTag`))
        ;;;[1 0.2552 0.2552] CHECK: InteractionObjTarget = valid
        (`/Engine/EditorBlueprintResources/StandardMacros.IsValid` (`Actor.GetComponentByClass` _hitactor_3 "/Game/CHARACTER_SYSTEM_V2/Blueprints/InteractiveObjSystem/AC_InteractiveObjTarget.AC_InteractiveObjTarget_C")
          (:`Is Valid`
            ;;;[1 1 1] form array of obj from scan
            (`KismetArrayLibrary.Array_AddUnique` (`self.IntObjArrayFromScan`) _hitactor_3)))))
    ;;[1 1 1] Define the best actor for interact
    ;;;[1 0.2552 0.2552] CHECK: IntObjArrayFromScan Length = 0
    (if (== (`KismetArrayLibrary.Array_Length` (`self.IntObjArrayFromScan`)) 0)
      ;;;[1 0.2552 0.2552] CHECK: IntObjArrayForInteract Length = 0
      (if (== (`KismetArrayLibrary.Array_Length` (`self.IntObjArrayForInteract`)) 0) :!label _label_2
        ;;;[1 1 1] Off interact
        (bind _output_get (set `self.InteractiveObjectFound` false))
        (`self.ServerUpdateInteractiveObjectFound` _output_get)
        ;;;[1 0.6824 0] TO CHARACTER COMMON
        (`/Game/CHARACTER_SYSTEM_V2/Blueprints/CharacterCommon/BP_CharacterCommon.ClientHandleUpdateInteractiveObjectFound` (`self.GetCharacterCommon`))
        (else
          ;;;[1 1 1] Initialize the best obj for interact
          (bind _output_get_2 (set `self.TheBestIntObj` (`.ReturnValue` (`GameplayStatics.FindNearestActor` (`Actor.K2_GetActorLocation` (`self.GetOwner`)) (`self.IntObjArrayForInteract`)))))
          (`self.ServerUpdateTheBestObj` _output_get_2)
          ;;;[1 0.6824 0] TO INTERACTIVE OBJ TARGET
          (`/Game/CHARACTER_SYSTEM_V2/Blueprints/InteractiveObjSystem/AC_InteractiveObjTarget.ClientToggleInteractObj` (`Actor.GetComponentByClass` (`self.TheBestIntObj`) "/Game/CHARACTER_SYSTEM_V2/Blueprints/InteractiveObjSystem/AC_InteractiveObjTarget.AC_InteractiveObjTarget_C") true)
          ;;;[1 1 1] Initialize interact obj type from target component
          (bind _output_get_3 (set `self.InteractiveObjType` (`/Game/CHARACTER_SYSTEM_V2/Blueprints/InteractiveObjSystem/AC_InteractiveObjTarget.GetInteractiveObjType` (`Actor.GetComponentByClass` (`self.TheBestIntObj`) "/Game/CHARACTER_SYSTEM_V2/Blueprints/InteractiveObjSystem/AC_InteractiveObjTarget.AC_InteractiveObjTarget_C"))))
          (`self.ServerUpdateInteractiveObjType` _output_get_3)
          ;;;[1 0.6824 0] TO CHARACTER COMMON
          (`/Game/CHARACTER_SYSTEM_V2/Blueprints/CharacterCommon/BP_CharacterCommon.ClientHandleInteractEnable` (`self.GetCharacterCommon`))
          ;;;[1 1 1] On interact
          (bind _output_get_4 (set `self.InteractiveObjectFound` true))
          (`self.ServerUpdateInteractiveObjectFound` _output_get_4)
          ;;;[1 0.6824 0] TO CHARACTER COMMON
          (`/Game/CHARACTER_SYSTEM_V2/Blueprints/CharacterCommon/BP_CharacterCommon.ClientHandleUpdateInteractiveObjectFound` (`self.GetCharacterCommon`))))
      (else
        ;;;[1 1 1] Foreach loop
        (for _array_element_4 (`self.IntObjArrayForInteract`)
          (for _array_element_5 (`self.IntObjArrayFromScan`)
            (if (== _array_element_5 _array_element_4)
              (`KismetArrayLibrary.Array_AddUnique` (`self.IntObjArrayFinalCommon`) _array_element_5))))
        ;;;[1 0.2552 0.2552] CHECK: IntObjArrayForInteract Length = 0
        (if (== (`KismetArrayLibrary.Array_Length` (`self.IntObjArrayFinalCommon`)) 0)
          (goto _label_2)
          (else
            ;;;[1 1 1] Initialize the best obj for interact
            (bind _output_get_5 (set `self.TheBestIntObj` (`.ReturnValue` (`GameplayStatics.FindNearestActor` (`Actor.K2_GetActorLocation` (`self.GetOwner`)) (`self.IntObjArrayFinalCommon`)))))
            (`self.ServerUpdateTheBestObj` _output_get_5)
            ;;;[1 0.6824 0] TO INTERACTIVE OBJ TARGET
            (`/Game/CHARACTER_SYSTEM_V2/Blueprints/InteractiveObjSystem/AC_InteractiveObjTarget.ClientToggleInteractObj` (`Actor.GetComponentByClass` (`self.TheBestIntObj`) "/Game/CHARACTER_SYSTEM_V2/Blueprints/InteractiveObjSystem/AC_InteractiveObjTarget.AC_InteractiveObjTarget_C") true)
            ;;;[1 1 1] Initialize interact obj type from target component
            (bind _output_get_6 (set `self.InteractiveObjType` (`/Game/CHARACTER_SYSTEM_V2/Blueprints/InteractiveObjSystem/AC_InteractiveObjTarget.GetInteractiveObjType` (`Actor.GetComponentByClass` (`self.TheBestIntObj`) "/Game/CHARACTER_SYSTEM_V2/Blueprints/InteractiveObjSystem/AC_InteractiveObjTarget.AC_InteractiveObjTarget_C"))))
            (`self.ServerUpdateInteractiveObjType` _output_get_6)
            ;;;[1 0.6824 0] TO CHARACTER COMMON
            (`/Game/CHARACTER_SYSTEM_V2/Blueprints/CharacterCommon/BP_CharacterCommon.ClientHandleInteractEnable` (`self.GetCharacterCommon`))
            ;;;[1 1 1] On interact
            (bind _output_get_7 (set `self.InteractiveObjectFound` true))
            (`self.ServerUpdateInteractiveObjectFound` _output_get_7)
            ;;;[1 0.6824 0] TO CHARACTER COMMON
            (`/Game/CHARACTER_SYSTEM_V2/Blueprints/CharacterCommon/BP_CharacterCommon.ClientHandleUpdateInteractiveObjectFound` (`self.GetCharacterCommon`))))))))

(event `ServerUpdateInteractiveObjectFound`
  (params (InteractiveObjectFound :type Boolean))
  ;[1 1 1] SCAN INTERACTIVE OBJECTS
  ;;[1 1 1] ServerUpdateInteractiveObjectFound
  (set `self.InteractiveObjectFound` InteractiveObjectFound))

(event `ServerUpdateInteractiveObjType`
  (params (InteractiveObjType :type "/Game/CHARACTER_SYSTEM_V2/Blueprints/DATA/E/InteractiveObj/E_InteractiveObjType Enum" :default "NewEnumerator3"))
  ;[1 1 1] SCAN INTERACTIVE OBJECTS
  ;;[1 1 1] ServerUpdateInteractiveObjType
  (set `self.InteractiveObjType` InteractiveObjType))

(event `ServerUpdateTheBestObj`
  (params (TheBestIntObj :type "Actor Object Reference"))
  ;[1 1 1] SCAN INTERACTIVE OBJECTS
  ;;[1 1 1] ServerUpdateTheBestObj
  (set `self.TheBestIntObj` TheBestIntObj))

(fn `GetCharacterCommon`
  (returns (CharacterCommon :type "/Game/CHARACTER_SYSTEM_V2/Blueprints/CharacterCommon/BP_CharacterCommon Object Reference"))
  (`/Engine/EditorBlueprintResources/StandardMacros.IsValid` (`self.GetOwner`)
    (:`Is Valid`
      (bind _asbp_character_common (cast `/Game/CHARACTER_SYSTEM_V2/Blueprints/CharacterCommon/BP_CharacterCommon` (`self.GetOwner`)))
      (return _asbp_character_common))))

(fn `GetInteractiveObjectFound`
  (returns (InteractiveObjectFound :type Boolean))
  (return (`self.InteractiveObjectFound`)))

(fn `GetInteractiveObjType`
  (returns (InteractiveObjType :type "/Game/CHARACTER_SYSTEM_V2/Blueprints/DATA/E/InteractiveObj/E_InteractiveObjType Enum"))
  (return (`self.InteractiveObjType`)))

(fn `GetMainPlayerCamera`
  (returns (MainPlayerCamera :type "CameraComponent Object Reference"))
  (bind _output (`|GetArrayItem` (`Actor.GetComponentsByTag` (`self.GetOwner`) "/Script/Engine.CameraComponent" (`self.MainPlayerCameraTag`))))
  (`/Engine/EditorBlueprintResources/StandardMacros.IsValid` _output
    (:`Is Valid`
      (return _output))))

(fn `GetTheBestIntObj`
  (returns (TheBestIntObj :type "Actor Object Reference"))
  (return (`self.TheBestIntObj`)))