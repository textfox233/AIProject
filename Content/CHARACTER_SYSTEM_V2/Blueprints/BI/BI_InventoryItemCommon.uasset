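; Blueprint interface for common inventory item data in the character system.
; It declares getters for weapon wheel and weapon module icons, title, description, rarity type and ammo count.
; A single setter passes an ammo count along with a Default argument.
; The file holds only signatures with empty default returns, so implementing items supply the actual values.
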(fn `GetInventoryItemCommonAmmoCount`
  (returns (AmmoCount :type Integer))
  (return 0))

(fn `GetInventoryItemCommonDesc`
  (returns (Title :type Text))
  (return ""))

(fn `GetInventoryItemCommonIconWeaponModule`
  (returns (Icon :type "Texture2D Object Reference"))
  (return null))

(fn `GetInventoryItemCommonIconWeaponWheel`
  (returns (Icon :type "Texture2D Object Reference"))
  (return null))

(fn `GetInventoryItemCommonRarityType`
  (returns (RarityType :type "/Game/CHARACTER_SYSTEM_V2/Blueprints/DATA/E/Inventory/E_RarityType Enum"))
  (return "NewEnumerator0"))

(fn `GetInventoryItemCommonTitle`
  (returns (Title :type Text))
  (return ""))

(fn `InventoryItemCommonSetAmmoCount`
  (params (AmmoCount :type Integer) (Default :type Boolean)))