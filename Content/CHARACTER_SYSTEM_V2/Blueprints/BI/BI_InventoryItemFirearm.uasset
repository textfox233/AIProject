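; Blueprint interface for firearm inventory items in the character system.
; It declares setters for attachments, including a reset to default attachments.
; Getters expose ammo type, firearm type, current attachments and stats such as damage, fire rate, magazine size, reload time, accuracy and handling.
; The file holds only signatures with default returns, leaving the logic to implementing items.
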(fn `GetInventoryItemFirearmAccuracyAttribute`
  (returns (AccuracyAttribute :type Integer))
  (return 0))

(fn `GetInventoryItemFirearmAmmoType`
  (returns (FirearmAmmoType :type "/Game/CHARACTER_SYSTEM_V2/Blueprints/DATA/E/E_FirearmAmmoType Enum"))
  (return "NewEnumerator0"))

(fn `GetInventoryItemFirearmAttachments`
  (returns (FirearmAttachments :type "Array of /Game/CHARACTER_SYSTEM_V2/Blueprints/DATA/STR/STR_GL_FirearmAttachmentDesc Structure"))
  (return))

(fn `GetInventoryItemFirearmDamageValue`
  (returns (DamageValue :type "Float (double-precision)"))
  (return 0.0))

(fn `GetInventoryItemFirearmFireRate`
  (returns (FireRate :type Integer))
  (return 0))

(fn `GetInventoryItemFirearmHandlingAttribute `
  (returns (`HandlingAttribute ` :type Integer))
  (return 0))

(fn `GetInventoryItemFirearmMagazinSize`
  (returns (MagazinSize :type Integer))
  (return 0))

(fn `GetInventoryItemFirearmMainReloadTime`
  (returns (MainReloadTime :type "Float (double-precision)"))
  (return 0.0))

(fn `GetInventoryItemFirearmType`
  (returns (FirearmType :type "/Game/CHARACTER_SYSTEM_V2/Blueprints/DATA/E/E_FirearmType Enum"))
  (return "NewEnumerator0"))

(fn `InventoryItemFirearmSetAttachments`
  (params (FirearmAttachments :type "Array of /Game/CHARACTER_SYSTEM_V2/Blueprints/DATA/STR/STR_GL_FirearmAttachmentDesc Structure")))

(fn `InventoryItemFirearmSetDefaultAttachments`)