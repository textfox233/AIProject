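; Test-case game mode that spawns characters for all player controllers and respawns them on request.
; Initial spawning is staggered on a looping timer, counting down the controller index and possessing one pawn per tick at the matching start point, or the world origin if none exists.
; Respawn waits briefly, then spawns and possesses a new character at a random start point.
; A local wrapper tags debug logs behind a toggle.
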(event `self.SpawnCharactersForPlayers`
  ;[1 1 1] SPAWN CHARACTERS FOR PLAYERS
  ;;[0.1778 0 1] PARENT INPUT
  ;;[0.05604 0 1] LogAdvanced
  (`self.LogAdvanced` "<SPAWN>" "Spawn Characters For Players handeling")
  ;;[1 1 1] Initialize sparced spawn timer
  (bind _returnvalue (`KismetSystemLibrary.K2_SetTimerDelegate` (delegate `ServerSpawnCharacter`) 0.2 true 0.2))
  (set `self.TimerSparcedSpawn` _returnvalue)
  (set `self.PlayerIndex` (`KismetArrayLibrary.Array_Length` (`self.GetPlayerControllers`)))
  (`/Engine/EditorBlueprintResources/StandardMacros.DecrementInt` (`self.PlayerIndex`)))

(event `ServerSpawnCharacter`
  ;[1 1 1] SPAWN CHARACTERS FOR PLAYERS
  ;;[1 0.2552 0.2552] CHECK: PlayerCount
  (if (< (`self.PlayerIndex`) 0)
    ;;[1 1 1] Spawn finish
    ;;;[0.05604 0 1] LogAdvanced
    (`self.LogAdvanced` "<SPAWN>" "Characters spawn is finished")
    (`KismetSystemLibrary.K2_ClearAndInvalidateTimerHandle` (`self.TimerSparcedSpawn`))
    (else
      ;;[1 1 1] Spawn character
      (bind _returnvalue (`|SpawnActorFromClass` (`self.CharacterClass`) (select `bool` (> (`self.PlayerIndex`) (`KismetArrayLibrary.Array_LastIndex` (`self.GetPlayerStartPoints`))) :`false` (`self.GetTransform` (`|GetArrayItem` (`self.GetPlayerStartPoints`) (`self.PlayerIndex`))) :`true` (`KismetMathLibrary.MakeTransform` (0.0 0.0 0.0))) "Undefined" "SelectDefaultAtRuntime" null null))
      (bind _aspawn (cast `Pawn` _returnvalue))
      ;;;[0.05604 0 1] LogAdvanced
      (`self.LogAdvanced` "<SPAWN>" (`KismetStringLibrary.Concat_StrStr` "Spawned character: " (`KismetSystemLibrary.GetDisplayName` _aspawn) " /// for player controller: " (`KismetSystemLibrary.GetDisplayName` (`|GetArrayItem` (`self.GetPlayerControllers`) (`self.PlayerIndex`))) " /// player index: " (`KismetStringLibrary.Conv_IntToString` (`self.PlayerIndex`))))
      (`Controller.Possess` (`|GetArrayItem` (`self.GetPlayerControllers`) (`self.PlayerIndex`)) _aspawn)
      (`/Engine/EditorBlueprintResources/StandardMacros.DecrementInt` (`self.PlayerIndex`)))))

(event `self.RespawnCharacterForPlayer`
  (params (PlayerController :type "PlayerController Object Reference"))
  ;[1 1 1] RESPAWN CHARACTER FOR PLAYER
  ;;[0.1778 0 1] PARENT INPUT
  (`KismetSystemLibrary.Delay` 3.0)
  (bind _returnvalue (`|SpawnActorFromClass` (`self.CharacterClass`) (`self.GetTransform` (`KismetArrayLibrary.Array_Random` (`self.GetPlayerStartPoints`))) "Undefined" "SelectDefaultAtRuntime" null null))
  (bind _aspawn (cast `Pawn` _returnvalue))
  (`Controller.Possess` PlayerController _aspawn)
  ;;[0.05604 0 1] LogAdvanced
  (`self.LogAdvanced` "<SPAWN>" (`KismetStringLibrary.Concat_StrStr` "Respawned character: " (`KismetSystemLibrary.GetDisplayName` _aspawn) " /// for player controller: " (`KismetSystemLibrary.GetDisplayName` PlayerController))))

(fn `UserConstructionScript`
  (`parent.UserConstructionScript`))