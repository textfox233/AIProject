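; BP_GameModeCommon is a base game mode that coordinates player character spawning and respawning.
; On begin play it caches all PlayerStart actors and, after a short delay, fires SpawnCharactersForPlayers; post login collects player controllers.
; Respawn requests forward to RespawnCharacterForPlayer; both spawn events are empty hooks for child classes.
; Getters expose the start points and controllers, and a tagged, toggleable debug log traces each step.
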(event `self.ReceiveBeginPlay`
  ;[1 1 1] EVENT BEGIN PLAY
  ;;[0.05604 0 1] LogAdvanced
  (`self.LogAdvanced` "<SPAWN>" "Gamemode created (event begin play)")
  ;;[1 1 1] Initialize all players start from a current playable level
  (bind _outactors (`GameplayStatics.GetAllActorsOfClass` "/Script/Engine.PlayerStart"))
  (set `self.PlayerStartPoints` _outactors)
  (`KismetSystemLibrary.Delay` 2.0)
  ;;[0.05604 0 1] LogAdvanced
  (`self.LogAdvanced` "<SPAWN>" "Spawn Characters For Players triggered")
  (`self.SpawnCharactersForPlayers`))

(event `SpawnCharactersForPlayers`
  ;[1 1 1] EVENT BEGIN PLAY
  ;;[0.1778 0 1] PARENT OUTPUT EVENT
)

(event `self.K2_PostLogin`
  (params (NewPlayer :type "PlayerController Object Reference"))
  ;[1 1 1] EVENT ON POST LOGIN
  ;;[0.05604 0 1] LogAdvanced
  (`self.LogAdvanced` "<SPAWN>" (`KismetStringLibrary.Concat_StrStr` "Initialize player controller: " (`KismetSystemLibrary.GetDisplayName` NewPlayer)))
  (`KismetArrayLibrary.Array_AddUnique` (`self.PlayerControllers`) NewPlayer))

(event `PlayerCharacterRequestedRespawn`
  (params (PlayerController :type "PlayerController Object Reference"))
  ;[1 1 1] RESPAWN CHARACTER FOR PLAYER
  ;;[0.05604 0 1] LogAdvanced
  (`self.LogAdvanced` "<SPAWN>" (`KismetStringLibrary.Concat_StrStr` "Player character requested respawn for player controller: " (`KismetSystemLibrary.GetDisplayName` PlayerController)))
  (`self.RespawnCharacterForPlayer` PlayerController))

(event `RespawnCharacterForPlayer`
  (params (PlayerController :type "PlayerController Object Reference"))
  ;[1 1 1] RESPAWN CHARACTER FOR PLAYER
  ;;[0.1778 0 1] PARENT OUTPUT EVENT
)

(fn `GetPlayerControllers`
  (returns (PlayerControllers :type "Array of PlayerController Object Reference"))
  (return (`self.PlayerControllers`)))

(fn `GetPlayerStartPoints`
  (returns (PlayerStartPoints :type "Array of PlayerStart Object Reference"))
  (return (`self.PlayerStartPoints`)))

(fn `UserConstructionScript`)