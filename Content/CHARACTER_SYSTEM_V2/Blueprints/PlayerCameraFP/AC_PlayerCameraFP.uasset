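; First-person camera component for the player character that handles aim-down-sights FOV, depth of field and stance-based view pitch limits.
; Aiming steps FOV between default and aim values on a looping timer paced by the ADS time.
; Optional DOF applies aim post-process values and line-traces focal distance on a fast timer while aiming.
; Stance changes set camera manager pitch limits, easing them when the crouch or prone view is out of range.
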(event `ClientInitializeFPCamera`
  (params (PlayerCamera :type "CameraComponent Object Reference") (SetFOV :type Boolean))
  (bind ((`DepthOfFieldFstop` _depthoffieldfstop) (`VignetteIntensity` _vignetteintensity) (`DepthOfFieldSensorWidth` _depthoffieldsensorwidth) (`DepthOfFieldFocalDistance` _depthoffieldfocaldistance)) (break `PostProcessSettings` (`CameraComponent.PostProcessSettings` (`self.Player Camera`))))
  ;[1 1 1] INITIALIZE CAMERA
  ;;[1 0.1179 0] INPUT FP CHARACTER
  (set `self.Player Camera` PlayerCamera)
  ;;[1 1 1] Initialize default FOV
  (set `self.CurrentCameraFOV` (`self.CameraDefaultFOV`))
  (if SetFOV
    (set `CameraComponent.FieldOfView` (`self.CurrentCameraFOV`) (`self.Player Camera`)))
  ;;[1 1 1] Initialize Min & Max pitch angles for camera
  (set `PlayerCameraManager.ViewPitchMax` (`self.StandViewPitchMax`) (`GameplayStatics.GetPlayerCameraManager` 0))
  (set `PlayerCameraManager.ViewPitchMin` (`self.StandViewPitchMin`) (`GameplayStatics.GetPlayerCameraManager` 0))
  ;;[1 1 1] Initialize default DOF properties
  (set `self.DefCameraApertureFStop` _depthoffieldfstop)
  (set `self.DefCameraVignetteIntensity` _vignetteintensity)
  (set `self.DefCameraSensorWidthMm` _depthoffieldsensorwidth)
  (set `self.DefCameraFocalDistance` _depthoffieldfocaldistance))

(event `ClientUpdateFPCameraState`
  (params (`FPCameraState?` :type Boolean))
  ;[1 1 1] UPDATE FP CAMERA STATE
  ;;[1 0.1179 0] INPUT TP-FP CHARACTER
  (set `self.FPCameraState` `FPCameraState?`))

(event `ClientInitializeCurrentADSTime`
  (params (CurrentADSTime :type "Float (double-precision)"))
  ;[1 1 1] INITIALIZE CURRENT ADS TIME
  ;;[1 0.1179 0] INPUT FP CHARACTER
  (set `self.CurrentADSTime` CurrentADSTime))

(event `ClientUpdateCurrentFOV`
  (params (NewCurrentFOV :type "Float (double-precision)"))
  ;[1 1 1] UPDATE CURRENT FOV
  ;;[1 0.1179 0] INPUT TP-FP CHARACTER
  (set `self.CurrentCameraFOV` NewCurrentFOV))

(event `ClientChangeCameraOnAim`
  (params (InADS :type Boolean))
  ;[1 1 1] CHANGE CAMERA ON AIM
  ;;[1 1 1] START CHANGE CAMERA ON AIM
  ;;;[1 0.1179 0] INPUT FP CHARACTER
  (set `self.InADS` InADS)
  (`self.ClientStopChangeCameraOnAim`)
  (set `self.InChangingOnAim` true)
  ;;;[1 1 1] Calculation InterpolationTimeStep
  (set `self.FOVInterpolationTimeStep` (/ (`self.CurrentADSTime`) (`KismetMathLibrary.Conv_IntToDouble` (`self.CommonInterpStepCount`))))
  ;;;[1 0.2552 0.2552] CHECK: In ADS
  (if (`self.InADS`)
    ;;;[1 1 1] FOV Initialize DEFAULT to AIM
    (set `self.FOVInterpolationStep` (/ (- (`self.GetCameraAimFOVWithGunsmithInf`) (`self.CurrentCameraFOV`)) (`KismetMathLibrary.Conv_IntToDouble` (`self.CommonInterpStepCount`))))
    (else
      ;;;[1 1 1] FOV Initialize AIM to DEFAULT
      (set `self.FOVInterpolationStep` (/ (- (`self.CameraDefaultFOV`) (`self.CurrentCameraFOV`)) (`KismetMathLibrary.Conv_IntToDouble` (`self.CommonInterpStepCount`))))))
  ;;;[1 1 1] Start interpolation
  (`self.ClientInterpStepChangeCameraOnAim`)
  (`KismetSystemLibrary.K2_SetTimer` null "ClientInterpStepChangeCameraOnAim" (`self.FOVInterpolationTimeStep`) true)
  ;;;[1 0.2552 0.2552] CHECK: UseDOFEffect
  (if (`self.UseDOFEffect`)
    ;;;[1 0.2552 0.2552] CHECK: In ADS
    (if (`self.InADS`)
      ;;;[1 1 1] Set DOF for Aim state
      (set `self.CurrentCameraApertureFStop` (`self.AimCameraApertureFStop`))
      (set `self.CurrentCameraVignetteIntensity` (`self.AimCameraVignetteIntensity`))
      (set `self.CurrentCameraSensorWidthMm` (`self.AimCameraSensorWidthMm`))
      ;;;[1 1 1] Start update DOF
      (`KismetSystemLibrary.K2_SetTimer` null "ClientUpdateDOF" 0.01 true)
      (else
        ;;;[1 1 1] Set DOF for Aim state
        (set `self.CurrentCameraApertureFStop` (`self.DefCameraApertureFStop`))
        (set `self.CurrentCameraVignetteIntensity` (`self.DefCameraVignetteIntensity`))
        (set `self.CurrentCameraSensorWidthMm` (`self.DefCameraSensorWidthMm`))
        ;;;[1 1 1] Stop update DOF
        (`KismetSystemLibrary.K2_ClearTimer` null "ClientUpdateDOF")))
    ;;;[1 1 1] Update DOF on aim on / off
    (set `CameraComponent.PostProcessSettings` (make `PostProcessSettings` :`DepthOfFieldFstop` (`self.CurrentCameraApertureFStop`) :`VignetteIntensity` (`self.CurrentCameraVignetteIntensity`) :`DepthOfFieldSensorWidth` (`self.CurrentCameraSensorWidthMm`) :`DepthOfFieldFocalDistance` (select `bool` (`self.InADS`) :`true` (`self.CurrentFocalDistance`))) (`self.Player Camera`))))

(event `ClientStopChangeCameraOnAim`
  ;[1 1 1] CHANGE CAMERA ON AIM
  ;;[1 1 1] ClientStopChangingFPCameraFOV
  (`KismetSystemLibrary.K2_ClearTimer` null "ClientInterpStepChangeCameraOnAim"))

(event `ClientInterpStepChangeCameraOnAim`
  ;[1 1 1] CHANGE CAMERA ON AIM
  ;;[1 1 1] Interpolation
  ;;;[1 0.2552 0.2552] CHECK: In ADS
  (if (`self.InADS`)
    ;;;[1 0.2552 0.2552] CHECK: Main to Aim Condition
    (if (`KismetMathLibrary.NearlyEqual_FloatFloat` (`self.CurrentCameraFOV`) (`self.GetCameraAimFOVWithGunsmithInf`) 1.0)
      ;;;[1 1 1] Aim state setted
      (`self.ClientStopChangeCameraOnAim`)
      ;;;;[1 1 1] Set FOV for Aim state
      (set `self.CurrentCameraFOV` (`self.GetCameraAimFOVWithGunsmithInf`))
      (set `CameraComponent.FieldOfView` (`self.CurrentCameraFOV`) (`self.Player Camera`))
      (set `self.InChangingOnAim` false)
      (else
        ;;;[1 1 1] Interpolation
        ;;;;[1 1 1] FOV
        (set `self.CurrentCameraFOV` (+ (`self.CurrentCameraFOV`) (`self.FOVInterpolationStep`)) :!label _label)
        (set `CameraComponent.FieldOfView` (`self.CurrentCameraFOV`) (`self.Player Camera`))))
    (else
      ;;;[1 0.2552 0.2552] CHECK: Aim to Main Condition
      (if (`KismetMathLibrary.NearlyEqual_FloatFloat` (`self.CurrentCameraFOV`) (`self.CameraDefaultFOV`) 1.0)
        ;;;[1 1 1] Default state setted
        (`self.ClientStopChangeCameraOnAim`)
        ;;;;[1 1 1] Set FOV for Default state
        (set `self.CurrentCameraFOV` (`self.CameraDefaultFOV`))
        (set `CameraComponent.FieldOfView` (`self.CameraDefaultFOV`) (`self.Player Camera`))
        (set `self.InChangingOnAim` false)
        (else
          (goto _label))))))

(event `ClientUpdateDOF`
  (bind _returnvalue (`SceneComponent.K2_GetComponentLocation` (`self.Player Camera`)))
  ;[1 1 1] CHANGE CAMERA ON AIM
  ;;[1 1 1] Update DOF on AIM ON
  (if (`self.FPCameraState`)
    ;;;[1 1 1] Calculation focal distance by line trace
    (bind (_outhit _returnvalue_2) (`KismetSystemLibrary.LineTraceSingleForObjects` _returnvalue (+ _returnvalue (* (`SceneComponent.GetForwardVector` (`self.Player Camera`)) (`self.MaxViewDistanceDOF`))) (`|MakeArray` "ObjectTypeQuery1" "ObjectTypeQuery2" "ObjectTypeQuery3" "ObjectTypeQuery4" "ObjectTypeQuery5" "ObjectTypeQuery7" "ObjectTypeQuery8" :!type "EObjectTypeQuery Enum") true (`|MakeArray` (`self.GetOwner` self))))
    (if _returnvalue_2
      (bind (_bblockinghit _binitialoverlap _time _distance _location _impactpoint _normal _impactnormal _physmat _hitactor _hitcomponent _hitbonename _bonename _hititem _elementindex _faceindex _tracestart) (`GameplayStatics.BreakHitResult` _outhit))
      (set `self.CurrentFocalDistance` (`KismetMathLibrary.VSize` (- _location _tracestart)))
      (else
        (set `self.CurrentFocalDistance` (`self.MaxViewDistanceDOF`))))
    ;;;[1 0.2552 0.2552] CHECK: UseDOFEffect
    (if (`self.UseDOFEffect`)
      ;;;[1 1 1] Update DOF if AIM ON
      (set `CameraComponent.PostProcessSettings` (make `PostProcessSettings` :`DepthOfFieldFstop` (`self.CurrentCameraApertureFStop`) :`VignetteIntensity` (`self.CurrentCameraVignetteIntensity`) :`DepthOfFieldSensorWidth` (`self.CurrentCameraSensorWidthMm`) :`DepthOfFieldFocalDistance` (select `bool` (`self.InADS`) :`true` (`self.CurrentFocalDistance`))) (`self.Player Camera`)))))

(event `ClientUpdateMaxCameraAngels`
  (params (MainCharacterState :type "/Game/CHARACTER_SYSTEM_V2/Blueprints/DATA/E/E_CharacterMainState Enum" :default "NewEnumerator0"))
  (bind _returnvalue (`GameplayStatics.GetPlayerCameraManager` 0))
  ;[1 1 1] UPDATE MIN / MAX CAMERA ANGELS
  ;;[1 1 1] Start update min / max camera angles
  ;;;[1 0.1179 0] INPUT FP CHARACTER
  (`/Engine/EditorBlueprintResources/StandardMacros.IsValid` (`GameplayStatics.GetPlayerCameraManager` 0)
    (:`Is Valid`
      (`KismetSystemLibrary.Delay` 0.1)
      ;;;[1 0.2552 0.2552] CHECK: CharacterMainState
      (switch `/Game/CHARACTER_SYSTEM_V2/Blueprints/DATA/E/E_CharacterMainState` MainCharacterState
        (:`NewEnumerator0`
          ;;;[1 1 1] STAND
          (set `PlayerCameraManager.ViewPitchMax` (`self.StandViewPitchMax`) _returnvalue :!label _label_2)
          (set `PlayerCameraManager.ViewPitchMin` (`self.StandViewPitchMin`) _returnvalue))
        (:`NewEnumerator1`
          (goto _label_2))
        (:`NewEnumerator2`
          ;;;[1 1 1] CROUCH
          ;;;;[1 1 1] Set View Max
          (set `PlayerCameraManager.ViewPitchMax` (`self.CrouchViewPitchMax`) (`GameplayStatics.GetPlayerCameraManager` 0) :!label _label_3)
          ;;;;[1 1 1] Condition for Min Pitch Angle
          (if (< (.pitch (`Actor.K2_GetActorRotation` (`GameplayStatics.GetPlayerCameraManager` 0))) (`self.CrouchViewPitchMin`))
            ;;;;[1 1 1] Initialize Interp Values
            (set `self.CurrentPitchAngle` (.pitch (`Actor.K2_GetActorRotation` (`GameplayStatics.GetPlayerCameraManager` 0))))
            (set `self.TargetPitchAngle` (`self.CrouchViewPitchMin`))
            (set `self.ChangeMinCameraAngle` true)
            ;;;[1 1 1] Calculation InterpolationTimeStep
            (set `self.MinMaxAngleInterpolationTimeStep` (/ (`self.ChangingMinMaxAngleIterpTime`) (`KismetMathLibrary.Conv_IntToDouble` (`self.CommonInterpStepCount`))) :!label _label_4)
            (`self.ClientStopChangingMinMaxAngles`)
            ;;;[1 1 1] MinMaxAngleInterpolationStep
            (set `self.MinMaxAngleInterpolationStep` (/ (- (`self.TargetPitchAngle`) (`self.CurrentPitchAngle`)) (`KismetMathLibrary.Conv_IntToDouble` (`self.CommonInterpStepCount`))))
            ;;;[1 1 1] Start interpolation
            (`self.ClientInterpStepChangeCameraMinMaxAngle`)
            (`KismetSystemLibrary.K2_SetTimer` null "ClientInterpStepChangeCameraMinMaxAngle" (`self.MinMaxAngleInterpolationTimeStep`) true)
            (else
              ;;;;[1 1 1] Set Pitch Min
              (set `PlayerCameraManager.ViewPitchMin` (`self.CrouchViewPitchMin`) (`GameplayStatics.GetPlayerCameraManager` 0)))))
        (:`NewEnumerator3`
          (goto _label_3))
        (:`NewEnumerator4`
          ;;;[1 1 1] PRONE
          (`|ExecutionSequence` :!label _label_5
            (:`then_0`
              ;;;;[1 1 1] Min Angle
              ;;;;;[1 1 1] Condition for Min Pitch Angle
              (if (<= (.pitch (`Actor.K2_GetActorRotation` (`GameplayStatics.GetPlayerCameraManager` 0))) (`self.ProneViewPitchMin`))
                ;;;;;[1 1 1] Initialize Interp Values
                (set `self.CurrentPitchAngle` (.pitch (`Actor.K2_GetActorRotation` (`GameplayStatics.GetPlayerCameraManager` 0))))
                (set `self.TargetPitchAngle` (`self.ProneViewPitchMin`))
                (set `self.ChangeMinCameraAngle` true)
                (goto _label_4)
                (else
                  ;;;;;[1 1 1] Set Min Angle
                  (set `PlayerCameraManager.ViewPitchMin` (`self.ProneViewPitchMin`) (`GameplayStatics.GetPlayerCameraManager` 0)))))
            (:`then_1`
              ;;;;[1 1 1] Max Angle
              ;;;;;[1 1 1] Condition for Max Angle
              (if (<= (`self.ProneViewPitchMax`) (.pitch (`Actor.K2_GetActorRotation` (`GameplayStatics.GetPlayerCameraManager` 0))))
                ;;;;;[1 1 1] initialize Interp Values
                (set `self.CurrentPitchAngle` (.pitch (`Actor.K2_GetActorRotation` (`GameplayStatics.GetPlayerCameraManager` 0))))
                (set `self.TargetPitchAngle` (`self.ProneViewPitchMax`))
                (set `self.ChangeMinCameraAngle` false)
                (goto _label_4)
                (else
                  ;;;;;[1 1 1] Set Max angle
                  (set `PlayerCameraManager.ViewPitchMax` (`self.ProneViewPitchMax`) (`GameplayStatics.GetPlayerCameraManager` 0)))))))
        (:`NewEnumerator5`
          (goto _label_5))))))

(event `ClientStopChangingMinMaxAngles`
  ;[1 1 1] UPDATE MIN / MAX CAMERA ANGELS
  ;;[1 1 1] ClientStopChangingFPCameraFOV
  (`KismetSystemLibrary.K2_ClearTimer` null "ClientInterpStepChangeCameraMinMaxAngle"))

(event `ClientInterpStepChangeCameraMinMaxAngle`
  ;[1 1 1] UPDATE MIN / MAX CAMERA ANGELS
  ;;[1 1 1] Interpolation
  ;;;[1 0.2552 0.2552] CHECK: Target = Current Pitch Angle
  (if (`KismetMathLibrary.NearlyEqual_FloatFloat` (`self.TargetPitchAngle`) (`self.CurrentPitchAngle`) 1.0)
    (set `self.CurrentPitchAngle` (`self.TargetPitchAngle`))
    (`self.ClientStopChangingMinMaxAngles`)
    (else
      (set `self.CurrentPitchAngle` (+ (`self.CurrentPitchAngle`) (`self.MinMaxAngleInterpolationStep`)))))
  ;;;[1 0.2552 0.2552] CHECK: ChangeMinCameraAngle
  (if (`self.ChangeMinCameraAngle`)
    (set `PlayerCameraManager.ViewPitchMin` (`self.CurrentPitchAngle`) (`GameplayStatics.GetPlayerCameraManager` 0))
    (else
      (set `PlayerCameraManager.ViewPitchMax` (`self.CurrentPitchAngle`) (`GameplayStatics.GetPlayerCameraManager` 0)))))

(event `ClientUpdateDOFOnChangeCameraMode`
  (params (InADS :type Boolean))
  ;[1 1 1] UPDATE DOF ON CHANGE CAMERA
  ;;[1 0.1179 0] INPUT TP-FP CHARACTER
  (set `self.InADS` InADS)
  ;;[1 0.2552 0.2552] CHECK: UseDOFEffect
  (if (`self.UseDOFEffect`)
    ;;[1 0.2552 0.2552] CHECK: In ADS
    (if (`self.InADS`)
      ;;[1 1 1] Set DOF for Aim state
      (set `self.CurrentCameraApertureFStop` (`self.AimCameraApertureFStop`))
      (set `self.CurrentCameraVignetteIntensity` (`self.AimCameraVignetteIntensity`))
      (set `self.CurrentCameraSensorWidthMm` (`self.AimCameraSensorWidthMm`))
      ;;[1 1 1] Start update DOF
      (`KismetSystemLibrary.K2_SetTimer` null "ClientUpdateDOF" 0.01 true)
      (else
        ;;[1 1 1] Set DOF for Aim state
        (set `self.CurrentCameraApertureFStop` (`self.DefCameraApertureFStop`))
        (set `self.CurrentCameraVignetteIntensity` (`self.DefCameraVignetteIntensity`))
        (set `self.CurrentCameraSensorWidthMm` (`self.DefCameraSensorWidthMm`))
        ;;[1 1 1] Stop update DOF
        (`KismetSystemLibrary.K2_ClearTimer` null "ClientUpdateDOF")))
    ;;[1 1 1] Update DOF on aim on / off
    (set `CameraComponent.PostProcessSettings` (make `PostProcessSettings` :`DepthOfFieldFstop` (`self.CurrentCameraApertureFStop`) :`VignetteIntensity` (`self.CurrentCameraVignetteIntensity`) :`DepthOfFieldSensorWidth` (`self.CurrentCameraSensorWidthMm`) :`DepthOfFieldFocalDistance` (select `bool` (`self.InADS`) :`true` (`self.CurrentFocalDistance`))) (`self.Player Camera`))))

(fn `GetCameraAimFOVWithGunsmithInf`
  (returns (AimFOV :type "Float (double-precision)"))
  (return (/ (`self.CameraAimFOV`) 1.0)))

(fn `GetInChangingOnAim`
  (returns (InChangingFOV :type Boolean))
  (return (`self.InChangingOnAim`)))