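; BP_PickupCommon is a common pickup actor for the character system, likely serving as a base for specific pickups.
; It stores a PickupType with a getter and setter, and destroys itself through a multicast removal event triggered from the common character.
; Its inventory getters for common, equip and firearm data are stubs that return empty or default values.
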(event `MulticastRemovePickupFromLevel`
  ;[1 1 1] REMOVE PICKUP
  ;;[1 0.1179 0] INPUT FROM CHARACTER COMMON
  (`self.K2_DestroyActor`))

(fn `GetInventoryItemCommonAmmoCount`
  (returns (AmmoCount :type Integer))
  (return 0))

(fn `GetInventoryItemCommonDesc`
  (returns (Title :type Text))
  (return ""))

(fn `GetInventoryItemCommonIconWeaponModule`
  (returns (Icon :type "Texture2D Object Reference"))
  (return null))

(fn `GetInventoryItemCommonIconWeaponWheel`
  (returns (Icon :type "Texture2D Object Reference"))
  (return null))

(fn `GetInventoryItemCommonRarityType`
  (returns (RarityType :type "/Game/CHARACTER_SYSTEM_V2/Blueprints/DATA/E/Inventory/E_RarityType Enum"))
  (return "NewEnumerator0"))

(fn `GetInventoryItemCommonTitle`
  (returns (Title :type Text))
  (return ""))

(fn `GetInventoryItemEquipCanBeCrafted`
  (returns (CanBeCrafted :type Boolean))
  (return false))

(fn `GetInventoryItemEquipCommonType`
  (returns (EquipCommonType :type "/Game/CHARACTER_SYSTEM_V2/Blueprints/DATA/E/Equipment/E_EquipmentCommonType Enum"))
  (return "NewEnumerator0"))

(fn `GetInventoryItemEquipNeededResourcesList`
  (returns (NeededResourcesList :type "Array of /Game/CHARACTER_SYSTEM_V2/Blueprints/DATA/STR/STR_GL_InventoryResourceDesc Structure") (NewParam :type Boolean))
  (return _ false))

(fn `GetInventoryItemEquipUpgrades`
  (returns (EquipmentUpgrades :type "Array of /Game/CHARACTER_SYSTEM_V2/Blueprints/DATA/STR/STR_GL_EquipmentUpgradeDesc Structure"))
  (return))

(fn `GetInventoryItemEquipUsingType`
  (returns (EquipmentUsingType :type "/Game/CHARACTER_SYSTEM_V2/Blueprints/DATA/E/Equipment/E_EquipmentUsingType Enum"))
  (return "NewEnumerator0"))

(fn `GetInventoryItemFirearmAccuracyAttribute`
  (returns (AccuracyAttribute :type Integer))
  (return 0))

(fn `GetInventoryItemFirearmAmmoType`
  (returns (FirearmAmmoType :type "/Game/CHARACTER_SYSTEM_V2/Blueprints/DATA/E/E_FirearmAmmoType Enum"))
  (return "NewEnumerator0"))

(fn `GetInventoryItemFirearmAttachments`
  (returns (FirearmAttachments :type "Array of /Game/CHARACTER_SYSTEM_V2/Blueprints/DATA/STR/STR_GL_FirearmAttachmentDesc Structure"))
  (return))

(fn `GetInventoryItemFirearmDamageValue`
  (returns (DamageValue :type "Float (double-precision)"))
  (return 0.0))

(fn `GetInventoryItemFirearmFireRate`
  (returns (FireRate :type Integer))
  (return 0))

(fn `GetInventoryItemFirearmHandlingAttribute `
  (returns (`HandlingAttribute ` :type Integer))
  (return 0))

(fn `GetInventoryItemFirearmMagazinSize`
  (returns (MagazinSize :type Integer))
  (return 0))

(fn `GetInventoryItemFirearmMainReloadTime`
  (returns (MainReloadTime :type "Float (double-precision)"))
  (return 0.0))

(fn `GetInventoryItemFirearmType`
  (returns (FirearmType :type "/Game/CHARACTER_SYSTEM_V2/Blueprints/DATA/E/E_FirearmType Enum"))
  (return "NewEnumerator0"))

(fn `GetPickupType`
  (returns (PickupType :type "/Game/CHARACTER_SYSTEM_V2/Blueprints/DATA/E/InteractiveObj/E_InteractiveObjPickupType Enum"))
  (return (`self.PickupType`)))

(fn `SetPickupType`
  (params (PickupType :type "/Game/CHARACTER_SYSTEM_V2/Blueprints/DATA/E/InteractiveObj/E_InteractiveObjPickupType Enum" :default "NewEnumerator0"))
  (set `self.PickupType` PickupType))

(fn `UserConstructionScript`)