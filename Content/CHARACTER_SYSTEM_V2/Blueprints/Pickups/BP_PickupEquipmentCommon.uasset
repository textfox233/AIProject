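; Base pickup for common equipment (lethal, tactical, support) that holds an equipment actor and count.
; When flagged as a level pickup with a positive count, it spawns the equipment class on server or standalone after a short BeginPlay delay.
; The spawn sends a default-attachments message, then multicasts attachment to the pickup mesh and initialization.
; Initialization reads title, icon, rarity and types through interface messages to fill the overview marker widget.
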(event `self.ReceiveBeginPlay`
  ;[1 1 1] EVENT BEGIN PLAY
  (`parent.ReceiveBeginPlay`)
  ;;[1 1 1] Set pickup as firearm pickup
  (`self.SetPickupType` "NewEnumerator6")
  ;;[1 1 1] Delay 2 sec
  (`KismetSystemLibrary.Delay` 2.0)
  ;;[1 0.2552 0.2552] CHECK: SpawnAsLevelPickup
  (if (`self.SpawnAsLevelPickup`)
    ;;[1 0.2552 0.2552] CHECK: Equip count
    (if (> (`self.EquipmentCount`) 0)
      ;;[1 0.2552 0.2552] CHECK: IsStandalone or server
      (if (or (`KismetSystemLibrary.IsStandalone`) (`KismetSystemLibrary.IsServer`))
        (`self.ServerSpawnEquipmentInPickup`)))))

(event `ServerSpawnEquipmentInPickup`
  ;[1 1 1] SPAWN FIREARM IN PICKUP
  ;;[1 1 1] Spawn Weapon In Pickup
  (bind _returnvalue (`|SpawnActorFromClass` (`self.EquipmentClass`) (`SceneComponent.GetRelativeTransform` (`self.DefaultSceneRoot`)) "AlwaysSpawn" "OverrideRootScale" null null))
  ;;[1 1 1] Check Valid actor as equipment
  (`/Engine/EditorBlueprintResources/StandardMacros.IsValid` _returnvalue
    (:`Is Valid`
      (bind _output_get (set `self.EquipmentActor` _returnvalue))
      (cast `/Game/CHARACTER_SYSTEM_V2/Blueprints/Equipments/BP_EquipmentActorCommon` _output_get)
      ;;[1 1 1] Initialize default attachments in spawned firearm
      (message `/Game/CHARACTER_SYSTEM_V2/Blueprints/BI/BI_InventoryItemFirearm.InventoryItemFirearmSetDefaultAttachments` (`self.EquipmentActor`))
      ;;[1 1 1] Attach & Initialize spawned actor
      (`self.MulticastAttachEquipmentActor`)
      (`self.MulticastInitializeEquipementPickup`))))

(event `MulticastAttachEquipmentActor`
  ;[1 1 1] ATTACH
  (`/Engine/EditorBlueprintResources/StandardMacros.IsValid` (`self.EquipmentActor`)
    (:`Is Valid`
      (`self.K2_AttachToComponent` (`self.EquipmentActor`) (`self.EquipmentMesh`) "None" "SnapToTarget" "SnapToTarget" "KeepRelative" true))))

(event `MulticastInitializeEquipementPickup`
  ;[1 1 1] INITIALIZE FIREARM PICKUP
  ;;[1 1 1] Getting values from actor across BI
  (bind _icon (message `/Game/CHARACTER_SYSTEM_V2/Blueprints/BI/BI_InventoryItemCommon.GetInventoryItemCommonIconWeaponWheel` (`self.EquipmentActor`)))
  (set `self.IconWeaponWheel` _icon)
  (bind _title (message `/Game/CHARACTER_SYSTEM_V2/Blueprints/BI/BI_InventoryItemCommon.GetInventoryItemCommonTitle` (`self.EquipmentActor`)))
  (set `self.Title` _title)
  (bind _raritytype (message `/Game/CHARACTER_SYSTEM_V2/Blueprints/BI/BI_InventoryItemCommon.GetInventoryItemCommonRarityType` (`self.EquipmentActor`)))
  (set `self.RarityType` _raritytype)
  (bind _equipcommontype (message `/Game/CHARACTER_SYSTEM_V2/Blueprints/BI/BI_InventoryItemEquip.GetInventoryItemEquipCommonType` (`self.EquipmentActor`)))
  (set `self.EquipCommonType` _equipcommontype)
  (bind _equipmentusingtype (message `/Game/CHARACTER_SYSTEM_V2/Blueprints/BI/BI_InventoryItemEquip.GetInventoryItemEquipUsingType` (`self.EquipmentActor`)))
  (set `self.EquipmentUsingType` _equipmentusingtype)
  ;;[1 0.6824 0] TO WBP_InteractiveObjectMarkerView
  (bind _aswbp_interactive_object_marker_overview_pickup (cast `/Game/CHARACTER_SYSTEM_V2/Blueprints/PlayerHUD/InteractiveObject/WBP_InteractiveObjectMarkerOverviewPickup` (`WidgetComponent.GetWidget` (`self.InteractiveObjectMarkerOverviewPickup`))))
  (`/Game/CHARACTER_SYSTEM_V2/Blueprints/PlayerHUD/InteractiveObject/WBP_InteractiveObjectMarkerOverviewPickup.InitializeOverviewMarker` _aswbp_interactive_object_marker_overview_pickup (`self.Title`) (select `/Game/CHARACTER_SYSTEM_V2/Blueprints/DATA/E/Equipment/E_EquipmentCommonType` (`self.EquipCommonType`) :`NewEnumerator0` "LETHAL EQUIPMENT" :`NewEnumerator1` "TACTICAL EQUIPMENT" :`NewEnumerator2` "SUPPORT EQUIPMENT" :!type "Text") (select `/Game/CHARACTER_SYSTEM_V2/Blueprints/DATA/E/Equipment/E_EquipmentUsingType` (`self.EquipmentUsingType`) :`NewEnumerator0` "THROW" :`NewEnumerator1` "SET" :`NewEnumerator3` "USE ON SELF" :!type "Text") (`self.RarityType`) (`self.EquipmentCount`) "NewEnumerator6" (`self.IconWeaponWheel`)))

(fn `GetEquipmentActor`
  (returns (EquipmentActor :type "Actor Object Reference"))
  (return (`self.EquipmentActor`)))

(fn `GetEquipmentCount`
  (returns (EquipmentCount :type Integer))
  (return (`self.EquipmentCount`)))

(fn `UserConstructionScript`
  (`parent.UserConstructionScript`))