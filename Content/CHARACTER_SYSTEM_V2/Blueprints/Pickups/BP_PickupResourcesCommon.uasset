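; Common resource pickup Blueprint that holds a resource type and amount, exposed through getters.
; On BeginPlay it sets its pickup type, waits two seconds, then calls a multicast initializer if spawned as a level pickup.
; That initializer scans DT_ResourcesLibrary for the matching resource type, copying its titles, icon and rarity.
; It passes these and the amount to the overview marker widget.
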(event `self.ReceiveBeginPlay`
  ;[1 1 1] EVENT BEGIN PLAY
  (`parent.ReceiveBeginPlay`)
  ;;[1 1 1] Set pickup as firearm pickup
  (`self.SetPickupType` "NewEnumerator7")
  ;;[1 1 1] Delay 2 sec
  (`KismetSystemLibrary.Delay` 2.0)
  ;;[1 0.2552 0.2552] CHECK: SpawnAsLevelPickup
  (if (`self.SpawnAsLevelPickup`)
    (`self.MulticastInitializeResourcePickup`)))

(event `MulticastInitializeResourcePickup`
  ;[1 1 1] INITIALIZE RESOURCE PICKUP
  ;;[1 1 1] Getting values from resources lib
  (bind _outrownames (`DataTableFunctionLibrary.GetDataTableRowNames` "/Game/CHARACTER_SYSTEM_V2/Blueprints/InventorySystem/DT_ResourcesLibrary.DT_ResourcesLibrary"))
  (for _array_element _outrownames
    (bind _returnvalue (`|GetDataTableRow` "/Game/CHARACTER_SYSTEM_V2/Blueprints/InventorySystem/DT_ResourcesLibrary.DT_ResourcesLibrary" _array_element)
      (:`then`
        (bind (_resourcetype _typetitle _titletext _icon _desctext _raritytype) (break `/Game/CHARACTER_SYSTEM_V2/Blueprints/DATA/STR/STR_ResourceLibDesc` _returnvalue))
        (if (`|EnumEquality` _resourcetype (`self.ResourceType`))
          (set `self.Type Title` _typetitle)
          (set `self.Title` _titletext)
          (set `self.Icon` _icon)
          (set `self.Rarity` _raritytype)))))
  ;;[1 0.6824 0] TO WBP_InteractiveObjectMarkerView
  (bind _aswbp_interactive_object_marker_overview_pickup (cast `/Game/CHARACTER_SYSTEM_V2/Blueprints/PlayerHUD/InteractiveObject/WBP_InteractiveObjectMarkerOverviewPickup` (`WidgetComponent.GetWidget` (`self.InteractiveObjectMarkerOverviewPickup`))))
  (`/Game/CHARACTER_SYSTEM_V2/Blueprints/PlayerHUD/InteractiveObject/WBP_InteractiveObjectMarkerOverviewPickup.InitializeOverviewMarker` _aswbp_interactive_object_marker_overview_pickup (`self.Title`) (`self.Type Title`) "" (`self.Rarity`) (`self.RecourceAmount`) "NewEnumerator7" (`self.Icon`)))

(fn `GetRecourceAmount`
  (returns (RecourceAmount :type Integer))
  (return (`self.RecourceAmount`)))

(fn `GetResourceType`
  (returns (ResourceType :type "/Game/CHARACTER_SYSTEM_V2/Blueprints/DATA/E/Inventory/E_ResourceType Enum"))
  (return (`self.ResourceType`)))

(fn `UserConstructionScript`
  (`parent.UserConstructionScript`))