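; Firearm pickup base that holds a real firearm actor and shows its details on an overview marker widget.
; When flagged as a level pickup, after a short BeginPlay delay the server or standalone game spawns the firearm with default attachments and ammo.
; Multicast events then attach it to the weapon mesh, read title, icon, rarity, type and ammo through interface messages, and fill the marker with weapon category labels.
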(event `self.ReceiveBeginPlay`
  ;[1 1 1] EVENT BEGIN PLAY
  (`parent.ReceiveBeginPlay`)
  ;;[1 1 1] Set pickup as firearm pickup
  (`self.SetPickupType` "NewEnumerator0")
  ;;[1 1 1] Delay 2 sec
  (`KismetSystemLibrary.Delay` 2.0)
  ;;[1 0.2552 0.2552] CHECK: SpawnAsLevelPickup
  (if (`self.SpawnAsLevelPickup`)
    ;;[1 0.2552 0.2552] CHECK: IsStandalone or server
    (if (or (`KismetSystemLibrary.IsStandalone`) (`KismetSystemLibrary.IsServer`))
      (`self.ServerSpawnFirearmInPickup`))))

(event `ServerSpawnFirearmInPickup`
  ;[1 1 1] SPAWN FIREARM IN PICKUP
  ;;[1 1 1] Spawn Weapon In Pickup
  (bind _returnvalue (`|SpawnActorFromClass` (`self.FirearmClass`) (`SceneComponent.GetRelativeTransform` (`self.DefaultSceneRoot`)) "AlwaysSpawn" "OverrideRootScale" self null))
  ;;[1 1 1] Check Valid actor as firearm
  (`/Engine/EditorBlueprintResources/StandardMacros.IsValid` _returnvalue
    (:`Is Valid`
      (bind _output_get (set `self.FirearmActor` _returnvalue))
      (cast `/Game/CHARACTER_SYSTEM_V2/Blueprints/FirearmSystem/BP_FirearmActorCommon` _output_get)
      ;;[1 1 1] Initialize default attachments in spawned firearm
      (message `/Game/CHARACTER_SYSTEM_V2/Blueprints/BI/BI_InventoryItemFirearm.InventoryItemFirearmSetDefaultAttachments` (`self.FirearmActor`))
      (message `/Game/CHARACTER_SYSTEM_V2/Blueprints/BI/BI_InventoryItemCommon.InventoryItemCommonSetAmmoCount` (`self.FirearmActor`) 0 true)
      ;;[1 1 1] Attach & Initialize spawned actor
      (`self.MulticastAttachFirearmActor`)
      (`self.MulticastInitializeFirearmPickup`))))

(event `MulticastAttachFirearmActor`
  ;[1 1 1] ATTACH
  (`/Engine/EditorBlueprintResources/StandardMacros.IsValid` (`self.FirearmActor`)
    (:`Is Valid`
      (`self.K2_AttachToComponent` (`self.FirearmActor`) (`self.WeaponMesh`) "None" "SnapToTarget" "SnapToTarget" "KeepRelative" true)
      (`self.K2_SetActorRelativeRotation` (`self.FirearmActor`) (struct :`Yaw` -90.0) false false))))

(event `MulticastInitializeFirearmPickup`
  ;[1 1 1] INITIALIZE FIREARM PICKUP
  ;;[1 1 1] Getting values from actor across BI
  (bind _icon (message `/Game/CHARACTER_SYSTEM_V2/Blueprints/BI/BI_InventoryItemCommon.GetInventoryItemCommonIconWeaponModule` (`self.FirearmActor`)))
  (set `self.IconWeaponModule` _icon)
  (bind _title (message `/Game/CHARACTER_SYSTEM_V2/Blueprints/BI/BI_InventoryItemCommon.GetInventoryItemCommonTitle` (`self.FirearmActor`)))
  (set `self.Title` _title)
  (bind _raritytype (message `/Game/CHARACTER_SYSTEM_V2/Blueprints/BI/BI_InventoryItemCommon.GetInventoryItemCommonRarityType` (`self.FirearmActor`)))
  (set `self.RarityType` _raritytype)
  (bind _firearmtype (message `/Game/CHARACTER_SYSTEM_V2/Blueprints/BI/BI_InventoryItemFirearm.GetInventoryItemFirearmType` (`self.FirearmActor`)))
  (set `self.FirearmType` _firearmtype)
  (bind _ammocount (message `/Game/CHARACTER_SYSTEM_V2/Blueprints/BI/BI_InventoryItemCommon.GetInventoryItemCommonAmmoCount` (`self.FirearmActor`)))
  (set `self.AmmoCount` _ammocount)
  ;;[1 0.6824 0] TO WBP_InteractiveObjectMarkerView
  (bind _aswbp_interactive_object_marker_overview_pickup (cast `/Game/CHARACTER_SYSTEM_V2/Blueprints/PlayerHUD/InteractiveObject/WBP_InteractiveObjectMarkerOverviewPickup` (`WidgetComponent.GetWidget` (`self.InteractiveObjectMarkerOverviewPickup`))))
  (`/Game/CHARACTER_SYSTEM_V2/Blueprints/PlayerHUD/InteractiveObject/WBP_InteractiveObjectMarkerOverviewPickup.InitializeOverviewMarker` _aswbp_interactive_object_marker_overview_pickup (`self.Title`) (select `/Game/CHARACTER_SYSTEM_V2/Blueprints/DATA/E/E_FirearmType` (`self.FirearmType`) :`NewEnumerator0` "PRIMARY WEAPON" :`NewEnumerator1` "PRIMARY WEAPON" :`NewEnumerator2` "PRIMARY WEAPON" :`NewEnumerator3` "PRIMARY WEAPON" :`NewEnumerator4` "PRIMARY WEAPON" :`NewEnumerator5` "PRIMARY WEAPON" :`NewEnumerator6` "SECONDARY WEAPON" :!type "Text") (select `/Game/CHARACTER_SYSTEM_V2/Blueprints/DATA/E/E_FirearmType` (`self.FirearmType`) :`NewEnumerator0` "ASSAULT RIFLE" :`NewEnumerator1` "SMG" :`NewEnumerator2` "SHOTGUN" :`NewEnumerator3` "LMG" :`NewEnumerator4` "MARKSMAN RIFLE" :`NewEnumerator5` "SNIPER RIFLE" :`NewEnumerator6` "PISTOL" :!type "Text") (`self.RarityType`) (`self.AmmoCount`) "NewEnumerator0" (`self.IconWeaponModule`)))

(fn `GetFirearmActor`
  (returns (FirearmActor :type "Actor Object Reference"))
  (return (`self.FirearmActor`)))

(fn `UserConstructionScript`
  (`parent.UserConstructionScript`))