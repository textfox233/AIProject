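; Backpack menu overlay actor that shows a preview of a resource pickup through a 2D scene capture.
; An update event, fed by the backpack menu, scans DT_ResourcesLibrary for rows matching the given resource type and sets the child actor to that row's pickup class.
; The capture's show-only list is limited to this actor and its child actors, and is refreshed at BeginPlay and after each swap.
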(event `self.ReceiveBeginPlay`
  (`SceneCaptureComponent.ShowOnlyActorComponents` (`self.SceneCaptureComponent2D`) self true))

(event `ClientUpdateResourceActor`
  (params (RresourceType :type "/Game/CHARACTER_SYSTEM_V2/Blueprints/DATA/E/Inventory/E_ResourceType Enum" :default "NewEnumerator0"))
  ;[1 0.1179 0] INPUT FROM BACKPACK MENU INVENTORY WEAPONS
  (bind _outrownames (`DataTableFunctionLibrary.GetDataTableRowNames` "/Game/CHARACTER_SYSTEM_V2/Blueprints/InventorySystem/DT_ResourcesLibrary.DT_ResourcesLibrary"))
  (for _array_element _outrownames
    (bind _returnvalue (`|GetDataTableRow` "/Game/CHARACTER_SYSTEM_V2/Blueprints/InventorySystem/DT_ResourcesLibrary.DT_ResourcesLibrary" _array_element)
      (:`then`
        (bind (_resourcetype _typetitle _titletext _icon _desctext _raritytype _pickupclass) (break `/Game/CHARACTER_SYSTEM_V2/Blueprints/DATA/STR/STR_ResourceLibDesc` _returnvalue))
        (if (`|EnumEquality` _resourcetype RresourceType)
          (`ChildActorComponent.SetChildActorClass` (`self.ResourceActor`) _pickupclass)
          (`SceneCaptureComponent.ShowOnlyActorComponents` (`self.SceneCaptureComponent2D`) self true))))))

(fn `UserConstructionScript`)