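; Blueprint function library of shared debug helpers for the character system.
; LogAdvanced builds one tagged line from game time, server, dedicated-server and standalone flags, object title, logic tag and message, then prints it with screen output off.
; Its PrintToLog input is stored but never visibly wired into the print, and the Warning function is an empty stub.
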(fn `LogAdvanced`
  (params (PrintToLog :type Boolean) (Object :type "Object Object Reference") (ObjectTitle :type String) (LogicTag :type String) (LogMessage :type String))
  (locals (InputObject :type "Object Object Reference") (InputPrintToLog :type Boolean) (InputObjectTitle :type String) (InputLogicTag :type String) (InputLogMessage :type String))
  ;[1 1 1] Initialize input values
  (set `local.InputPrintToLog` PrintToLog)
  (set `local.InputObject` Object)
  (set `local.InputObjectTitle` ObjectTitle)
  (set `local.InputLogicTag` LogicTag)
  (set `local.InputLogMessage` LogMessage)
  (`KismetSystemLibrary.PrintString` (`local.InputObject`) (`KismetStringLibrary.Concat_StrStr` (`KismetStringLibrary.Concat_StrStr` "[" (`KismetStringLibrary.Conv_DoubleToString` (`KismetSystemLibrary.GetGameTimeInSeconds` (`local.InputObject`))) "]") " " (`KismetStringLibrary.Concat_StrStr` "[" "IsS = " (`KismetStringLibrary.Conv_IntToString` (select `bool` (`KismetSystemLibrary.IsServer` (`local.InputObject`)) :`true` 1)) "; " "IsDS = " (`KismetStringLibrary.Conv_IntToString` (select `bool` (`KismetSystemLibrary.IsDedicatedServer` (`local.InputObject`)) :`true` 1)) "; " "IsSl = " (`KismetStringLibrary.Conv_IntToString` (select `bool` (`KismetSystemLibrary.IsStandalone` (`local.InputObject`)) :`true` 1)) "]") " " (`KismetStringLibrary.Concat_StrStr` "[" (`local.InputObjectTitle`) "]") " " (`KismetStringLibrary.Concat_StrStr` "[" (`local.InputLogicTag`) "]") ": " (`local.InputLogMessage`)) false true (struct :`R` 1.0 :`G` 0.008376 :`A` 1.0) 5.0))

(fn `Warning`)