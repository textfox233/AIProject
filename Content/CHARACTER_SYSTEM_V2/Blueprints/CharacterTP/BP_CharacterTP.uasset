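; Third-person character Blueprint that adds body animation, weapon attachment and camera behavior on top of its parent character.
; Parent server events multicast to the mesh AnimInstance and attach firearms or equipment to hand sockets, switching hands for reloads and stowing during cover moves.
; Client events drive firearm VFX and hide mesh and firearm when scoped.
; The TPCamera graph maps character state to PlayerCameraTP presets and re-parents the spring arm during cover actions.
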(event `self.ReceiveBeginPlay`
  ;[1 1 1] EVENT BEGIN PLAY
  (`parent.ReceiveBeginPlay`)
  (`self.ClientInitTPCameraAdvancedOnSpawn`))

(event `self.ReceiveTick`
  (params (DeltaSeconds :type "Float (single-precision)"))
  ;[1 1 1] EVENT TICK
  (`parent.ReceiveTick` DeltaSeconds))

(event `self.ServerAttachFirearm`
  (params (FirearmActor :type "Actor Object Reference"))
  ;[1 1 1] HANDLE ATTACH & INITIALIZE FIREARM
  ;;[1 1 1] Handle Attach Firearm
  ;;;[0.1778 0 1] PARENT INPUT
  (set `self.CurrentTPFirearm` FirearmActor)
  (bind _asbp_firearm_actor_common (cast `/Game/CHARACTER_SYSTEM_V2/Blueprints/FirearmSystem/BP_FirearmActorCommon` (`self.CurrentTPFirearm`)))
  (`self.MulticastInitBaseAnimBP` (`/Game/CHARACTER_SYSTEM_V2/Blueprints/FirearmSystem/BP_FirearmActorCommon.FirearmTag` _asbp_firearm_actor_common))
  (`self.ServerAttachCurrentFirearm`)
  ;;;[1 0.6824 0] TO PLAYER CAMERA TP
  (`/Game/CHARACTER_SYSTEM_V2/Blueprints/PlayerCameraTP/AC_PlayerCameraTP.ClientUpdateAimTime` (`self.PlayerCameraTP`) (`/Game/CHARACTER_SYSTEM_V2/Blueprints/FirearmSystem/BP_FirearmActorCommon.GetAimTime` _asbp_firearm_actor_common)))

(event `MulticastInitBaseAnimBP`
  (params (FirearmTag :type Name))
  ;[1 1 1] HANDLE ATTACH & INITIALIZE FIREARM
  ;;[1 1 1] Initialize Base Anim BP
  ;;;[1 0.6824 0] BI TO MESH ANIM INSTANCE
  (message `/Game/CHARACTER_SYSTEM_V2/Blueprints/BI/BI_CharacterAnim.CharacterAnimIntializeFirearm` (`SkeletalMeshComponent.GetAnimInstance` (`self.Mesh`)) FirearmTag))

(event `ServerAttachCurrentFirearm`
  ;[1 1 1] HANDLE ATTACH & INITIALIZE FIREARM
  ;;[1 1 1] ServerAttachCurrentFirearm
  (bind _asbp_firearm_actor_common (cast `/Game/CHARACTER_SYSTEM_V2/Blueprints/FirearmSystem/BP_FirearmActorCommon` (`self.CurrentTPFirearm`)))
  (if (`/Game/CHARACTER_SYSTEM_V2/Blueprints/FirearmSystem/BP_FirearmActorCommon.GetUseExtraReload` _asbp_firearm_actor_common)
    (switch `/Game/CHARACTER_SYSTEM_V2/Blueprints/DATA/E/E_GL_FirearmHoldingHand` (`/Game/CHARACTER_SYSTEM_V2/Blueprints/FirearmSystem/BP_FirearmActorCommon.GetHoldingHandExtraReload` _asbp_firearm_actor_common)
      (:`NewEnumerator0`
        (`self.MulticastAttachCurrentFirearmToMesh` true (`self.CurrentTPFirearm`)))
      (:`NewEnumerator1`
        (`self.MulticastAttachCurrentFirearmToMesh` false (`self.CurrentTPFirearm`))))
    (else
      (`self.MulticastAttachCurrentFirearmToMesh` true (`self.CurrentTPFirearm`)))))

(event `MulticastAttachCurrentFirearmToMesh`
  (params (AttachToRightHand :type Boolean) (FirearmActor :type "Actor Object Reference"))
  ;[1 1 1] HANDLE ATTACH & INITIALIZE FIREARM
  ;;[1 1 1] MulticastAttachCurrentFirearmToMesh
  (`/Engine/EditorBlueprintResources/StandardMacros.IsValid` FirearmActor
    (:`Is Valid`
      (`self.K2_AttachToComponent` FirearmActor (`self.Mesh`) (select `bool` AttachToRightHand :`false` (`self.FirearmLHandAttachBone`) :`true` (`self.FirearmRHandAttachBone`)) "SnapToTarget" "SnapToTarget" "KeepRelative" true))))

(event `self.ServerHandleFirearmEvent`
  (params (FirearmEventType :type "/Game/CHARACTER_SYSTEM_V2/Blueprints/DATA/E/E_GL_FirearmEventType Enum" :default "NewEnumerator0"))
  ;[1 1 1] HANDLE FIREARM EVENT
  ;;[1 1 1] Server Handle Firearm Event
  ;;;[0.1778 0 1] PARENT INPUT
  (`self.ClientHandleChildFirearmEvent` FirearmEventType)
  (`self.MulticastHandleChildFirearmEvent` FirearmEventType)
  ;;;[1 0.6824 0] TO FIREARM ACTOR COMMON
  (bind _asbp_firearm_actor_common (cast `/Game/CHARACTER_SYSTEM_V2/Blueprints/FirearmSystem/BP_FirearmActorCommon` (`self.CurrentTPFirearm`)))
  (`/Game/CHARACTER_SYSTEM_V2/Blueprints/FirearmSystem/BP_FirearmActorCommon.ServerHandleTPFirearmEvent` _asbp_firearm_actor_common FirearmEventType)
  (switch `/Game/CHARACTER_SYSTEM_V2/Blueprints/DATA/E/E_GL_FirearmEventType` FirearmEventType
    (:`NewEnumerator2`
      (`self.ServerHandleChildMainReloadStart`))
    (:`NewEnumerator3`
      (`self.ServerHandleChildMainReloadFinish`))))

(event `ClientHandleChildFirearmEvent`
  (params (FirearmEventType :type "/Game/CHARACTER_SYSTEM_V2/Blueprints/DATA/E/E_GL_FirearmEventType Enum" :default "NewEnumerator0"))
  ;[1 1 1] HANDLE FIREARM EVENT
  ;;[1 1 1] Client Handle Firearm Event
  (switch `/Game/CHARACTER_SYSTEM_V2/Blueprints/DATA/E/E_GL_FirearmEventType` FirearmEventType
    (:`NewEnumerator0`
      (bind _asbp_firearm_actor_common (cast `/Game/CHARACTER_SYSTEM_V2/Blueprints/FirearmSystem/BP_FirearmActorCommon` (`self.CurrentTPFirearm`)))
      ;;;[1 0.6824 0] TO FIREARM VFX CONTROLLER
      (`/Game/CHARACTER_SYSTEM_V2/Blueprints/FirearmSystem/AC_FirearmVFXController.ClientCreateVFXOnShotTP` (`self.GetFirearmVFXController`) false (`/Game/CHARACTER_SYSTEM_V2/Blueprints/FirearmSystem/BP_FirearmActorCommon.FirearmMesh` _asbp_firearm_actor_common)))))

(event `MulticastHandleChildFirearmEvent`
  (params (FirearmEventType :type "/Game/CHARACTER_SYSTEM_V2/Blueprints/DATA/E/E_GL_FirearmEventType Enum" :default "NewEnumerator0"))
  ;[1 1 1] HANDLE FIREARM EVENT
  ;;[1 1 1] Multicast Handle Firearm Event
  ;;;[1 0.6824 0] BI TO MESH ANIM INSTANCE
  (message `/Game/CHARACTER_SYSTEM_V2/Blueprints/BI/BI_CharacterAnim.CharacterAnimHandleFirearmEvent` (`SkeletalMeshComponent.GetAnimInstance` (`self.Mesh`)) FirearmEventType))

(event `ServerHandleChildMainReloadStart`
  ;[1 1 1] HANDLE FIREARM EVENT
  ;;[1 1 1] Server Main Reload Start
  (bind _asbp_firearm_actor_common (cast `/Game/CHARACTER_SYSTEM_V2/Blueprints/FirearmSystem/BP_FirearmActorCommon` (`self.CurrentTPFirearm`)))
  (`self.MulticastAttachCurrentFirearmToMesh` (select `/Game/CHARACTER_SYSTEM_V2/Blueprints/DATA/E/E_GL_FirearmHoldingHand` (`/Game/CHARACTER_SYSTEM_V2/Blueprints/FirearmSystem/BP_FirearmActorCommon.GetHoldingHandMainReload` _asbp_firearm_actor_common) :`NewEnumerator0` true) (`self.CurrentTPFirearm`)))

(event `ServerHandleChildMainReloadFinish`
  ;[1 1 1] HANDLE FIREARM EVENT
  ;;[1 1 1] Server Main Reload Finish
  (bind _asbp_firearm_actor_common (cast `/Game/CHARACTER_SYSTEM_V2/Blueprints/FirearmSystem/BP_FirearmActorCommon` (`self.CurrentTPFirearm`)))
  (if (`/Game/CHARACTER_SYSTEM_V2/Blueprints/FirearmSystem/BP_FirearmActorCommon.GetUseExtraReload` _asbp_firearm_actor_common)
    (switch `/Game/CHARACTER_SYSTEM_V2/Blueprints/DATA/E/E_GL_FirearmHoldingHand` (`/Game/CHARACTER_SYSTEM_V2/Blueprints/FirearmSystem/BP_FirearmActorCommon.GetHoldingHandExtraReload` _asbp_firearm_actor_common)
      (:`NewEnumerator0`
        (`self.MulticastAttachCurrentFirearmToMesh` true (`self.CurrentTPFirearm`)))
      (:`NewEnumerator1`
        (`self.MulticastAttachCurrentFirearmToMesh` false (`self.CurrentTPFirearm`))))
    (else
      (`self.MulticastAttachCurrentFirearmToMesh` true (`self.CurrentTPFirearm`)))))

(event `self.ClientHandleChildSingleTraceCreated`
  (params (SingleTraceDesc :type "/Game/CHARACTER_SYSTEM_V2/Blueprints/DATA/STR/STR_FirearmHitScanDesc Structure"))
  ;[1 1 1] HANDLE CREATED HITSCAN
  ;;[1 1 1] Single Trace
  ;;;[0.1778 0 1] PARENT INPUT
  (bind _asbp_firearm_actor_common (cast `/Game/CHARACTER_SYSTEM_V2/Blueprints/FirearmSystem/BP_FirearmActorCommon` (`self.CurrentTPFirearm`)))
  ;;;[1 0.6824 0] TO FIREARM VFX CONTROLLER
  (`/Game/CHARACTER_SYSTEM_V2/Blueprints/FirearmSystem/AC_FirearmVFXController.ClientStartPlayVFXOnCreateSingleHitScanTP` (`self.GetFirearmVFXController`) SingleTraceDesc (`/Game/CHARACTER_SYSTEM_V2/Blueprints/FirearmSystem/BP_FirearmActorCommon.FirearmMesh` _asbp_firearm_actor_common) false))

(event `self.ClientHandleChildMultiTraceCreated`
  (params (MultiTraceDesc :type "Array of /Game/CHARACTER_SYSTEM_V2/Blueprints/DATA/STR/STR_FirearmHitScanDesc Structure (by ref)"))
  ;[1 1 1] HANDLE CREATED HITSCAN
  ;;[1 1 1] Multi Trace
  ;;;[0.1778 0 1] PARENT INPUT
  (bind _asbp_firearm_actor_common (cast `/Game/CHARACTER_SYSTEM_V2/Blueprints/FirearmSystem/BP_FirearmActorCommon` (`self.CurrentTPFirearm`)))
  ;;;[1 0.6824 0] TO FIREARM VFX CONTROLLER
  (`/Game/CHARACTER_SYSTEM_V2/Blueprints/FirearmSystem/AC_FirearmVFXController.ClientStartPlayVFXOnCreateMultiHitScanTP` (`self.GetFirearmVFXController`) MultiTraceDesc (`/Game/CHARACTER_SYSTEM_V2/Blueprints/FirearmSystem/BP_FirearmActorCommon.FirearmMesh` _asbp_firearm_actor_common) false))

(event `self.ClientHandleChildShellOnExtraReload`
  ;[1 1 1] HANDLE SHELL ON EXTRA RELOAD
  ;;[0.1778 0 1] PARENT INPUT
  (bind _asbp_firearm_actor_common (cast `/Game/CHARACTER_SYSTEM_V2/Blueprints/FirearmSystem/BP_FirearmActorCommon` (`self.CurrentTPFirearm`)))
  ;;[1 0.6824 0] TO FIREARM VFX CONTROLLER
  (`/Game/CHARACTER_SYSTEM_V2/Blueprints/FirearmSystem/AC_FirearmVFXController.ClientCreateShellOnExtraReloadForTP` (`self.GetFirearmVFXController`) (`/Game/CHARACTER_SYSTEM_V2/Blueprints/FirearmSystem/BP_FirearmActorCommon.FirearmMesh` _asbp_firearm_actor_common) false))

(event `self.ServerClipEndFollow`
  ;[1 1 1] HADNLE CLIP OBJ EVENTS
  ;;[1 1 1] Server Clip End Follow
  ;;;[0.1778 0 1] PARENT INPUT
  ;;;[1 0.6824 0] TO FIREARM ACTOR COMMON
  (bind _asbp_firearm_actor_common (cast `/Game/CHARACTER_SYSTEM_V2/Blueprints/FirearmSystem/BP_FirearmActorCommon` (`self.CurrentTPFirearm`)))
  (`/Game/CHARACTER_SYSTEM_V2/Blueprints/FirearmSystem/BP_FirearmActorCommon.ServerHandleClipEndFollowTP` _asbp_firearm_actor_common))

(event `self.ServerClipInHand`
  ;[1 1 1] HADNLE CLIP OBJ EVENTS
  ;;[1 1 1] Server Clip In Hand
  ;;;[0.1778 0 1] PARENT INPUT
  ;;;[1 0.6824 0] TO FIREARM ACTOR COMMON
  (bind _asbp_firearm_actor_common (cast `/Game/CHARACTER_SYSTEM_V2/Blueprints/FirearmSystem/BP_FirearmActorCommon` (`self.CurrentTPFirearm`)))
  (`/Game/CHARACTER_SYSTEM_V2/Blueprints/FirearmSystem/BP_FirearmActorCommon.ServerHandleClipInHandTP` _asbp_firearm_actor_common))

(event `MulticastChildHandleSwitchEquipmentDown`
  (params (SwitchTime :type "Float (double-precision)"))
  ;[1 1 1] HANDLE SWITCH WEAPON
  ;;[1 1 1] ServerHandleSwitchEquipmentDown
  ;;;[1 0.6824 0] BI TO MESH ANIM INSTANCE
  (message `/Game/CHARACTER_SYSTEM_V2/Blueprints/BI/BI_CharacterAnim.CharacterAnimHandleSwitchEquipmentDown` (`SkeletalMeshComponent.GetAnimInstance` (`self.Mesh`)) SwitchTime))

(event `self.ServerHandleSwitchFirearmDown`
  (params (SwitchTime :type "Float (double-precision)"))
  ;[1 1 1] HANDLE SWITCH WEAPON
  ;;[1 1 1] ServerHandleSwitchFirearmDown
  ;;;[0.1778 0 1] PARENT INPUT
  (`self.MulticastChildHandleSwitchFirearmDown` SwitchTime))

(event `MulticastChildHandleSwitchFirearmDown`
  (params (SwitchTime :type "Float (double-precision)"))
  ;[1 1 1] HANDLE SWITCH WEAPON
  ;;[1 1 1] ServerHandleSwitchFirearmDown
  ;;;[1 0.6824 0] BI TO MESH ANIM INSTANCE
  (message `/Game/CHARACTER_SYSTEM_V2/Blueprints/BI/BI_CharacterAnim.CharacterAnimHandleSwithFirearmDown` (`SkeletalMeshComponent.GetAnimInstance` (`self.Mesh`)) SwitchTime))

(event `MulticastChildHandleSwitchMeleeDown`
  (params (SwitchTime :type "Float (double-precision)"))
  ;[1 1 1] HANDLE SWITCH WEAPON
  ;;[1 1 1] ServerHandleSwitchMeleeDown
  ;;;[1 0.6824 0] BI TO MESH ANIM INSTANCE
  (message `/Game/CHARACTER_SYSTEM_V2/Blueprints/BI/BI_CharacterAnim.CharacterAnimHandleSwitchMeleeDown` (`SkeletalMeshComponent.GetAnimInstance` (`self.Mesh`)) SwitchTime))

(event `MulticastChildHandleSwitchUnarmedDown`
  (params (SwitchTime :type "Float (double-precision)"))
  ;[1 1 1] HANDLE SWITCH WEAPON
  ;;[1 1 1] ServerHandleSwitchUnarmedDown
  ;;;[1 0.6824 0] BI TO MESH ANIM INSTANCE
  (message `/Game/CHARACTER_SYSTEM_V2/Blueprints/BI/BI_CharacterAnim.CharacterAnimHandleSwitchUnarmedDown` (`SkeletalMeshComponent.GetAnimInstance` (`self.Mesh`)) SwitchTime))

(event `self.ServerHandleSwitchEquipmentDown`
  (params (SwitchTime :type "Float (double-precision)"))
  ;[1 1 1] HANDLE SWITCH WEAPON
  ;;[1 1 1] ServerHandleSwitchEquipmentDown
  ;;;[0.1778 0 1] PARENT INPUT
  (`self.MulticastChildHandleSwitchEquipmentDown` SwitchTime))

(event `self.ServerHandleSwitchMeleeDown`
  (params (SwitchTime :type "Float (double-precision)"))
  ;[1 1 1] HANDLE SWITCH WEAPON
  ;;[1 1 1] ServerHandleSwitchMeleeDown
  ;;;[0.1778 0 1] PARENT INPUT
  (`self.MulticastChildHandleSwitchMeleeDown` SwitchTime))

(event `self.ServerHandleSwitchUnarmedDown`
  (params (SwitchTime :type "Float (double-precision)"))
  ;[1 1 1] HANDLE SWITCH WEAPON
  ;;[1 1 1] ServerHandleSwitchUnarmedDown
  ;;;[0.1778 0 1] PARENT INPUT
  (`self.MulticastChildHandleSwitchUnarmedDown` SwitchTime))

(event `self.ServerHandleSwitchMeleeUp`
  (params (SwitchTime :type "Float (double-precision)"))
  ;[1 1 1] HANDLE SWITCH WEAPON
  ;;[1 1 1] ServerHandleSwitchMeleeUp
  ;;;[0.1778 0 1] PARENT INPUT
  (`self.MulticastChildHandleSwitchMeleeUp` SwitchTime))

(event `ServerSwitchWeaponFirearmUp_1`
  (params (SwitchFirearmUpTime :type "Float (double-precision)"))
  ;[1 1 1] HANDLE SWITCH WEAPON
  ;;[1 1 1] ServerHandleSwitchFirearmUp
  ;;;[0.1778 0 1] PARENT INPUT
  (`self.MulticastChildHandleSwitchFirearmUp ` SwitchFirearmUpTime))

(event `self.ServerHandleSwitchEquipmentUp`
  (params (SwitchTime :type "Float (double-precision)"))
  ;[1 1 1] HANDLE SWITCH WEAPON
  ;;[1 1 1] ServerHandleSwitchEquipmentUp
  ;;;[0.1778 0 1] PARENT INPUT
  (`self.MulticastChildHandleSwitchEquipmentUp` SwitchTime))

(event `self.ServerHandleSwitchUnarmedUp `
  (params (SwitchTime :type "Float (double-precision)"))
  ;[1 1 1] HANDLE SWITCH WEAPON
  ;;[1 1 1] ServerHandleSwitchUnarmedUp
  ;;;[0.1778 0 1] PARENT INPUT
  (`self.MulticastChildHandleSwitchUnarmedUp ` SwitchTime))

(event `MulticastChildHandleSwitchEquipmentUp`
  (params (SwitchTime :type "Float (double-precision)"))
  ;[1 1 1] HANDLE SWITCH WEAPON
  ;;[1 1 1] ServerHandleSwitchEquipmentUp
  ;;;[1 0.6824 0] BI TO MESH ANIM INSTANCE
  (message `/Game/CHARACTER_SYSTEM_V2/Blueprints/BI/BI_CharacterAnim.CharacterAnimHandleSwitchEquipmentUp` (`SkeletalMeshComponent.GetAnimInstance` (`self.Mesh`)) SwitchTime))

(event `MulticastChildHandleSwitchMeleeUp`
  (params (SwitchTime :type "Float (double-precision)"))
  ;[1 1 1] HANDLE SWITCH WEAPON
  ;;[1 1 1] ServerHandleSwitchMeleeUp
  ;;;[1 0.6824 0] BI TO MESH ANIM INSTANCE
  (message `/Game/CHARACTER_SYSTEM_V2/Blueprints/BI/BI_CharacterAnim.CharacterAnimHandleSwitchMeleeUp` (`SkeletalMeshComponent.GetAnimInstance` (`self.Mesh`)) SwitchTime))

(event `MulticastChildHandleSwitchFirearmUp`
  (params (SwitchTime :type "Float (double-precision)"))
  ;[1 1 1] HANDLE SWITCH WEAPON
  ;;[1 1 1] ServerHandleSwitchFirearmUp
  ;;;[1 0.6824 0] BI TO MESH ANIM INSTANCE
  (message `/Game/CHARACTER_SYSTEM_V2/Blueprints/BI/BI_CharacterAnim.CharacterAnimHandleSwithFirearmUp` (`SkeletalMeshComponent.GetAnimInstance` (`self.Mesh`)) SwitchTime))

(event `MulticastChildHandleSwitchUnarmedUp`
  (params (SwitchTime :type "Float (double-precision)"))
  ;[1 1 1] HANDLE SWITCH WEAPON
  ;;[1 1 1] ServerHandleSwitchUnarmedUp
  ;;;[1 0.6824 0] BI TO MESH ANIM INSTANCE
  (message `/Game/CHARACTER_SYSTEM_V2/Blueprints/BI/BI_CharacterAnim.CharacterAnimHandleSwitchUnarmedUp ` (`SkeletalMeshComponent.GetAnimInstance` (`self.Mesh`)) SwitchTime))

(event `self.ServerAttachEquipment`
  (params (EquipActor :type "Actor Object Reference"))
  ;[1 1 1] HANDLE ATTACH EQUIPMENT
  ;;[0.1778 0 1] PARENT INPUT
  (set `self.CurrentTPEquip` EquipActor)
  (`self.MulticastHandleAttachEquipment` (`self.CurrentTPEquip`)))

(event `MulticastHandleAttachEquipment`
  (params (EquipActor :type "Actor Object Reference"))
  ;[1 1 1] HANDLE ATTACH EQUIPMENT
  (`/Engine/EditorBlueprintResources/StandardMacros.IsValid` EquipActor
    (:`Is Valid`
      (`self.K2_AttachToComponent` EquipActor (`self.Mesh`) (`self.FirearmRHandAttachBone`) "SnapToTarget" "SnapToTarget" "KeepRelative" true))))

(event `self.ServerChangedMainState`
  (params (MainCharacterState :type "/Game/CHARACTER_SYSTEM_V2/Blueprints/DATA/E/E_CharacterMainState Enum" :default "NewEnumerator0"))
  ;[1 1 1] HANDLE CHANGING MAIN STATE
  ;;[0.1778 0 1] PARENT INPUT EVENT
  (`self.ClientDifineNewCameraPreset` MainCharacterState)
  (`self.ClientSwitchAttachignTPCamera` MainCharacterState))

(event `self.ClientHandleChildScopetOnOff`
  (params (ScopeON :type Boolean))
  ;[1 1 1] HANDLE SCOPER ON / OFF
  ;;[0.1778 0 1] PARENT INPUT EVENT
  (if ScopeON
    ;;[1 1 1] Hide TP Mesh
    (`SceneComponent.SetHiddenInGame` (`self.Mesh`) true false)
    ;;[1 1 1] Hide TP Firearm
    (`self.SetActorHiddenInGame` (`self.CurrentTPFirearm`) true)
    (bind _asbp_firearm_actor_common (cast `/Game/CHARACTER_SYSTEM_V2/Blueprints/FirearmSystem/BP_FirearmActorCommon` (`self.CurrentTPFirearm`)))
    (`PrimitiveComponent.SetCastHiddenShadow` (`/Game/CHARACTER_SYSTEM_V2/Blueprints/FirearmSystem/BP_FirearmActorCommon.FirearmMesh` _asbp_firearm_actor_common) true)
    (else
      ;;[1 1 1] Set TP Camera Preset
      (`self.ClientDifineNewCameraPreset` (`self.GetMainCharacterState`))
      ;;[1 1 1] Show TP Mesh
      (`SceneComponent.SetHiddenInGame` (`self.Mesh`) false false)
      ;;[1 1 1] Show TP Firearm
      (`self.SetActorHiddenInGame` (`self.CurrentTPFirearm`) false)
      (bind _asbp_firearm_actor_common_2 (cast `/Game/CHARACTER_SYSTEM_V2/Blueprints/FirearmSystem/BP_FirearmActorCommon` (`self.CurrentTPFirearm`)))
      (`PrimitiveComponent.SetCastHiddenShadow` (`/Game/CHARACTER_SYSTEM_V2/Blueprints/FirearmSystem/BP_FirearmActorCommon.FirearmMesh` _asbp_firearm_actor_common_2) false))))

(event `MulticastHandleChildUseEquipmentOn`
  (params (EquipmentUsingType :type "/Game/CHARACTER_SYSTEM_V2/Blueprints/DATA/E/Equipment/E_EquipmentUsingType Enum" :default "NewEnumerator0"))
  ;[1 1 1] HANDLE USING EQUIPMENT
  ;;[1 0.6824 0] BI TO MESH ANIM INSTANCE
  (message `/Game/CHARACTER_SYSTEM_V2/Blueprints/BI/BI_CharacterAnim.CharacterAnimUseEquipmentOn` (`SkeletalMeshComponent.GetAnimInstance` (`self.Mesh`)) EquipmentUsingType))

(event `self.ServerHandleUseEquipmentOn`
  (params (EquipmentUsingType :type "/Game/CHARACTER_SYSTEM_V2/Blueprints/DATA/E/Equipment/E_EquipmentUsingType Enum" :default "NewEnumerator0"))
  ;[1 1 1] HANDLE USING EQUIPMENT
  ;;[0.1778 0 1] PARENT INPUT
  (`self.MulticastHandleChildUseEquipmentOn` EquipmentUsingType))

(event `self.ClientHandleTPCameraMirrorTrigger`
  ;[1 1 1] HANDLE CAMERA MIRROR INPUT
  ;;[0.1778 0 1] PARENT INPUT EVENT
  (`self.ClientHandleTPCameraMirrorInput`))

(event `MulticastAttachThrowableEquipBeforeUse`
  (params (EquipActor :type "Actor Object Reference"))
  ;[1 1 1] HANDLE USING EQUIPMENT
  (`/Engine/EditorBlueprintResources/StandardMacros.IsValid` EquipActor
    (:`Is Valid`
      (`self.K2_AttachToComponent` EquipActor (`self.Mesh`) (`self.EquipmentAttachPointThrow`) "SnapToTarget" "SnapToTarget" "KeepRelative" true))))

(event `self.ServerAttachThrowableEquipBeforeUse`
  (params (EquipActor :type "Actor Object Reference"))
  ;[1 1 1] HANDLE USING EQUIPMENT
  ;;[0.1778 0 1] PARENT INPUT
  (`self.MulticastAttachThrowableEquipBeforeUse` EquipActor))

(event `MulticastHandleTPVaultHighCoverTrigger`
  ;[1 1 1] HANDLE COVERS INTERACTION
  ;;[1 1 1] VaultHighCover
  ;;;[1 0.6824 0] BI TO MESH ANIM INSTANCE
  (message `/Game/CHARACTER_SYSTEM_V2/Blueprints/BI/BI_CharacterAnim.CharacterAnimVaultHighCoverTriger` (`SkeletalMeshComponent.GetAnimInstance` (`self.Mesh`))))

(event `self.ServerVaultHighCoverTriger`
  ;[1 1 1] HANDLE COVERS INTERACTION
  ;;[1 1 1] VaultHighCover
  ;;;[0.1778 0 1] PARENT INPUT
  (`self.MulticastHandleTPVaultHighCoverTrigger`))

(event `self.ServerJumpOverLowCoverTriger`
  ;[1 1 1] HANDLE COVERS INTERACTION
  ;;[1 1 1] JumpOverLowCover
  ;;;[0.1778 0 1] PARENT INPUT
  (`self.MulticastHandleTPJumpOverLowCoverTrigger`))

(event `MulticastHandleTPJumpOverLowCoverTrigger`
  ;[1 1 1] HANDLE COVERS INTERACTION
  ;;[1 1 1] JumpOverLowCover
  ;;;[1 0.6824 0] BI TO MESH ANIM INSTANCE
  (message `/Game/CHARACTER_SYSTEM_V2/Blueprints/BI/BI_CharacterAnim.CharacterAnimJumpOverLowCoverTriger` (`SkeletalMeshComponent.GetAnimInstance` (`self.Mesh`))))

(event `MulticastHandleTPClimbLowCoverTrigger`
  ;[1 1 1] HANDLE COVERS INTERACTION
  ;;[1 1 1] ClimbLowCover
  ;;;[1 0.6824 0] BI TO MESH ANIM INSTANCE
  (message `/Game/CHARACTER_SYSTEM_V2/Blueprints/BI/BI_CharacterAnim.CharacterAnimClimbLowCoverTriger` (`SkeletalMeshComponent.GetAnimInstance` (`self.Mesh`))))

(event `self.ServerClimbLowCoverTriger`
  ;[1 1 1] HANDLE COVERS INTERACTION
  ;;[1 1 1] ClimbLowCover
  ;;;[0.1778 0 1] PARENT INPUT
  (`self.MulticastHandleTPClimbLowCoverTrigger`))

(event `self.ServerClimbHighCoverTriger`
  ;[1 1 1] HANDLE COVERS INTERACTION
  ;;[1 1 1] ClimbHighCover
  ;;;[0.1778 0 1] PARENT INPUT
  (`self.MulticastHandleTPClimbHighCoverTrigger`))

(event `MulticastHandleTPClimbHighCoverTrigger`
  ;[1 1 1] HANDLE COVERS INTERACTION
  ;;[1 1 1] ClimbHighCover
  ;;;[1 0.6824 0] BI TO MESH ANIM INSTANCE
  (message `/Game/CHARACTER_SYSTEM_V2/Blueprints/BI/BI_CharacterAnim.CharacterAnimClimbHighCoverTriger` (`SkeletalMeshComponent.GetAnimInstance` (`self.Mesh`))))

(event `MulticastShowCurrentEquipmentOnAction`
  (params (Show :type Boolean))
  ;[1 1 1] HANDLE COVERS INTERACTION
  ;;[1 1 1] HANDLE ATACH & SHOW WEAPON ON COVER ACTION
  (if Show
    (`self.SetActorHiddenInGame` (`self.CurrentTPEquip`) false)
    (else
      (`self.SetActorHiddenInGame` (`self.CurrentTPEquip`) true))))

(event `self.ServerAttachToBackpackWeaponOnCoverInteraction`
  (params (CharacterWeaponStateBeforeCovInt :type "/Game/CHARACTER_SYSTEM_V2/Blueprints/DATA/E/E_CharacterWeaponState Enum" :default "NewEnumerator0"))
  ;[1 1 1] HANDLE COVERS INTERACTION
  ;;[1 1 1] HANDLE ATACH & SHOW WEAPON ON COVER ACTION
  ;;;[0.1778 0 1] PARENT INPUT
  (switch `/Game/CHARACTER_SYSTEM_V2/Blueprints/DATA/E/E_CharacterWeaponState` CharacterWeaponStateBeforeCovInt
    (:`NewEnumerator1`
      ;;;[1 0.6824 0] TO INVENTORY SYSTEM
      (`/Game/CHARACTER_SYSTEM_V2/Blueprints/InventorySystem/AC_InventorySystem.ServerAttachCurrentFirearmToBackPackOnAction` (`self.InventorySystem`)))
    (:`NewEnumerator2`
      (`self.MulticastShowCurrentEquipmentOnAction` false))))

(event `self.ServerReAttachToHandWeaponAfterCoverInteraction`
  (params (CharacterWeaponStateBeforeCovInt :type "/Game/CHARACTER_SYSTEM_V2/Blueprints/DATA/E/E_CharacterWeaponState Enum" :default "NewEnumerator0"))
  ;[1 1 1] HANDLE COVERS INTERACTION
  ;;[1 1 1] HANDLE ATACH & SHOW WEAPON ON COVER ACTION
  ;;;[0.1778 0 1] PARENT INPUT
  (switch `/Game/CHARACTER_SYSTEM_V2/Blueprints/DATA/E/E_CharacterWeaponState` CharacterWeaponStateBeforeCovInt
    (:`NewEnumerator1`
      (`self.ServerAttachCurrentFirearm`))
    (:`NewEnumerator2`
      (`self.MulticastShowCurrentEquipmentOnAction` true))))

(event `MulticastHandleVehicleOn`
  ;[1 1 1] HANDLE VEHICLE
  ;;[1 1 1] Handle Vehicle on
  (`SceneComponent.SetVisibility` (`self.Backpack`) false false)
  (`SceneComponent.SetVisibility` (`self.Mesh`) false false))

(event `self.ServerHandleVehicleOn`
  ;[1 1 1] HANDLE VEHICLE
  ;;[1 1 1] Handle Vehicle on
  ;;;[0.1778 0 1] PARENT INPUT
  (`self.MulticastHandleVehicleOn`))

(event `MulticastHandleVehicleOff`
  ;[1 1 1] HANDLE VEHICLE
  ;;[1 1 1] Handle Vehicle off
  (`SceneComponent.SetVisibility` (`self.Backpack`) true false)
  (`SceneComponent.SetVisibility` (`self.Mesh`) true false))

(event `self.ServerHandleVehicleOff`
  ;[1 1 1] HANDLE VEHICLE
  ;;[1 1 1] Handle Vehicle off
  ;;;[0.1778 0 1] PARENT INPUT
  (`self.MulticastHandleVehicleOff`))

(event `ClientInitTPCameraAdvancedOnSpawn`
  ;[1 1 1] Init Camera On Spawn
  (`/Engine/EditorBlueprintResources/StandardMacros.IsValid` (`self.PlayerCameraTP`)
    (:`Is Valid`
      (`/Engine/EditorBlueprintResources/StandardMacros.IsValid` (`self.SpringArm`)
        (:`Is Valid`
          (`/Engine/EditorBlueprintResources/StandardMacros.IsValid` (`self.Camera`)
            (:`Is Valid`
              ;;[1 0.6824 0] TO PLAYER CAMERA TP
              (`/Game/CHARACTER_SYSTEM_V2/Blueprints/PlayerCameraTP/AC_PlayerCameraTP.ClientSetStartCameraMode` (`self.PlayerCameraTP`) (`self.SpringArm`) (`self.Camera`) "StandIdle" true))))))))

(event `ClientTPCameraAdvancedChangePreset`
  (params (NewCameraPreset :type Name))
  ;[1 1 1] Change Camera Preset
  ;;[1 0.6824 0] TO PLAYER CAMERA TP
  (`/Game/CHARACTER_SYSTEM_V2/Blueprints/PlayerCameraTP/AC_PlayerCameraTP.ClientOpenGateChange` (`self.PlayerCameraTP`))
  ;;[1 0.6824 0] TO PLAYER CAMERA TP
  (`/Game/CHARACTER_SYSTEM_V2/Blueprints/PlayerCameraTP/AC_PlayerCameraTP.ClientChangeCameraMode` (`self.PlayerCameraTP`) (`self.SpringArm`) (`self.Camera`) NewCameraPreset))

(event `ClientDifineNewCameraPreset`
  (params (MainCharacterState :type "/Game/CHARACTER_SYSTEM_V2/Blueprints/DATA/E/E_CharacterMainState Enum" :default "NewEnumerator0"))
  (bind _characterweaponstate (`self.GetCharacterWeaponState`))
  (bind _characterweaponstate_2 (`self.GetCharacterWeaponState`))
  (bind _characterweaponstate_3 (`self.GetCharacterWeaponState`))
  ;[1 1 1] Difine New Camera Preset
  (if (not (`/Game/CHARACTER_SYSTEM_V2/Blueprints/FirearmSystem/AC_FirearmScopeController.GetInScope` (`self.GetFirearmScopeController`)))
    (switch `/Game/CHARACTER_SYSTEM_V2/Blueprints/DATA/E/E_CharacterMainState` MainCharacterState
      (:`NewEnumerator0`
        (`self.ClientTPCameraAdvancedChangePreset` "StandIdle"))
      (:`NewEnumerator12`
        (`self.ClientTPCameraAdvancedChangePreset` "StandMove"))
      (:`NewEnumerator1`
        ;;[1 1 1] Check: Equip / Unarmed / Melee
        (if (not (or (`|EnumEquality` _characterweaponstate_2 "NewEnumerator0") (`|EnumEquality` _characterweaponstate_2 "NewEnumerator2") (`|EnumEquality` _characterweaponstate_2 "NewEnumerator3"))) :!label _label
          (`self.ClientTPCameraAdvancedChangePreset` "StandAim")))
      (:`NewEnumerator13`
        (goto _label))
      (:`NewEnumerator2`
        (`self.ClientTPCameraAdvancedChangePreset` "CrouchIdle"))
      (:`NewEnumerator14`
        (`self.ClientTPCameraAdvancedChangePreset` "CrouchMove"))
      (:`NewEnumerator3`
        ;;[1 1 1] Check: Equip / Unarmed / Melee
        (if (not (or (`|EnumEquality` _characterweaponstate_3 "NewEnumerator0") (`|EnumEquality` _characterweaponstate_3 "NewEnumerator2") (`|EnumEquality` _characterweaponstate_3 "NewEnumerator3"))) :!label _label_2
          (`self.ClientTPCameraAdvancedChangePreset` "CrouchAim")))
      (:`NewEnumerator15`
        (goto _label_2))
      (:`NewEnumerator4`
        (`self.ClientTPCameraAdvancedChangePreset` "ProneIdle"))
      (:`NewEnumerator16`
        (`self.ClientTPCameraAdvancedChangePreset` "ProneMove"))
      (:`NewEnumerator5`
        ;;[1 1 1] Check: Equip / Unarmed / Melee
        (if (not (or (`|EnumEquality` _characterweaponstate "NewEnumerator0") (`|EnumEquality` _characterweaponstate "NewEnumerator2") (`|EnumEquality` _characterweaponstate "NewEnumerator3"))) :!label _label_3
          (`self.ClientTPCameraAdvancedChangePreset` "ProneAim")))
      (:`NewEnumerator17`
        (goto _label_3))
      (:`NewEnumerator6`
        (`self.ClientTPCameraAdvancedChangePreset` "Sprint"))
      (:`NewEnumerator7`
        (`self.ClientTPCameraAdvancedChangePreset` "HighCoverClimb" :!label _label_4))
      (:`NewEnumerator8`
        (goto _label_4))
      (:`NewEnumerator9`
        (goto _label_4))
      (:`NewEnumerator10`
        (goto _label_4))
      (:`NewEnumerator11`
        (`self.ClientTPCameraAdvancedChangePreset` "Dead")))))

(event `ClientHandleTPCameraMirrorInput`
  ;[1 1 1] Camera Mirror
  ;;[1 0.6824 0] TO PLAYER CAMERA TP
  (`/Game/CHARACTER_SYSTEM_V2/Blueprints/PlayerCameraTP/AC_PlayerCameraTP.ClientUpdateCameraMirror` (`self.PlayerCameraTP`)))

(event `ClientSwitchAttachignTPCamera`
  (params (CharacterState :type "/Game/CHARACTER_SYSTEM_V2/Blueprints/DATA/E/E_CharacterMainState Enum" :default "NewEnumerator0"))
  ;[1 1 1] Switch Attacing TP Camera
  (if (or (`|EnumEquality` CharacterState "NewEnumerator7") (`|EnumEquality` CharacterState "NewEnumerator8") (`|EnumEquality` CharacterState "NewEnumerator9") (`|EnumEquality` CharacterState "NewEnumerator10"))
    (`KismetSystemLibrary.Delay` 0.2)
    (`SceneComponent.K2_AttachToComponent` (`self.SpringArm`) (`self.Mesh`) "None" "KeepRelative" "KeepRelative" "KeepRelative" true)
    (`SceneComponent.K2_SetRelativeLocation` (`self.SpringArm`) (0.0 0.0 150.0) false true)
    (else
      (`KismetSystemLibrary.Delay` 0.3)
      (`SceneComponent.K2_AttachToComponent` (`self.SpringArm`) (`self.Mesh`) "VB TPCamRootPoint" "KeepRelative" "KeepRelative" "KeepRelative" true)
      (`SceneComponent.K2_SetRelativeLocation` (`self.SpringArm`) (0.0 0.0 0.0) false false))))

(fn `UserConstructionScript`
  (`parent.UserConstructionScript`))