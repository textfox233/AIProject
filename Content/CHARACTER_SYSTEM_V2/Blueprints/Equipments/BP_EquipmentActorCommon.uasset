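; Common equipment actor for the character system, holding an owning character and a mesh, with events for removal and collision object type changes.
; Visibility events toggle mesh and hidden shadow on inventory request or by the owner's FP/TP camera mode, though the net-mode-checked spawn call is disconnected.
; Getters read DT_EquipmentLibrary rows by EquipmentTag, feeding inventory-facing functions for type, text, icons, rarity and crafting, with ammo and upgrades stubbed.
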(event `self.ReceiveBeginPlay`
  ;[1 1 1] EVENT BEGIN PLAY
)

(event `ClientShowMeshForFPEquipment`
  ;[1 1 1] INITIALIZE VISIBILITY MESH ON SPAWN
  ;;[1 1 1] ClientShowMeshForFPEquipment
  ;;;[1 0.1179 0] INPUT FROM CHARACTER FP
  (`SceneComponent.SetVisibility` (`self.EquipmentMesh`) true false)
  (`PrimitiveComponent.SetCastHiddenShadow` (`self.EquipmentMesh`) false))

(event `ClientInitializeVisibilityMeshItemOnSpawn`
  ;[1 1 1] INITIALIZE VISIBILITY MESH ON SPAWN
  ;;[1 1 1] ClientInitializeVisibilityMeshItemOnSpawn
  (`/Engine/EditorBlueprintResources/StandardMacros.IsValid` (`self.GetOwner`)
    (:`Is Valid`
      ;;;[1 0.2552 0.2552] CHECK: FP or TP-FP Character
      (bind _asbp_character_common (cast `/Game/CHARACTER_SYSTEM_V2/Blueprints/CharacterCommon/BP_CharacterCommon` (`self.GetOwner`)))
      (bind _charactertype (`/Game/CHARACTER_SYSTEM_V2/Blueprints/CharacterCommon/BP_CharacterCommon.CharacterType` _asbp_character_common))
      (if (or (`|EnumEquality` _charactertype "NewEnumerator1") (`|EnumEquality` _charactertype "NewEnumerator2"))
        (switch `/Game/CHARACTER_SYSTEM_V2/Blueprints/DATA/E/E_CharacterCameraMode` (`/Game/CHARACTER_SYSTEM_V2/Blueprints/CharacterCommon/BP_CharacterCommon.GetCurrentCameraMode` _asbp_character_common)
          (:`NewEnumerator0`
            (`self.ClientHandleUpdateVisibilityMeshItem` "NewEnumerator2"))
          (:`NewEnumerator1`
            (`self.ClientHandleUpdateVisibilityMeshItem` "NewEnumerator1")))))))

(event `/Game/CHARACTER_SYSTEM_V2/Blueprints/BI/BI_InventoryToggleVisibilityForOwner.BIInventoryUpdateVisibilityMeshItem`
  (params (NewVisibilityMode :type "/Game/CHARACTER_SYSTEM_V2/Blueprints/DATA/E/E_InventoryItemVisibilityMode Enum" :default "NewEnumerator0"))
  ;[1 1 1] HANDLE UPDATE VISIBILITY MESH ITEM FOR OWNER
  ;;[1 0.1179 0] [CLIENT] BI FROM INVENTORY
  (`self.ClientHandleUpdateVisibilityMeshItem` NewVisibilityMode))

(event `ClientHandleUpdateVisibilityMeshItem`
  (params (NewVisibilityMode :type "/Game/CHARACTER_SYSTEM_V2/Blueprints/DATA/E/E_InventoryItemVisibilityMode Enum" :default "NewEnumerator0"))
  ;[1 1 1] HANDLE UPDATE VISIBILITY MESH ITEM FOR OWNER
  (switch `/Game/CHARACTER_SYSTEM_V2/Blueprints/DATA/E/E_InventoryItemVisibilityMode` NewVisibilityMode
    (:`NewEnumerator0`
      ;;[1 1 1] Show Mesh & Show Cast Hidden Shadows
      (`SceneComponent.SetVisibility` (`self.EquipmentMesh`) true false)
      (`PrimitiveComponent.SetCastHiddenShadow` (`self.EquipmentMesh`) true))
    (:`NewEnumerator2`
      ;;[1 1 1] Show Mesh & Hide Cast Hidden Shadows
      (`SceneComponent.SetVisibility` (`self.EquipmentMesh`) true false)
      (`PrimitiveComponent.SetCastHiddenShadow` (`self.EquipmentMesh`) false))
    (:`NewEnumerator1`
      ;;[1 1 1] Hide Mesh & Show Cast Hidden Shadows
      (`SceneComponent.SetVisibility` (`self.EquipmentMesh`) false false)
      (`PrimitiveComponent.SetCastHiddenShadow` (`self.EquipmentMesh`) true))
    (:`NewEnumerator3`
      ;;[1 1 1] Hide Mesh & Hide Cast Hidden Shadows
      (`SceneComponent.SetVisibility` (`self.EquipmentMesh`) false false)
      (`PrimitiveComponent.SetCastHiddenShadow` (`self.EquipmentMesh`) false))))

(event `MulticastRemoveEquipment`
  ;[1 1 1] REMOVE EQUIPMENT
  ;;[1 0.1179 0] INPUT FROM CHILD ACTOR
  (`/Engine/EditorBlueprintResources/StandardMacros.IsValid` self
    (:`Is Valid`
      (`self.K2_DestroyActor`))))

(event `ServerInitializeOwner`
  (params (OwnedCharacter :type "Actor Object Reference"))
  ;[1 1 1] INITIALIZE OWNER
  ;;[1 0.1179 0] INPUT FROM CHARACTER COMMON
  (set `self.OwnedCharacter` OwnedCharacter))

(event `MulticastEquipMeshChangeObjectType`
  (params (Channel :type "ECollisionChannel Enum" :default "ECC_WorldStatic"))
  ;[1 1 1] EQUIPMENT MESH CHANGE OBJECT TYPE
  ;;[1 0.1179 0] INPUT FROM CHILD ACTOR
  (`PrimitiveComponent.SetCollisionObjectType` (`self.EquipmentMesh`) Channel))

(fn `GetEquipmentCanBeCrafted`
  (returns (`Can be Crafted` :type Boolean))
  (bind _returnvalue (`|GetDataTableRow` "/Game/CHARACTER_SYSTEM_V2/Blueprints/Equipments/DT_EquipmentLibrary.DT_EquipmentLibrary" (`self.EquipmentTag`))
    (:`then`
      (return (`.CanbeCrafted_15_91A5962340F9AD8008F417A55735CDB9` (break `/Game/CHARACTER_SYSTEM_V2/Blueprints/DATA/STR/STR_EquipmentLibraryDesc` _returnvalue))))))

(fn `GetEquipmentCommonType`
  (returns (EquipmentCommonType :type "/Game/CHARACTER_SYSTEM_V2/Blueprints/DATA/E/Equipment/E_EquipmentCommonType Enum"))
  (bind _returnvalue (`|GetDataTableRow` "/Game/CHARACTER_SYSTEM_V2/Blueprints/Equipments/DT_EquipmentLibrary.DT_EquipmentLibrary" (`self.EquipmentTag`))
    (:`then`
      (return (`.EquipmentCommonType_30_4F02270F4209D2894E31E2B8CFF42ACE` (break `/Game/CHARACTER_SYSTEM_V2/Blueprints/DATA/STR/STR_EquipmentLibraryDesc` _returnvalue))))))

(fn `GetEquipmentCraftResourcesList`
  (returns (`Craft Resources List` :type "Array of /Game/CHARACTER_SYSTEM_V2/Blueprints/DATA/STR/STR_GL_InventoryResourceDesc Structure"))
  (bind _returnvalue (`|GetDataTableRow` "/Game/CHARACTER_SYSTEM_V2/Blueprints/Equipments/DT_EquipmentLibrary.DT_EquipmentLibrary" (`self.EquipmentTag`))
    (:`then`
      (return (`.CraftResourcesList_21_76BBF01749A76C2112DFA7A7978BE2E6` (break `/Game/CHARACTER_SYSTEM_V2/Blueprints/DATA/STR/STR_EquipmentLibraryDesc` _returnvalue))))))

(fn `GetEquipmentDesc`
  (returns (Desc :type Text))
  (bind _returnvalue (`|GetDataTableRow` "/Game/CHARACTER_SYSTEM_V2/Blueprints/Equipments/DT_EquipmentLibrary.DT_EquipmentLibrary" (`self.EquipmentTag`))
    (:`then`
      (return (`.Desc_4_BB0F895A42E1231E75CAAA9DB3C3803E` (break `/Game/CHARACTER_SYSTEM_V2/Blueprints/DATA/STR/STR_EquipmentLibraryDesc` _returnvalue))))))

(fn `GetEquipmentIconWeaponModule`
  (returns (`Icon weaon module` :type "Texture2D Object Reference"))
  (bind _returnvalue (`|GetDataTableRow` "/Game/CHARACTER_SYSTEM_V2/Blueprints/Equipments/DT_EquipmentLibrary.DT_EquipmentLibrary" (`self.EquipmentTag`))
    (:`then`
      (return (`.Iconweaonmodule_9_57DC91994226FE62FAB4069DC3C8F167` (break `/Game/CHARACTER_SYSTEM_V2/Blueprints/DATA/STR/STR_EquipmentLibraryDesc` _returnvalue))))))

(fn `GetEquipmentIconWeaponWheel`
  (returns (`Icon weapon wheel` :type "Texture2D Object Reference"))
  (bind _returnvalue (`|GetDataTableRow` "/Game/CHARACTER_SYSTEM_V2/Blueprints/Equipments/DT_EquipmentLibrary.DT_EquipmentLibrary" (`self.EquipmentTag`))
    (:`then`
      (return (`.Iconweaponwheel_7_DC90F93B48257DBDE563BF874B03D8B7` (break `/Game/CHARACTER_SYSTEM_V2/Blueprints/DATA/STR/STR_EquipmentLibraryDesc` _returnvalue))))))

(fn `GetEquipmentRarityType`
  (returns (`Rarity type` :type "/Game/CHARACTER_SYSTEM_V2/Blueprints/DATA/E/Inventory/E_RarityType Enum"))
  (bind _returnvalue (`|GetDataTableRow` "/Game/CHARACTER_SYSTEM_V2/Blueprints/Equipments/DT_EquipmentLibrary.DT_EquipmentLibrary" (`self.EquipmentTag`))
    (:`then`
      (return (`.Raritytype_20_D831C95F4D8C726B0DABAABC31DA88E0` (break `/Game/CHARACTER_SYSTEM_V2/Blueprints/DATA/STR/STR_EquipmentLibraryDesc` _returnvalue))))))

(fn `GetEquipmentTitle`
  (returns (Title :type Text))
  (bind _returnvalue (`|GetDataTableRow` "/Game/CHARACTER_SYSTEM_V2/Blueprints/Equipments/DT_EquipmentLibrary.DT_EquipmentLibrary" (`self.EquipmentTag`))
    (:`then`
      (return (`.Title_2_38114300414C76475C14F78D50C9BA32` (break `/Game/CHARACTER_SYSTEM_V2/Blueprints/DATA/STR/STR_EquipmentLibraryDesc` _returnvalue))))))

(fn `GetEquipmentType`
  (returns (EquipmentType :type "/Game/CHARACTER_SYSTEM_V2/Blueprints/DATA/E/Equipment/E_EquipmentType Enum"))
  (bind _returnvalue (`|GetDataTableRow` "/Game/CHARACTER_SYSTEM_V2/Blueprints/Equipments/DT_EquipmentLibrary.DT_EquipmentLibrary" (`self.EquipmentTag`))
    (:`then`
      (return (`.EquipmentType_27_DF7FED684F6607F7757BBF8025540F69` (break `/Game/CHARACTER_SYSTEM_V2/Blueprints/DATA/STR/STR_EquipmentLibraryDesc` _returnvalue))))))

(fn `GetEquipmentUsingType`
  (returns (EquipmentUsingType :type "/Game/CHARACTER_SYSTEM_V2/Blueprints/DATA/E/Equipment/E_EquipmentUsingType Enum"))
  (bind _returnvalue (`|GetDataTableRow` "/Game/CHARACTER_SYSTEM_V2/Blueprints/Equipments/DT_EquipmentLibrary.DT_EquipmentLibrary" (`self.EquipmentTag`))
    (:`then`
      (return (`.EquipmentUsingType_24_D1732C44428108742AF8CB883E567155` (break `/Game/CHARACTER_SYSTEM_V2/Blueprints/DATA/STR/STR_EquipmentLibraryDesc` _returnvalue))))))

(fn `GetInventoryEquipCanBeCrafted`
  (returns (CanBeCrafted :type Boolean))
  (return (`self.GetEquipmentCanBeCrafted`)))

(fn `GetInventoryEquipCommonType`
  (returns (EquipCommonType :type "/Game/CHARACTER_SYSTEM_V2/Blueprints/DATA/E/Equipment/E_EquipmentCommonType Enum"))
  (return (`self.GetEquipmentCommonType`)))

(fn `GetInventoryEquipNeededResourcesList`
  (returns (NeededResourcesList :type "Array of /Game/CHARACTER_SYSTEM_V2/Blueprints/DATA/STR/STR_GL_InventoryResourceDesc Structure") (NewParam :type Boolean))
  (return (`self.GetEquipmentCraftResourcesList`) false))

(fn `GetInventoryEquipUpgrades`
  (returns (EquipmentUpgrades :type "Array of /Game/CHARACTER_SYSTEM_V2/Blueprints/DATA/STR/STR_GL_EquipmentUpgradeDesc Structure"))
  (return))

(fn `GetInventoryEquipUsingType`
  (returns (EquipmentUsingType :type "/Game/CHARACTER_SYSTEM_V2/Blueprints/DATA/E/Equipment/E_EquipmentUsingType Enum"))
  (return (`self.GetEquipmentUsingType`)))

(fn `GetInventoryItemAmmoCount`
  (returns (AmmoCount :type Integer))
  (return 0))

(fn `GetInventoryItemDesc`
  (returns (Title :type Text))
  (return (`self.GetEquipmentDesc`)))

(fn `GetInventoryItemIconWeaponModule`
  (returns (Icon :type "Texture2D Object Reference"))
  (return (`self.GetEquipmentIconWeaponModule`)))

(fn `GetInventoryItemIconWeaponWheel`
  (returns (Icon :type "Texture2D Object Reference"))
  (return (`self.GetEquipmentIconWeaponWheel`)))

(fn `GetInventoryItemRarityType`
  (returns (RarityType :type "/Game/CHARACTER_SYSTEM_V2/Blueprints/DATA/E/Inventory/E_RarityType Enum"))
  (return (`self.GetEquipmentRarityType`)))

(fn `GetInventoryItemTitle`
  (returns (Title :type Text))
  (return (`self.GetEquipmentTitle`)))

(fn `GetOwnedCharacter`
  (returns (OwnedCharacter :type "Actor Object Reference"))
  (return (`self.OwnedCharacter`)))

(fn `GetWeaponModuleIcon`
  (returns (WeaponModuleIcon :type "Texture2D Object Reference"))
  (return (`self.GetEquipmentIconWeaponModule`)))

(fn `UserConstructionScript`)