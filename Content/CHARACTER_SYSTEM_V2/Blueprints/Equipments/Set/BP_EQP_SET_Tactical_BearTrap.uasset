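; Tactical bear trap equipment that slows characters other than its owner who step into it.
; Parent-driven server activation arms it, multicasts the trigger sphere to WorldDynamic, and checks characters already inside, using DoOnce to hit just one.
; Later overlaps and that initial check both wait a trigger delay, message the target to reduce movement for a duration, then multicast a sound and, after another delay, equipment removal.
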(event `self.ServerHandleActivation`
  (bind _overlappingactors (`PrimitiveComponent.GetOverlappingActors` (`self.TriggerSphere`) "/Script/Engine.Character"))
  ;[1 1 1] HANDLE ACTIVATION
  ;;[0.1778 0 1] PARENT INPUT
  (set `self.CanBeTriggered` true)
  (`self.MulticastTriggerSphereChangeObjectType` "ECC_WorldDynamic")
  (if (>= (`KismetArrayLibrary.Array_Length` _overlappingactors) 1)
    (`self.ServerCheckOnActivation` _overlappingactors)))

(event `MulticastTriggerSphereChangeObjectType`
  (params (Channel :type "ECollisionChannel Enum" :default "ECC_WorldStatic"))
  ;[1 1 1] HANDLE ACTIVATION
  (`PrimitiveComponent.SetCollisionObjectType` (`self.TriggerSphere`) Channel))

(event `self.TriggerSphere.OnComponentBeginOverlap`
  (params (OverlappedComponent :type "PrimitiveComponent Object Reference") (OtherActor :type "Actor Object Reference") (OtherComp :type "PrimitiveComponent Object Reference") (OtherBodyIndex :type Integer) (bFromSweep :type Boolean) (SweepResult :type "HitResult Structure (by ref)"))
  ;[1 1 1] OVERLAP (TRIGGER)
  ;;[1 1 1] Condition. Check only characters and ignore owner.
  (if (`self.CanBeTriggered`)
    (bind _ascharacter (cast `Character` OtherActor))
    (bind _ascharacter_2 (cast `Character` (`self.GetOwnedCharacter`)))
    (if (not (== _ascharacter_2 _ascharacter))
      (`KismetSystemLibrary.Delay` (`self.TriggerDelay`))
      ;;[1 0.6824 0] TO TARGET
      (message `/Game/CHARACTER_SYSTEM_V2/Blueprints/BI/BI_EquipBearTrapInfluence.BearTrapReduceMovement` OtherActor (`self.Reduce Movement Multiplier`) (`self.Duration`))
      (`self.MulticastTriggering` (`SceneComponent.K2_GetComponentLocation` (`self.EquipmentMesh`)) :!label _label)
      (`KismetSystemLibrary.Delay` (`self.RemoveItemDelay`))
      (`self.MulticastRemoveEquipment`))))

(event `ServerCheckOnActivation`
  (params (OverlappingActors :type "Array of Actor Object Reference"))
  ;[1 1 1] OVERLAP (TRIGGER)
  (for _array_element OverlappingActors
    (bind _ascharacter (cast `Character` _array_element))
    (bind _ascharacter_2 (cast `Character` (`self.GetOwnedCharacter`)))
    (if (not (== _ascharacter_2 _ascharacter))
      (set `self.Target` _array_element)
      (`/Engine/EditorBlueprintResources/StandardMacros.DoOnce` false
        (:`Completed`
          (`KismetSystemLibrary.Delay` (`self.TriggerDelay`))
          ;;[1 0.6824 0] TO TARGET
          (message `/Game/CHARACTER_SYSTEM_V2/Blueprints/BI/BI_EquipBearTrapInfluence.BearTrapReduceMovement` (`self.Target`) (`self.Reduce Movement Multiplier`) (`self.Duration`))
          (goto _label))))))

(event `MulticastTriggering`
  (params (EquipmentMeshLocation :type "Vector Structure"))
  ;[1 1 1] HANDLE TRIGGING
  ;;[1 1 1] Sound
  (`GameplayStatics.PlaySoundAtLocation` "/Game/CHARACTER_SYSTEM_V2/Demo/Sound/WeaponsSound/Cue/CUE_BoltAction_01.CUE_BoltAction_01" EquipmentMeshLocation (struct) 1.0 1.0 0.0 null null null null))

(fn `UserConstructionScript`
  (`parent.UserConstructionScript`))