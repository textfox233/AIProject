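; Base Blueprint for equipment actors that are set in the world and activate after a delay.
; ServerActivateSetEquipment calls the set hook, plays its sound and switches the mesh object type to WorldDynamic through an inherited multicast event.
; After ActivationDelay it calls the activation hook and plays the activation sound.
; Both hooks are empty events for children to implement, while multicast events play both sounds at the mesh location with attenuation.
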(event `ServerActivateSetEquipment`
  ;[1 1 1] ACTIVATE SET EQUIPMENT
  (`self.ServerHandleSet`)
  (`self.MulticastPlay3DSoundSet`)
  ;;[1 0 0.5639] TO PARENT ACTOR
  (`self.MulticastEquipMeshChangeObjectType` "ECC_WorldDynamic")
  (`KismetSystemLibrary.Delay` (`self.ActivationDelay`))
  (`self.ServerHandleActivation`)
  (`self.MulticastPlay3DSoundActivation`))

(event `ServerHandleActivation`
  ;[1 1 1] ACTIVATE SET EQUIPMENT
  ;;[0.1778 0 1] PARENT OUTPUT
)

(event `ServerHandleSet`
  ;[1 1 1] ACTIVATE SET EQUIPMENT
  ;;[0.1778 0 1] PARENT OUTPUT
)

(event `MulticastPlay3DSoundSet`
  ;[1 1 1] Sound
  (`GameplayStatics.PlaySoundAtLocation` (`self.SoundSet`) (`SceneComponent.K2_GetComponentLocation` (`self.EquipmentMesh`)) (struct) 1.0 1.0 0.0 "/Game/CHARACTER_SYSTEM_V2/Demo/Sound/AttenuationPresets/ATT_HitSound.ATT_HitSound" null null null))

(event `MulticastPlay3DSoundActivation`
  ;[1 1 1] Sound
  (`GameplayStatics.PlaySoundAtLocation` (`self.SoundActivation`) (`SceneComponent.K2_GetComponentLocation` (`self.EquipmentMesh`)) (struct) 1.0 1.0 0.0 "/Game/CHARACTER_SYSTEM_V2/Demo/Sound/AttenuationPresets/ATT_HitSound.ATT_HitSound" null null null))

(fn `UserConstructionScript`
  (`parent.UserConstructionScript`))