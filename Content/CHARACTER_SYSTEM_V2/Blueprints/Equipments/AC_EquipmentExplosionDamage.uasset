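; Equipment component that deals explosion damage to actors within a radius, through an event named as a server call.
; ServerSpawnRadialDamage stores its inputs and runs a complex multi-sphere object trace at the given location, skipping ignored actors.
; Hit actors are deduplicated into an array, then each receives the same base damage and damage type, with no distance falloff.
; The event never clears that array before reuse.
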(event `ServerSpawnRadialDamage`
  (params (ExplosionRadius :type "Float (double-precision)") (`Actors to Ignore` :type "Array of Actor Object Reference") (`Object Types` :type "Array of EObjectTypeQuery Enum") (Location :type "Vector Structure") (Damage :type "Float (double-precision)") (`Damage Type Class` :type "DamageType Class Reference"))
  (bind _location (`self.Location`))
  ;[1 0.1179 0] INPUT FROM EQUIPMENT
  ;[1 1 1] Initialize
  (set `self.ExplosionRadius` ExplosionRadius)
  (set `self.Actors to Ignore` `Actors to Ignore`)
  (set `self.Object Types` `Object Types`)
  (set `self.Location` Location)
  (set `self.Damage` Damage)
  (set `self.Damage Type Class` `Damage Type Class`)
  ;[1 1 1] Create Sphere Trace
  (bind _outhits (`KismetSystemLibrary.SphereTraceMultiForObjects` _location _location (`self.ExplosionRadius`) (`self.Object Types`) true (`self.Actors to Ignore`)))
  ;[1 1 1] Add unique hitted actors
  (for _array_element _outhits
    (`KismetArrayLibrary.Array_AddUnique` (`self.HittedActorsArray`) (`.HitActor` (`GameplayStatics.BreakHitResult` _array_element))))
  (for _array_element_2 (`self.HittedActorsArray`)
    (`GameplayStatics.ApplyDamage` _array_element_2 (`self.Damage`) null null (`self.Damage Type Class`))))