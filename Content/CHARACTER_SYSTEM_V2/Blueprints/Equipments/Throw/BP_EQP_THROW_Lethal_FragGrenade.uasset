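; Lethal frag grenade throwable, a child equipment Blueprint that deals radial damage when it explodes.
; It overrides the parent's server collision and explosion events, multicasting a once-only impact sound and the blast's particle, sound and mesh hiding.
; The server spawns damage through the explosion damage component, then removes the grenade via multicast after a short delay.
; Inventory getter overrides are empty stubs, and the debug sphere is disconnected.
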(event `self.ServerHandleThrowCollisionHappened`
  ;[1 1 1] HANDLE COLLISION EVENT
  ;;[0.1778 0 1] PARENT INPUT
  (`self.MulticastCreateHit`))

(event `self.ServerHandleThrowExplosionHappened`
  (params (EquipmentMeshLocation :type "Vector Structure"))
  ;[1 1 1] HANDLE EXPLOSION EVENT
  ;;[0.1778 0 1] PARENT INPUT
  ;;[1 0.6824 0] TO Equipment Explosion Damage
  (`/Game/CHARACTER_SYSTEM_V2/Blueprints/Equipments/AC_EquipmentExplosionDamage.ServerSpawnRadialDamage` (`self.AC_EquipmentExplosionDamage`) (`self.ExplosionRadius`) (`|MakeArray` self :!type "Actor Object Reference") (`|MakeArray` "ObjectTypeQuery7" :!type "EObjectTypeQuery Enum") EquipmentMeshLocation (`self.Damage`) (`self.Damage Type Class`))
  (`self.MulticastCreateExplosion` EquipmentMeshLocation)
  (`KismetSystemLibrary.Delay` 0.2)
  (`self.MulticastRemoveEquipment`))

(event `MulticastCreateHit`
  ;[1 1 1] CREATE HIT
  (`/Engine/EditorBlueprintResources/StandardMacros.DoOnce` false
    (:`Completed`
      ;;[1 1 1] Sound
      (`GameplayStatics.PlaySoundAtLocation` "/Game/CHARACTER_SYSTEM_V2/Demo/Sound/WeaponsSound/Cue/CUE_ClipIn_02.CUE_ClipIn_02" (`SceneComponent.K2_GetComponentLocation` (`self.EquipmentMesh`)) (struct) 1.0 1.0 0.0 null null null null))))

(event `MulticastCreateExplosion`
  (params (EquipmentMeshLocation :type "Vector Structure"))
  ;[1 1 1] CREATE EXPLOSION
  ;;[1 1 1] VFX
  (`GameplayStatics.SpawnEmitterAtLocation` "/Game/CHARACTER_SYSTEM_V2/Demo/Effects/ParticleSystems/PS_Launcher_IH.PS_Launcher_IH" EquipmentMeshLocation (struct) (1.3 1.3 1.3))
  (`SceneComponent.SetHiddenInGame` (`self.EquipmentMesh`) true false)
  ;;[1 1 1] Sound
  (`GameplayStatics.PlaySoundAtLocation` "/Game/CHARACTER_SYSTEM_V2/Demo/Sound/Equipment/Cue/CUE_Explosion_01.CUE_Explosion_01" EquipmentMeshLocation (struct) 1.0 1.0 0.0 null null null null))

(fn `GetInventoryItemCommonIconWeaponModule`
  (returns (Icon :type "Texture2D Object Reference"))
  (return null))

(fn `GetInventoryItemEquipNeededResourcesList`
  (returns (NeededResourcesList :type "Array of /Game/CHARACTER_SYSTEM_V2/Blueprints/DATA/STR/STR_GL_InventoryResourceDesc Structure") (NewParam :type Boolean))
  (return _ false))

(fn `GetInventoryItemEquipUpgrades`
  (returns (EquipmentUpgrades :type "Array of /Game/CHARACTER_SYSTEM_V2/Blueprints/DATA/STR/STR_GL_EquipmentUpgradeDesc Structure"))
  (return))

(fn `UserConstructionScript`
  (`parent.UserConstructionScript`))