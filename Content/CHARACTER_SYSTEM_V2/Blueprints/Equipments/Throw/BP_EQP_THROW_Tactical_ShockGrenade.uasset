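; Throwable tactical shock grenade equipment that creates a timed zone applying a movement reduction effect to characters.
; Server throw, collision and explosion events drive multicasts for collision type, sound, particles and zone state.
; Sphere overlaps send start and stop shock messages to non-owner characters, while a delayed activation check affects only the owner.
; When the zone expires, it stops the effect on the last stored actor and removes the equipment.
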(event `self.ServerHandleThrowCollisionHappened`
  ;[1 1 1] HANDLE COLLISION EVENT
  ;;[0.1778 0 1] PARENT INPUT
  (`self.MulticastCreateHit`))

(event `MulticastZoneSphereChangeObjectType`
  (params (Channel :type "ECollisionChannel Enum" :default "ECC_WorldStatic"))
  ;[1 1 1] HANDLE THROW EQUIPMENT
  (`PrimitiveComponent.SetCollisionObjectType` (`self.ZoneSphere`) Channel))

(event `self.ServerHandleThowEquipment`
  ;[1 1 1] HANDLE THROW EQUIPMENT
  ;;[0.1778 0 1] PARENT INPUT
  (`self.MulticastZoneSphereChangeObjectType` "ECC_WorldDynamic"))

(event `self.ServerHandleThrowExplosionHappened`
  (params (EquipmentMeshLocation :type "Vector Structure"))
  (bind _overlappingactors (`PrimitiveComponent.GetOverlappingActors` (`self.ZoneSphere`) "/Script/Engine.Character"))
  ;[1 1 1] HANDLE EXPLOSION EVENT
  ;;[0.1778 0 1] PARENT INPUT
  (`self.MulticastCreateZone` EquipmentMeshLocation)
  (`|ExecutionSequence`
    (:`then_0`
      (`KismetSystemLibrary.Delay` (`self.ZoneDuration`))
      (`self.MulticastEndZone` EquipmentMeshLocation)
      ;;[1 0.6824 0] TO TARGET
      (message `/Game/CHARACTER_SYSTEM_V2/Blueprints/BI/BI_EquipShockGrenadeInfluence.StopShockGrenadeInf` (`self.OverlapedActor`))
      (`KismetSystemLibrary.Delay` 1.0)
      (`self.MulticastRemoveEquipment`))
    (:`then_1`
      (`KismetSystemLibrary.Delay` 0.2)
      (if (>= (`KismetArrayLibrary.Array_Length` _overlappingactors) 1)
        (`self.ServerCheckOnActivation` _overlappingactors)))))

(event `ServerCheckOnActivation`
  (params (OverlappingActors :type "Array of Actor Object Reference"))
  ;[1 1 1] HANDLE EXPLOSION EVENT
  (for _array_element OverlappingActors
    (bind _ascharacter (cast `Character` _array_element))
    (bind _ascharacter_2 (cast `Character` (`self.GetOwnedCharacter`)))
    (if (== _ascharacter_2 _ascharacter)
      (set `self.OverlapedActor` _array_element)
      ;;[1 0.6824 0] TO TARGET
      (message `/Game/CHARACTER_SYSTEM_V2/Blueprints/BI/BI_EquipShockGrenadeInfluence.StartShockGrenadeInf` (`self.OverlapedActor`) (`self.Reduce Movement Multiplier`)))))

(event `MulticastCreateHit`
  ;[1 1 1] CREATE HIT
  (`/Engine/EditorBlueprintResources/StandardMacros.DoOnce` false
    (:`Completed`
      ;;[1 1 1] Sound
      (`GameplayStatics.PlaySoundAtLocation` "/Game/CHARACTER_SYSTEM_V2/Demo/Sound/WeaponsSound/Cue/CUE_ClipIn_02.CUE_ClipIn_02" (`SceneComponent.K2_GetComponentLocation` (`self.EquipmentMesh`)) (struct) 1.0 1.0 0.0 null null null null))))

(event `MulticastCreateZone`
  (params (EquipmentMeshLocation :type "Vector Structure"))
  ;[1 1 1] ZONE
  (set `self.CanBeTriggered` true)
  (`ActorComponent.Activate` (`self.ParticleSystem`) false)
  (`self.PlayerSound` EquipmentMeshLocation))

(event `MulticastEndZone`
  (params (EquipmentMeshLocation :type "Vector Structure"))
  ;[1 1 1] ZONE
  (set `self.CanBeTriggered` false)
  (`ActorComponent.Deactivate` (`self.ParticleSystem`)))

(event `PlayerSound`
  (params (Location :type "Vector Structure"))
  ;[1 1 1] ZONE
  (`GameplayStatics.PlaySoundAtLocation` "/Game/CHARACTER_SYSTEM_V2/Demo/Sound/Equipment/Cue/CUE_ShotZoneSound_01.CUE_ShotZoneSound_01" Location (struct) 0.6 1.0 0.0 "/Game/CHARACTER_SYSTEM_V2/Demo/Sound/AttenuationPresets/ATT_HitSound.ATT_HitSound" null null null))

(event `self.ZoneSphere.OnComponentBeginOverlap`
  (params (OverlappedComponent :type "PrimitiveComponent Object Reference") (OtherActor :type "Actor Object Reference") (OtherComp :type "PrimitiveComponent Object Reference") (OtherBodyIndex :type Integer) (bFromSweep :type Boolean) (SweepResult :type "HitResult Structure (by ref)"))
  ;[1 1 1] OVERLAP (TRIGGER)
  ;;[1 1 1] Condition. Check only characters and ignore owner.
  (if (`self.CanBeTriggered`)
    (bind _ascharacter (cast `Character` OtherActor))
    (bind _ascharacter_2 (cast `Character` (`self.GetOwnedCharacter`)))
    (if (not (== _ascharacter_2 _ascharacter))
      (set `self.OverlapedActor` OtherActor)
      ;;[1 0.6824 0] TO TARGET
      (message `/Game/CHARACTER_SYSTEM_V2/Blueprints/BI/BI_EquipShockGrenadeInfluence.StartShockGrenadeInf` (`self.OverlapedActor`) (`self.Reduce Movement Multiplier`)))))

(event `self.ZoneSphere.OnComponentEndOverlap`
  (params (OverlappedComponent :type "PrimitiveComponent Object Reference") (OtherActor :type "Actor Object Reference") (OtherComp :type "PrimitiveComponent Object Reference") (OtherBodyIndex :type Integer))
  ;[1 1 1] OVERLAP (TRIGGER)
  ;;[1 1 1] Condition. Check only characters and ignore owner.
  (bind _ascharacter (cast `Character` OtherActor))
  (bind _ascharacter_2 (cast `Character` (`self.GetOwnedCharacter`)))
  (if (not (== _ascharacter_2 _ascharacter))
    ;;[1 0.6824 0] TO TARGET
    (message `/Game/CHARACTER_SYSTEM_V2/Blueprints/BI/BI_EquipShockGrenadeInfluence.StopShockGrenadeInf` OtherActor)))

(fn `GetInventoryItemEquipNeededResourcesList`
  (returns (NeededResourcesList :type "Array of /Game/CHARACTER_SYSTEM_V2/Blueprints/DATA/STR/STR_GL_InventoryResourceDesc Structure") (NewParam :type Boolean))
  (return _ false))

(fn `GetInventoryItemEquipUpgrades`
  (returns (EquipmentUpgrades :type "Array of /Game/CHARACTER_SYSTEM_V2/Blueprints/DATA/STR/STR_GL_EquipmentUpgradeDesc Structure"))
  (return))

(fn `UserConstructionScript`
  (`parent.UserConstructionScript`))