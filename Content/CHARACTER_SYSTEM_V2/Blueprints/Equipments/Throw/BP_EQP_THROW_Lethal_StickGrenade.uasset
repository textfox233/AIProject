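; Lethal sticky grenade throwable that attaches to a character it overlaps and deals radial damage.
; Throwing switches the CharacterDetector to WorldDynamic; its overlap stops physics and snaps the mesh to the nearest "stick_grenade_point" socket.
; After a delay, server or standalone applies damage through ACEquipmentExplosionDamage, without explosion effects or removal on this path.
; The inherited explosion event applies damage, multicasts VFX and sound, then removes the grenade.
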(event `self.ServerHandleThrowCollisionHappened`
  ;[1 1 1] HANDLE COLLISION EVENT
  ;;[0.1778 0 1] PARENT INPUT
)

(event `MulticastCharacterDetectorChangeObjectType`
  (params (Channel :type "ECollisionChannel Enum" :default "ECC_WorldStatic"))
  ;[1 1 1] HANDLE THROW EQUIPMENT
  (`PrimitiveComponent.SetCollisionObjectType` (`self.CharacterDetector`) Channel))

(event `self.ServerHandleThowEquipment`
  ;[1 1 1] HANDLE THROW EQUIPMENT
  ;;[0.1778 0 1] PARENT INPUT
  (`self.MulticastCharacterDetectorChangeObjectType` "ECC_WorldDynamic"))

(event `self.ServerEquipmentHit`
  (params (`Hit Component` :type "PrimitiveComponent Object Reference") (`Other Actor` :type "Actor Object Reference"))
  ;[1 1 1] HANDLE EQUIPMENT HIT
  ;;[0.1778 0 1] PARENT INPUT
)

(event `MulticastEquipmentHit`
  (params (Parent :type "SceneComponent Object Reference") (MeshLocation :type "Vector Structure"))
  ;[1 1 1] HANDLE EQUIPMENT HIT
  (`PrimitiveComponent.SetSimulatePhysics` (`self.EquipmentMesh`) false)
  (`PrimitiveComponent.SetCollisionEnabled` (`self.EquipmentMesh`) "NoCollision")
  (`PrimitiveComponent.SetPhysicsLinearVelocity` (`self.EquipmentMesh`) (0.0 0.0 0.0) true "None")
  (`SceneComponent.K2_AttachToComponent` (`self.EquipmentMesh`) Parent "None" "KeepWorld" "KeepWorld" "KeepWorld" true)
  ;[1 1 1] Sound
  (`GameplayStatics.PlaySoundAtLocation` "/Game/CHARACTER_SYSTEM_V2/Demo/Sound/WeaponsSound/Cue/CUE_BoltAction_01.CUE_BoltAction_01" MeshLocation (struct) 1.0 1.0 0.0 "/Game/CHARACTER_SYSTEM_V2/Demo/Sound/AttenuationPresets/ATT_HitSound.ATT_HitSound" null null null))

(event `ServerExplosionStick`
  (params (EquipmentMeshLocation :type "Vector Structure"))
  ;[1 1 1] HANDLE EXPLOSION EVENT
  ;;[1 0.6824 0] TO Equipment Explosion Damage
  (`/Game/CHARACTER_SYSTEM_V2/Blueprints/Equipments/AC_EquipmentExplosionDamage.ServerSpawnRadialDamage` (`self.AC_EquipmentExplosionDamage`) (`self.ExplosionRadius`) (`|MakeArray` self :!type "Actor Object Reference") (`|MakeArray` "ObjectTypeQuery7" :!type "EObjectTypeQuery Enum") EquipmentMeshLocation (`self.Damage`) (`self.Damage Type Class`)))

(event `self.ServerHandleThrowExplosionHappened`
  (params (EquipmentMeshLocation :type "Vector Structure"))
  ;[1 1 1] HANDLE EXPLOSION EVENT
  ;;[0.1778 0 1] PARENT INPUT
  ;;[1 0.6824 0] TO Equipment Explosion Damage
  (`/Game/CHARACTER_SYSTEM_V2/Blueprints/Equipments/AC_EquipmentExplosionDamage.ServerSpawnRadialDamage` (`self.AC_EquipmentExplosionDamage`) (`self.ExplosionRadius`) (`|MakeArray` self :!type "Actor Object Reference") (`|MakeArray` "ObjectTypeQuery7" :!type "EObjectTypeQuery Enum") EquipmentMeshLocation (`self.Damage`) (`self.Damage Type Class`))
  (`self.MulticastCreateExplosion` EquipmentMeshLocation)
  (`KismetSystemLibrary.Delay` 0.2)
  (`self.MulticastRemoveEquipment`))

(event `MulticastCreateExplosion`
  (params (EquipmentMeshLocation :type "Vector Structure"))
  ;[1 1 1] CREATE EXPLOSION
  ;;[1 1 1] VFX
  (`GameplayStatics.SpawnEmitterAtLocation` "/Game/CHARACTER_SYSTEM_V2/Demo/Effects/ParticleSystems/PS_Launcher_IH.PS_Launcher_IH" EquipmentMeshLocation (struct) (1.3 1.3 1.3))
  (`SceneComponent.SetHiddenInGame` (`self.EquipmentMesh`) true false)
  ;;[1 1 1] Sound
  (`GameplayStatics.PlaySoundAtLocation` "/Game/CHARACTER_SYSTEM_V2/Demo/Sound/Equipment/Cue/CUE_Explosion_01.CUE_Explosion_01" EquipmentMeshLocation (struct) 1.0 1.0 0.0 null null null null))

(event `self.CharacterDetector.OnComponentBeginOverlap`
  (params (OverlappedComponent :type "PrimitiveComponent Object Reference") (OtherActor :type "Actor Object Reference") (OtherComp :type "PrimitiveComponent Object Reference") (OtherBodyIndex :type Integer) (bFromSweep :type Boolean) (SweepResult :type "HitResult Structure (by ref)"))
  ;[1 1 1] CHARACTER
  (if (`self.GetCanHandleHitEvent`)
    (bind _ascharacter (cast `Character` OtherActor))
    (`/Engine/EditorBlueprintResources/StandardMacros.DoOnce` false
      (:`Completed`
        (bind _skeletalmeshcomponent (message `/Game/CHARACTER_SYSTEM_V2/Blueprints/BI/BI_EquipStickGrenadeCharacterMesh.GetSkeletalMeshComponent` _ascharacter))
        (`PrimitiveComponent.SetSimulatePhysics` (`self.EquipmentMesh`) false)
        (`PrimitiveComponent.SetSimulatePhysics` (`self.Sphere`) false)
        (`PrimitiveComponent.SetCollisionEnabled` (`self.EquipmentMesh`) "NoCollision")
        (`PrimitiveComponent.SetCollisionEnabled` (`self.Sphere`) "NoCollision")
        (`PrimitiveComponent.SetPhysicsLinearVelocity` (`self.EquipmentMesh`) (0.0 0.0 0.0) true "None")
        (bind _socketforattach (`self.GetNearestSocketForAttach` _skeletalmeshcomponent))
        (`/Engine/EditorBlueprintResources/StandardMacros.IsValid` (`self.EquipmentMesh`)
          (:`Is Valid`
            (`/Engine/EditorBlueprintResources/StandardMacros.IsValid` _skeletalmeshcomponent
              (:`Is Valid`
                (`SceneComponent.K2_AttachToComponent` (`self.EquipmentMesh`) _skeletalmeshcomponent _socketforattach "SnapToTarget" "KeepWorld" "KeepWorld" true)
                (`|ExecutionSequence`
                  (:`then_0`
                    ;;[1 1 1] Sound
                    (`GameplayStatics.PlaySoundAtLocation` null (`SceneComponent.K2_GetComponentLocation` (`self.EquipmentMesh`)) (struct) 1.0 1.0 0.0 null null null null))
                  (:`then_1`
                    (if (`KismetSystemLibrary.IsStandalone`)
                      (`KismetSystemLibrary.Delay` (`self.TimeExplosionAfterCollision`) :!label _label)
                      (`self.ServerExplosionStick` (`SceneComponent.K2_GetComponentLocation` (`self.EquipmentMesh`)))
                      (elif (`KismetSystemLibrary.IsServer`)
                        (goto _label)))))))))))))

(fn `GetNearestSocketForAttach`
  (params (CharacterMesh :type "SkeletalMeshComponent Object Reference"))
  (returns (SocketForAttach :type Name))
  (locals (loc_character_mesh :type "SkeletalMeshComponent Object Reference") (loc_valid_sockets_id :type "Array of Integer") (loc_min_distance :type "Float (double-precision)" :default 500.0) (loc_min_distance_socket_id :type Integer))
  (set `local.loc_character_mesh` CharacterMesh)
  ;[1 1 1] Finding all sockets for attaching stick grenade
  (for (_array_element _array_index) (`SceneComponent.GetAllSocketNames` (`local.loc_character_mesh`))
    (if (`KismetStringLibrary.Contains` (`KismetStringLibrary.Conv_NameToString` _array_element) "stick_grenade_point" true)
      (`KismetArrayLibrary.Array_Set` (`local.loc_valid_sockets_id`) _array_index _array_index true)))
  ;[1 1 1] Finding nearest socket for attach
  (for (_array_element_2 _array_index_2) (`local.loc_valid_sockets_id`)
    (bind _returnvalue (`KismetMathLibrary.Vector_Distance` (`SceneComponent.K2_GetComponentLocation` (`self.EquipmentMesh`)) (.location (`SceneComponent.GetSocketTransform` (`local.loc_character_mesh`) (`|GetArrayItem` (`SceneComponent.GetAllSocketNames` (`local.loc_character_mesh`)) _array_element_2) "RTS_World"))))
    (if (<= _returnvalue (`local.loc_min_distance`))
      (set `local.loc_min_distance` _returnvalue)
      (set `local.loc_min_distance_socket_id` _array_index_2)))
  ;[1 1 1] OUTPUT
  (return (`|GetArrayItem` (`SceneComponent.GetAllSocketNames` (`local.loc_character_mesh`)) (`local.loc_min_distance_socket_id`))))

(fn `GetSkeletalMeshComponent`
  (returns (SkeletalMeshComponent :type "SkeletalMeshComponent Object Reference"))
  (return null))

(fn `UserConstructionScript`
  (`parent.UserConstructionScript`))