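; Base equipment actor for throwable items, handling the throw, first impact and delayed explosion.
; A one-shot server throw switches mesh and sphere to physics bodies, then multicasts physics simulation with the launch velocity.
; Hit events are ignored briefly after throwing; the first valid hit, processed on server or standalone, fires collision, then timed explosion, then disables sphere collision.
; Empty server handler events act as hooks, presumably for child classes.
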(event `MulticastThrowEquipment`
  (params (Velocity :type "Vector Structure"))
  ;[1 1 1] THROW EQUIPMENT
  (`PrimitiveComponent.SetCollisionEnabled` (`self.EquipmentMesh`) "QueryAndPhysics")
  (`PrimitiveComponent.SetSimulatePhysics` (`self.EquipmentMesh`) true)
  (`PrimitiveComponent.SetPhysicsLinearVelocity` (`self.EquipmentMesh`) Velocity true "None")
  ;;[1 1 1] Open opportunity for hit event after thrwing
  (`KismetSystemLibrary.Delay` (`self.TimeIgnoringHitEventAfterThrow`))
  (set `self.CanHandleHitEvent?` true))

(event `ServerThrowEquipment`
  (params (Velocity :type "Vector Structure"))
  ;[1 1 1] THROW EQUIPMENT
  ;;[1 0.1179 0] INPUT FROM CHARACTER COMMON
  (`/Engine/EditorBlueprintResources/StandardMacros.DoOnce` false
    (:`Completed`
      (`self.ServerHandleThowEquipment`)
      ;;[1 0 0.5639] TO PARENT ACTOR
      (`self.MulticastEquipMeshChangeObjectType` "ECC_PhysicsBody")
      (`self.MulticastSphereChangeObjectType` "ECC_PhysicsBody")
      (`self.MulticastThrowEquipment` Velocity))))

(event `ServerHandleThowEquipment`
  ;[1 1 1] THROW EQUIPMENT
  ;;[0.1778 0 1] PARENT OUTPUT
)

(event `MulticastSphereChangeObjectType`
  (params (Channel :type "ECollisionChannel Enum" :default "ECC_WorldStatic"))
  ;[1 1 1] THROW EQUIPMENT
  (`PrimitiveComponent.SetCollisionObjectType` (`self.Sphere`) Channel))

(event `self.EquipmentMesh.OnComponentHit`
  (params (HitComponent :type "PrimitiveComponent Object Reference") (OtherActor :type "Actor Object Reference") (OtherComp :type "PrimitiveComponent Object Reference") (NormalImpulse :type "Vector Structure") (Hit :type "HitResult Structure (by ref)"))
  ;[1 1 1] COLLISION
  (if (`self.CanHandleHitEvent?`)
    (`/Engine/EditorBlueprintResources/StandardMacros.DoOnce` false
      (:`Completed`
        (if (`KismetSystemLibrary.IsStandalone`)
          (`self.ServerEquipmentHit` OtherComp OtherActor :!label _label)
          (`self.ServerHandleThrowCollisionHappened`)
          (`KismetSystemLibrary.Delay` (`self.TimeExplosionAfterCollision`))
          (`self.ServerHandleThrowExplosionHappened` (`SceneComponent.K2_GetComponentLocation` (`self.EquipmentMesh`)))
          (`KismetSystemLibrary.Delay` 1.0)
          (`self.MulticastDisablePhys`)
          (elif (`KismetSystemLibrary.IsServer`)
            (goto _label)))))))

(event `ServerEquipmentHit`
  (params (`Hit Component` :type "PrimitiveComponent Object Reference") (`Other Actor` :type "Actor Object Reference"))
  ;[1 1 1] COLLISION
  ;;[0.1778 0 1] PARENT OUTPUT
)

(event `MulticastDisablePhys`
  ;[1 1 1] COLLISION
  (`PrimitiveComponent.SetCollisionEnabled` (`self.Sphere`) "NoCollision"))

(event `ServerHandleThrowCollisionHappened`
  ;[1 1 1] COLLISION
  ;;[0.1778 0 1] PARENT OUTPUT
)

(event `ServerHandleThrowExplosionHappened`
  (params (EquipmentMeshLocation :type "Vector Structure"))
  ;[1 1 1] COLLISION
  ;;[0.1778 0 1] PARENT OUTPUT
)

(fn `GetCanHandleHitEvent`
  (returns (`CanHandleHitEvent?` :type Boolean))
  (return (`self.CanHandleHitEvent?`)))

(fn `UserConstructionScript`
  (`parent.UserConstructionScript`))