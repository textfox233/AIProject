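; Throwable tactical smoke grenade equipment that releases a timed smoke effect when it goes off.
; Parent throw events on the server drive multicasts: collision plays a one-time hit sound, and explosion activates the Niagara smoke with its sound.
; After the smoke duration the server deactivates the effect, waits briefly, then multicasts removal of the equipment.
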(event `self.ServerHandleThrowCollisionHappened`
  ;[1 1 1] HANDLE COLLISION EVENT
  ;;[0.1778 0 1] PARENT INPUT
  (`self.MulticastCreateHit`))

(event `self.ServerHandleThrowExplosionHappened`
  (params (EquipmentMeshLocation :type "Vector Structure"))
  ;[1 1 1] HANDLE EXPLOSION EVENT
  ;;[0.1778 0 1] PARENT INPUT
  (`self.MulticastCreateSmoke` EquipmentMeshLocation)
  (`KismetSystemLibrary.Delay` (`self.SmokeDuration`))
  (`self.MulticastEndSmoke` EquipmentMeshLocation)
  (`KismetSystemLibrary.Delay` 2.0)
  (`self.MulticastRemoveEquipment`))

(event `MulticastCreateHit`
  ;[1 1 1] CREATE HIT
  (`/Engine/EditorBlueprintResources/StandardMacros.DoOnce` false
    (:`Completed`
      ;;[1 1 1] Sound
      (`GameplayStatics.PlaySoundAtLocation` "/Game/CHARACTER_SYSTEM_V2/Demo/Sound/WeaponsSound/Cue/CUE_ClipIn_02.CUE_ClipIn_02" (`SceneComponent.K2_GetComponentLocation` (`self.EquipmentMesh`)) (struct) 1.0 1.0 0.0 null null null null))))

(event `MulticastCreateSmoke`
  (params (EquipmentMeshLocation :type "Vector Structure"))
  ;[1 1 1] SMOKE
  (`ActorComponent.Activate` (`self.SmokeNiagara`) false)
  (`GameplayStatics.PlaySoundAtLocation` "/Game/CHARACTER_SYSTEM_V2/Demo/Sound/Equipment/Cue/CUE_SmokeGrenadeSound_01.CUE_SmokeGrenadeSound_01" EquipmentMeshLocation (struct) 0.7 1.0 0.0 "/Game/CHARACTER_SYSTEM_V2/Demo/Sound/AttenuationPresets/ATT_HitSound.ATT_HitSound" null null null))

(event `MulticastEndSmoke`
  (params (EquipmentMeshLocation :type "Vector Structure"))
  ;[1 1 1] SMOKE
  (`ActorComponent.Deactivate` (`self.SmokeNiagara`)))

(fn `GetInventoryItemEquipNeededResourcesList`
  (returns (NeededResourcesList :type "Array of /Game/CHARACTER_SYSTEM_V2/Blueprints/DATA/STR/STR_GL_InventoryResourceDesc Structure") (NewParam :type Boolean))
  (return _ false))

(fn `GetInventoryItemEquipUpgrades`
  (returns (EquipmentUpgrades :type "Array of /Game/CHARACTER_SYSTEM_V2/Blueprints/DATA/STR/STR_GL_EquipmentUpgradeDesc Structure"))
  (return))

(fn `UserConstructionScript`
  (`parent.UserConstructionScript`))