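; Player character that switches between third-person and first-person views, extending a parent character through its input and state hooks.
; One camera and spring arm serve both views, with timelines blending arm length, socket offset and FOV during switches.
; In third person, character state selects PlayerCameraTP presets, while cover moves reattach the spring arm.
; Mode-aware handlers toggle body, arms and weapon visibility for scopes, cover actions and vehicles.
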(event `self.ReceiveTick`
  (params (DeltaSeconds :type "Float (single-precision)"))
  ;[1 1 1] EVENT TICK
  (`parent.ReceiveTick` DeltaSeconds))

(event `self.ReceiveBeginPlay`
  ;[1 1 1] EVENT BEGIN PLAY
  (`parent.ReceiveBeginPlay`)
  ;;[1 0.2552 0.2552] CHECK: Character type & spawn camera type
  (if (`|EnumEquality` (`self.CharacterType`) "NewEnumerator2")
    (if (`self.GetSpawnInFPMode`)
      ;;[1 1 1] Spawn in fp mode
      ;;;[1 1 1] Initialize FP camera mode
      ;;;;[1 0.2552 0.2552] CHECK: IsStandalone
      (if (`KismetSystemLibrary.IsStandalone`)
        (`self.ServerActivateFPCharacterMode`)
        (else
          ;;;;[1 0.2552 0.2552] CHECK: IsServer
          (if (`KismetSystemLibrary.IsServer`)
            ;;;;[1 0.2552 0.2552] CHECK: IsDedicatedServer
            (if (`KismetSystemLibrary.IsDedicatedServer`)
              (`self.ServerActivateFPCharacterMode`)
              (else
                (`self.ServerActivateFPCharacterMode`)
                (`self.ClientActivateFPCharacterMode`)))
            (else
              (`self.ClientActivateFPCharacterMode`)))))
      (`self.ClientInitTPCameraAdvancedOnSpawn` false)
      ;;;[1 0.6824 0] TO PLAYER CAMERA TP
      (`/Game/CHARACTER_SYSTEM_V2/Blueprints/PlayerCameraTP/AC_PlayerCameraTP.ClientUpdateFPCameraState` (`self.PlayerCameraTP`) true)
      ;;;[1 0.6824 0] TO PLAYER CAMERA FP
      (`/Game/CHARACTER_SYSTEM_V2/Blueprints/PlayerCameraFP/AC_PlayerCameraFP.ClientInitializeFPCamera` (`self.PlayerCameraFP`) (`self.FPSCamera`) true)
      ;;;[1 0.6824 0] TO PLAYER CAMERA FP
      (`/Game/CHARACTER_SYSTEM_V2/Blueprints/PlayerCameraFP/AC_PlayerCameraFP.ClientUpdateFPCameraState` (`self.PlayerCameraFP`) true)
      (else
        ;;[1 1 1] Spawn in tp mode
        ;;;[1 1 1] Initialize TP camera mode
        ;;;;[1 0.2552 0.2552] CHECK: IsStandalone
        (if (`KismetSystemLibrary.IsStandalone`)
          (`self.ServerActivateTPCharacterMode`)
          (else
            ;;;;[1 0.2552 0.2552] CHECK: IsServer
            (if (`KismetSystemLibrary.IsServer`)
              ;;;;[1 0.2552 0.2552] CHECK: IsDedicatedServer
              (if (`KismetSystemLibrary.IsDedicatedServer`)
                (`self.ServerActivateTPCharacterMode`)
                (else
                  (`self.ServerActivateTPCharacterMode`)
                  (`self.ClientActivateTPCharacterMode`)))
              (else
                (`self.ClientActivateTPCharacterMode`)))))
        (`self.ClientInitTPCameraAdvancedOnSpawn` true)
        ;;;[1 0.6824 0] TO PLAYER CAMERA TP
        (`/Game/CHARACTER_SYSTEM_V2/Blueprints/PlayerCameraTP/AC_PlayerCameraTP.ClientUpdateFPCameraState` (`self.PlayerCameraTP`) false)
        ;;;[1 0.6824 0] TO PLAYER CAMERA FP
        (`/Game/CHARACTER_SYSTEM_V2/Blueprints/PlayerCameraFP/AC_PlayerCameraFP.ClientInitializeFPCamera` (`self.PlayerCameraFP`) (`self.FPSCamera`) false)
        ;;;[1 0.6824 0] TO PLAYER CAMERA FP
        (`/Game/CHARACTER_SYSTEM_V2/Blueprints/PlayerCameraFP/AC_PlayerCameraFP.ClientUpdateFPCameraState` (`self.PlayerCameraFP`) false)))))

(event `self.ServerChildHandleFirearmInitialized`
  (params (CurrentADSTime :type "Float (double-precision)"))
  ;[1 1 1] HANDLE ATTACH FIREARM
  ;;[0.1778 0 1] PARENT INPUT EVENT
  ;;[1 0.6824 0] TO PLAYER CAMERA TP
  (`/Game/CHARACTER_SYSTEM_V2/Blueprints/PlayerCameraTP/AC_PlayerCameraTP.ClientUpdateAimTime` (`self.PlayerCameraTP`) CurrentADSTime)
  (if (`|EnumEquality` (`self.CharacterType`) "NewEnumerator2")
    (switch `/Game/CHARACTER_SYSTEM_V2/Blueprints/DATA/E/E_CharacterCameraMode` (`self.GetCurrentCameraMode`)
      (:`NewEnumerator0`
        (`self.ServerActivateTPCharacterMode`))
      (:`NewEnumerator1`
        (`self.ServerActivateFPCharacterMode`)))))

(event `self.ServerChildHandleEquipInitialized`
  ;[1 1 1] HANDLE ATTACH EQUIPMENT
  ;;[0.1778 0 1] PARENT INPUT EVENT
  (if (`|EnumEquality` (`self.CharacterType`) "NewEnumerator2")
    (switch `/Game/CHARACTER_SYSTEM_V2/Blueprints/DATA/E/E_CharacterCameraMode` (`self.GetCurrentCameraMode`)
      (:`NewEnumerator0`
        (`self.ServerActivateTPCharacterMode`))
      (:`NewEnumerator1`
        (`self.ServerActivateFPCharacterMode`)))))

(event `ServerActivateTPCharacterMode`
  ;[1 1 1] ACTIVATE TP CHARACTER MODE
  (`self.ClientActivateTPCharacterMode`)
  ;;[1 0 0.1451] TO PARENT
  (`self.SetCurrentCameraState` "NewEnumerator0")
  ;;[1 1 1] Set FPS CAMERA Rotation == 0
  (`SceneComponent.K2_SetRelativeRotation` :`self` (`self.FPSCamera`)))

(event `ClientActivateTPCharacterMode`
  ;[1 1 1] ACTIVATE TP CHARACTER MODE
  ;;[1 1 1] Hide FP Body & FP Arms
  (`SceneComponent.SetVisibility` (`self.FPSBody`) false false)
  (`SceneComponent.SetVisibility` (`self.FPArms`) false false)
  ;;[1 1 1] Hide FP Firearm
  (`/Engine/EditorBlueprintResources/StandardMacros.IsValid` (`self.GetCurrentFPFirearm`)
    (:`Is Valid`
      (`self.SetActorHiddenInGame` (`self.GetCurrentFPFirearm`) true))
    (:`Is Not Valid`
      _))
  ;;[1 1 1] Hide FP Equip
  (`/Engine/EditorBlueprintResources/StandardMacros.IsValid` (`self.GetCurrentFPEquip`)
    (:`Is Valid`
      (`self.SetActorHiddenInGame` (`self.GetCurrentFPEquip`) true))
    (:`Is Not Valid`
      _))
  ;;[1 1 1] Show TP Mesh & Backpack (Owner No See = 0)
  (`PrimitiveComponent.SetOwnerNoSee` (`self.Mesh`) false)
  (`PrimitiveComponent.SetOwnerNoSee` (`self.Backpack`) false)
  ;;[1 0 0.1451] TO PARENT
  (`self.SetCurrentCameraState` "NewEnumerator0")
  ;;[1 0.6824 0] TO FIREARM SYSTEM
  (`/Game/CHARACTER_SYSTEM_V2/Blueprints/FirearmSystem/AC_FirearmSystem.ClientToggleFPMode` (`self.FirearmSystem`) false)
  ;;[1 1 1] Comment
  (set `SpringArmComponent.bUsePawnControlRotation` true (`self.SpringArm`))
  (set `CameraComponent.bUsePawnControlRotation` false (`self.FPSCamera`))
  ;;[1 1 1] Set FPS CAMERA Rotation == 0
  (`SceneComponent.K2_SetRelativeRotation` :`self` (`self.FPSCamera`)))

(event `self.ServerHandleChildChangedMain State`
  (params (MainCharacterState :type "/Game/CHARACTER_SYSTEM_V2/Blueprints/DATA/E/E_CharacterMainState Enum" :default "NewEnumerator0"))
  ;[1 1 1] HANDLE CHANGING MAIN STATE
  ;;[0.1778 0 1] PARENT INPUT
  (`self.ClientDifineNewCameraPreset` MainCharacterState)
  (`self.ClientSwitchAttachignTPCamera` MainCharacterState))

(event `self.ClientHandleSwitchTPFPModeTrigger`
  ;[1 1 1] HANDLE SWITCH TP-FP MODE
  ;;[0.1778 0 1] PARENT INPUT
  (`self.ClientChangeCameraMode`))

(event `self.ClientHandleTPCameraMirrorTrigger`
  ;[1 1 1] HANDLE CAMERA MIRROR INPUT
  ;;[0.1778 0 1] PARENT INPUT EVENT
  (`self.ClientHandleTPCameraMirrorInput`))

(event `self.ClientHandleTPFPScopeOnOff`
  (params (`Scope ON` :type Boolean))
  ;[1 1 1] HANDLE SCOPER ON / OFF
  ;;[0.1778 0 1] PARENT INPUT EVENT
  (if (`|EnumEquality` (`self.CharacterType`) "NewEnumerator2")
    (switch `/Game/CHARACTER_SYSTEM_V2/Blueprints/DATA/E/E_CharacterCameraMode` (`self.GetCurrentCameraMode`)
      (:`NewEnumerator0`
        ;;[1 1 1] TP Mode
        (if `Scope ON`
          ;;;[1 1 1] Hide TP Mesh
          (`SceneComponent.SetHiddenInGame` (`self.Mesh`) true false)
          ;;;[1 1 1] Hide TP Firearm
          (`self.SetActorHiddenInGame` (`self.GetCurrentTPFirearm`) true)
          (bind _asbp_firearm_actor_common (cast `/Game/CHARACTER_SYSTEM_V2/Blueprints/FirearmSystem/BP_FirearmActorCommon` (`self.GetCurrentTPFirearm`)))
          (`PrimitiveComponent.SetCastHiddenShadow` (`/Game/CHARACTER_SYSTEM_V2/Blueprints/FirearmSystem/BP_FirearmActorCommon.FirearmMesh` _asbp_firearm_actor_common) true)
          (else
            ;;;[1 1 1] Set TP Camera Preset
            (`self.ClientDifineNewCameraPreset` (`self.GetMainCharacterState`))
            ;;;[1 1 1] Show TP Mesh
            (`SceneComponent.SetHiddenInGame` (`self.Mesh`) false false)
            ;;;[1 1 1] Show TP Firearm
            (`self.SetActorHiddenInGame` (`self.GetCurrentTPFirearm`) false)
            (bind _asbp_firearm_actor_common_2 (cast `/Game/CHARACTER_SYSTEM_V2/Blueprints/FirearmSystem/BP_FirearmActorCommon` (`self.GetCurrentTPFirearm`)))
            (`PrimitiveComponent.SetCastHiddenShadow` (`/Game/CHARACTER_SYSTEM_V2/Blueprints/FirearmSystem/BP_FirearmActorCommon.FirearmMesh` _asbp_firearm_actor_common_2) false))))
      (:`NewEnumerator1`
        ;;[1 1 1] FP Mode
        (if `Scope ON`
          ;;;[1 1 1] Hide FPArms
          (`SceneComponent.SetVisibility` (`self.FPArms`) false false)
          ;;;[1 1 1] Hide FP Firearm
          (`/Engine/EditorBlueprintResources/StandardMacros.IsValid` (`self.GetCurrentFPFirearm`)
            (:`Is Valid`
              (`self.SetActorHiddenInGame` (`self.GetCurrentFPFirearm`) true)))
          (else
            ;;;[1 1 1] Show FPArms
            (`SceneComponent.SetVisibility` (`self.FPArms`) true false)
            ;;;[1 1 1] Show FP Firearm
            (`/Engine/EditorBlueprintResources/StandardMacros.IsValid` (`self.GetCurrentFPFirearm`)
              (:`Is Valid`
                (`self.SetActorHiddenInGame` (`self.GetCurrentFPFirearm`) false)))))))))

(event `self.ServerHandleChildAttachOnCoverInteraction`
  (params (WeaponState :type "/Game/CHARACTER_SYSTEM_V2/Blueprints/DATA/E/E_CharacterWeaponState Enum" :default "NewEnumerator0"))
  ;[1 1 1] HANDLE ATACH & SHOW WEAPON ON COVER ACTION
  ;;[0.1778 0 1] PARENT INPUT
  (if (`|EnumEquality` (`self.CharacterType`) "NewEnumerator2")
    (switch `/Game/CHARACTER_SYSTEM_V2/Blueprints/DATA/E/E_CharacterCameraMode` (`self.GetCurrentCameraMode`)
      (:`NewEnumerator0`
        (switch `/Game/CHARACTER_SYSTEM_V2/Blueprints/DATA/E/E_CharacterWeaponState` WeaponState
          (:`NewEnumerator1`
            ;;[1 0.6824 0] TO INVENTORY SYSTEM
            (`/Game/CHARACTER_SYSTEM_V2/Blueprints/InventorySystem/AC_InventorySystem.ServerAttachCurrentFirearmToBackPackOnAction` (`self.InventorySystem`)))
          (:`NewEnumerator2`
            (`self.MulticastShowCurrentEquipmentOnAction` false))))
      (:`NewEnumerator1`
        (switch `/Game/CHARACTER_SYSTEM_V2/Blueprints/DATA/E/E_CharacterWeaponState` WeaponState
          (:`NewEnumerator1`
            ;;[1 0.6824 0] TO INVENTORY SYSTEM
            (`/Game/CHARACTER_SYSTEM_V2/Blueprints/InventorySystem/AC_InventorySystem.ServerAttachCurrentFirearmToBackPackOnAction` (`self.InventorySystem`))
            (`self.ClientShowCurrentFirearmOnAction` false))
          (:`NewEnumerator2`
            (`self.MulticastShowCurrentEquipmentOnAction` false)
            (`self.ClientShowCurrentEquipmentOnAction` false)))))))

(event `self.ServerHandleChildReAttachOnCoverInteraction`
  (params (WeaponState :type "/Game/CHARACTER_SYSTEM_V2/Blueprints/DATA/E/E_CharacterWeaponState Enum" :default "NewEnumerator0"))
  ;[1 1 1] HANDLE ATACH & SHOW WEAPON ON COVER ACTION
  ;;[0.1778 0 1] PARENT INPUT
  (if (`|EnumEquality` (`self.CharacterType`) "NewEnumerator2")
    (switch `/Game/CHARACTER_SYSTEM_V2/Blueprints/DATA/E/E_CharacterCameraMode` (`self.GetCurrentCameraMode`)
      (:`NewEnumerator0`
        (switch `/Game/CHARACTER_SYSTEM_V2/Blueprints/DATA/E/E_CharacterWeaponState` WeaponState
          (:`NewEnumerator1`
            (`self.ServerAttachTPFirearm`))
          (:`NewEnumerator2`
            (`self.MulticastShowCurrentEquipmentOnAction` true))))
      (:`NewEnumerator1`
        (switch `/Game/CHARACTER_SYSTEM_V2/Blueprints/DATA/E/E_CharacterWeaponState` WeaponState
          (:`NewEnumerator1`
            (`self.ServerAttachTPFirearm`)
            (`self.ClientShowCurrentFirearmOnAction` true))
          (:`NewEnumerator2`
            (`self.MulticastShowCurrentEquipmentOnAction` true)
            (`self.ClientShowCurrentEquipmentOnAction` true)))))))

(event `ClientInitTPCameraAdvancedOnSpawn`
  (params (`Set Preset On Initialize?` :type Boolean))
  ;[1 1 1] TP CAMERA
  ;;[1 1 1] Init Camera On Spawn
  (`/Engine/EditorBlueprintResources/StandardMacros.IsValid` (`self.PlayerCameraTP`)
    (:`Is Valid`
      (`/Engine/EditorBlueprintResources/StandardMacros.IsValid` (`self.SpringArm`)
        (:`Is Valid`
          (`/Engine/EditorBlueprintResources/StandardMacros.IsValid` (`self.FPSCamera`)
            (:`Is Valid`
              ;;;[1 0.6824 0] TO PLAYER CAMERA TP
              (`/Game/CHARACTER_SYSTEM_V2/Blueprints/PlayerCameraTP/AC_PlayerCameraTP.ClientSetStartCameraMode` (`self.PlayerCameraTP`) (`self.SpringArm`) (`self.FPSCamera`) "StandIdle" `Set Preset On Initialize?`))))))))

(event `ClientTPCameraAdvancedChangePreset`
  (params (NewCameraPreset :type Name))
  ;[1 1 1] TP CAMERA
  ;;[1 1 1] Change Camera Preset
  (`/Game/CHARACTER_SYSTEM_V2/Blueprints/PlayerCameraTP/AC_PlayerCameraTP.ClientOpenGateChange` (`self.PlayerCameraTP`))
  (`/Game/CHARACTER_SYSTEM_V2/Blueprints/PlayerCameraTP/AC_PlayerCameraTP.ClientChangeCameraMode` (`self.PlayerCameraTP`) (`self.SpringArm`) (`self.FPSCamera`) NewCameraPreset))

(event `ClientDifineNewCameraPreset`
  (params (MainCharacterState :type "/Game/CHARACTER_SYSTEM_V2/Blueprints/DATA/E/E_CharacterMainState Enum" :default "NewEnumerator0"))
  (bind _characterweaponstate (`self.GetCharacterWeaponState`))
  (bind _characterweaponstate_2 (`self.GetCharacterWeaponState`))
  (bind _characterweaponstate_3 (`self.GetCharacterWeaponState`))
  ;[1 1 1] TP CAMERA
  ;;[1 1 1] Difine New Camera Preset
  ;;;[1 0.2552 0.2552] CHECK: TP Camera & No Changing Camera Mode
  (if (`|EnumEquality` (`self.GetCurrentCameraMode`) "NewEnumerator0")
    (if (not (`self.GetInChangingCameraMode`))
      ;;;[1 0.2552 0.2552] CHECK: Scope off
      (if (not (`/Game/CHARACTER_SYSTEM_V2/Blueprints/FirearmSystem/AC_FirearmScopeController.GetInScope` (`self.GetFirearmScopeController`)))
        (switch `/Game/CHARACTER_SYSTEM_V2/Blueprints/DATA/E/E_CharacterMainState` MainCharacterState
          (:`NewEnumerator0`
            (`self.ClientTPCameraAdvancedChangePreset` "StandIdle"))
          (:`NewEnumerator12`
            (`self.ClientTPCameraAdvancedChangePreset` "StandMove"))
          (:`NewEnumerator1`
            ;;;[1 0.2552 0.2552] CHECK: NOT NoWeapon, Equipment, Melee
            (if (not (or (`|EnumEquality` _characterweaponstate_2 "NewEnumerator0") (`|EnumEquality` _characterweaponstate_2 "NewEnumerator2") (`|EnumEquality` _characterweaponstate_2 "NewEnumerator3"))) :!label _label
              (`self.ClientTPCameraAdvancedChangePreset` "StandAim")))
          (:`NewEnumerator13`
            (goto _label))
          (:`NewEnumerator2`
            (`self.ClientTPCameraAdvancedChangePreset` "CrouchIdle"))
          (:`NewEnumerator14`
            (`self.ClientTPCameraAdvancedChangePreset` "CrouchMove"))
          (:`NewEnumerator3`
            (if (not (or (`|EnumEquality` _characterweaponstate_3 "NewEnumerator0") (`|EnumEquality` _characterweaponstate_3 "NewEnumerator2") (`|EnumEquality` _characterweaponstate_3 "NewEnumerator3"))) :!label _label_2
              (`self.ClientTPCameraAdvancedChangePreset` "CrouchAim")))
          (:`NewEnumerator15`
            (goto _label_2))
          (:`NewEnumerator4`
            (`self.ClientTPCameraAdvancedChangePreset` "ProneIdle"))
          (:`NewEnumerator16`
            (`self.ClientTPCameraAdvancedChangePreset` "ProneMove"))
          (:`NewEnumerator5`
            (if (not (or (`|EnumEquality` _characterweaponstate "NewEnumerator0") (`|EnumEquality` _characterweaponstate "NewEnumerator2") (`|EnumEquality` _characterweaponstate "NewEnumerator3"))) :!label _label_3
              (`self.ClientTPCameraAdvancedChangePreset` "ProneAim")))
          (:`NewEnumerator17`
            (goto _label_3))
          (:`NewEnumerator6`
            (`self.ClientTPCameraAdvancedChangePreset` "Sprint"))
          (:`NewEnumerator7`
            (`self.ClientTPCameraAdvancedChangePreset` "HighCoverClimb" :!label _label_4))
          (:`NewEnumerator8`
            (goto _label_4))
          (:`NewEnumerator9`
            (goto _label_4))
          (:`NewEnumerator10`
            (goto _label_4))
          (:`NewEnumerator11`
            (`self.ClientTPCameraAdvancedChangePreset` "Dead")))))))

(event `ClientHandleTPCameraMirrorInput`
  ;[1 1 1] TP CAMERA
  ;;[1 1 1] Camera Mirror
  ;;;[1 0.2552 0.2552] CHECK: TP Camera & No Changing Camera Mode
  (if (`|EnumEquality` (`self.GetCurrentCameraMode`) "NewEnumerator0")
    (if (not (`self.GetInChangingCameraMode`))
      ;;;[1 0.6824 0] TO PLAYER CAMERA TP
      (`/Game/CHARACTER_SYSTEM_V2/Blueprints/PlayerCameraTP/AC_PlayerCameraTP.ClientUpdateCameraMirror` (`self.PlayerCameraTP`)))))

(event `ClientSwitchAttachignTPCamera`
  (params (CharacterState :type "/Game/CHARACTER_SYSTEM_V2/Blueprints/DATA/E/E_CharacterMainState Enum" :default "NewEnumerator0"))
  ;[1 1 1] TP CAMERA
  ;;[1 1 1] Switch Attacing TP Camera
  (if (or (`|EnumEquality` CharacterState "NewEnumerator7") (`|EnumEquality` CharacterState "NewEnumerator8") (`|EnumEquality` CharacterState "NewEnumerator9") (`|EnumEquality` CharacterState "NewEnumerator10"))
    (`KismetSystemLibrary.Delay` 0.2)
    (`SceneComponent.K2_AttachToComponent` (`self.SpringArm`) (`self.Mesh`) "None" "KeepRelative" "KeepRelative" "KeepRelative" true)
    (`SceneComponent.K2_SetRelativeLocation` (`self.SpringArm`) (0.0 0.0 150.0) false true)
    (else
      (`KismetSystemLibrary.Delay` 0.3)
      (`SceneComponent.K2_AttachToComponent` (`self.SpringArm`) (`self.Mesh`) "VB TPCamRootPoint" "KeepRelative" "KeepRelative" "KeepRelative" true)
      (`SceneComponent.K2_SetRelativeLocation` (`self.SpringArm`) (0.0 0.0 0.0) false false))))

(event `ClientChangeCameraMode`
  (bind _playercamerafp (`self.PlayerCameraFP`))
  ;[1 1 1] CHANGING CAMERA MODE
  ;;[1 0.2552 0.2552] CHECK: Condition for switching camera mode
  (if (not (or (`self.Get in Scope`) (`self.GetInJumpOverLowCover`) (`self.GetInClimbLowCover`) (`self.GetInVaultHighCover`) (`self.GetInClimbHighCover`) (`self.Get In Use Equipment`) (`self.GetInDead`) (`/Game/CHARACTER_SYSTEM_V2/Blueprints/PlayerCameraFP/AC_PlayerCameraFP.GetInChangingOnAim` (`self.PlayerCameraFP`)) (`/Game/CHARACTER_SYSTEM_V2/Blueprints/PlayerCameraTP/AC_PlayerCameraTP.Get In Transition Between Presets` (`self.PlayerCameraTP`)) (`self.GetInChangingCameraMode`) (`self.Get In Switch Weapon`)))
    ;;[1 0 0.1451] TO PARENT CHARACTER FP
    (`self.ClientUpdateInChangingCameraMode` true)
    ;;[1 0.2552 0.2552] CHECK: Current camera mode
    (switch `/Game/CHARACTER_SYSTEM_V2/Blueprints/DATA/E/E_CharacterCameraMode` (`self.GetCurrentCameraMode`)
      (:`NewEnumerator0`
        ;;[1 1 1] TO FP View
        ;;;[1 0 0.1451] TO PARENT CHARACTER COMMON
        (`self.SetCurrentCameraState` "NewEnumerator1")
        ;;;[1 0.6824 0] TO PLAYER CAMERA TP
        (`/Game/CHARACTER_SYSTEM_V2/Blueprints/PlayerCameraTP/AC_PlayerCameraTP.ClientUpdateFPCameraState` (`self.PlayerCameraTP`) true)
        ;;;[1 0.6824 0] TO PLAYER CAMERA FP
        (`/Game/CHARACTER_SYSTEM_V2/Blueprints/PlayerCameraFP/AC_PlayerCameraFP.ClientUpdateFPCameraState` (`self.PlayerCameraFP`) true)
        ;;;[1 1 1] Define FP FOV
        (set `self.FinalFPFOV` (select `bool` (`self.GetInAimDownSight`) :`false` (`/Game/CHARACTER_SYSTEM_V2/Blueprints/PlayerCameraFP/AC_PlayerCameraFP.CameraDefaultFOV` _playercamerafp) :`true` (`/Game/CHARACTER_SYSTEM_V2/Blueprints/PlayerCameraFP/AC_PlayerCameraFP.CameraAimFOV` _playercamerafp)))
        ;;;[1 1 1] Interpolation
        (bind (_direction _updatecoeff) (`Timeline|ChangeCameraModeTPStoFPS` :!via `PlayFromStart`)
          (:`Update`
            (`|ExecutionSequence`
              (:`then_0`
                (if (>= _updatecoeff 0.8)
                  (`/Engine/EditorBlueprintResources/StandardMacros.DoOnce` false :!label _label_5
                    (:`Completed`
                      ;;;;[1 0 0.1437] TO PARENT CHARACTER FP
                      (`self.ServerActivateFPCharacterMode`)
                      ;;;;[1 0 0.1437] TO PARENT
                      (`self.ClientUpdateInChangingCameraMode` false)
                      ;;;;[1 0.6824 0] TO PLAYER CAMERA FP
                      (`/Game/CHARACTER_SYSTEM_V2/Blueprints/PlayerCameraFP/AC_PlayerCameraFP.ClientUpdateDOFOnChangeCameraMode` (`self.PlayerCameraFP`) (`self.GetInAimDownSight`))
                      ;;;;[1 0.6824 0] TO INVENTORY SYSTEM
                      (`/Game/CHARACTER_SYSTEM_V2/Blueprints/InventorySystem/AC_InventorySystem.ClientHandleChangeCameraMode` (`self.InventorySystem`))))))
              (:`then_1`
                (`self.SetCameraPreset` (`|EaseFunction` "Linear" _updatecoeff (`SpringArmComponent.TargetArmLength` (`self.SpringArm`))) (`|EaseFunction` "Linear" _updatecoeff (`SpringArmComponent.SocketOffset` (`self.SpringArm`)) (`self.FPCameraSpringSocetOffSetDefault`)) (`|EaseFunction` "Linear" _updatecoeff (`CameraComponent.FieldOfView` (`self.FPSCamera`)) (`self.FinalFPFOV`)))
                (goto _label_5 :!via `Reset`))))
          (:`Finished`
            ;;;[1 1 1] On Finish transition
            ;;;;[1 0.6824 0] TO PLAYER CAMERA FP
            (`/Game/CHARACTER_SYSTEM_V2/Blueprints/PlayerCameraFP/AC_PlayerCameraFP.ClientUpdateCurrentFOV` (`self.PlayerCameraFP`) (`self.FinalFPFOV`))
            ;;;;[1 0.6824 0] TP PLAYER CAMERA FP
            (`/Game/CHARACTER_SYSTEM_V2/Blueprints/PlayerCameraFP/AC_PlayerCameraFP.ClientChangeCameraOnAim` (`self.PlayerCameraFP`) (`self.GetInAimDownSight`)))))
      (:`NewEnumerator1`
        ;;[1 1 1] To TP view
        ;;;[1 0 0.1451] TO PARENT CHARACTER COMMON
        (`self.SetCurrentCameraState` "NewEnumerator0")
        ;;;[1 0.6824 0] TO PLAYER CAMERA TP
        (`/Game/CHARACTER_SYSTEM_V2/Blueprints/PlayerCameraTP/AC_PlayerCameraTP.ClientUpdateFPCameraState` (`self.PlayerCameraTP`) false)
        ;;;[1 0.6824 0] TO PLAYER CAMERA FP
        (`/Game/CHARACTER_SYSTEM_V2/Blueprints/PlayerCameraFP/AC_PlayerCameraFP.ClientUpdateFPCameraState` (`self.PlayerCameraFP`) false)
        (`|ExecutionSequence`
          (:`then_0`
            (`self.ServerActivateTPCharacterMode`)
            ;;;[1 0.6824 0] TO INVENTORY SYSTEM
            (`/Game/CHARACTER_SYSTEM_V2/Blueprints/InventorySystem/AC_InventorySystem.ClientHandleChangeCameraMode` (`self.InventorySystem`))
            (`self.DefineTPSCameraTransferPreset`)
            ;;;[1 0.6824 0] TO PLAYER CAMERA TP
            (`/Game/CHARACTER_SYSTEM_V2/Blueprints/PlayerCameraTP/AC_PlayerCameraTP.SetCurrentCameraPreset` (`self.PlayerCameraTP`) (`self.TransferTPSCameraName`))
            ;;;[1 1 1] Interpolation
            (bind (_direction_2 _updatecoeff_2) (`Timeline|ChangeCameraModeFPStoTPS` :!via `PlayFromStart`)
              (:`Update`
                ;;;;[1 0.6824 0] TO PLAYER CAMERA TP
                (bind (_targetarmlength _socketoffset _targetoffset _fov) (`/Game/CHARACTER_SYSTEM_V2/Blueprints/PlayerCameraTP/AC_PlayerCameraTP.GetCameraSettingsFromPreset` (`self.PlayerCameraTP`) (`self.TransferTPSCameraName`)))
                (`self.SetCameraPreset` (`|EaseFunction` "Linear" _updatecoeff_2 (`SpringArmComponent.TargetArmLength` (`self.SpringArm`)) _targetarmlength) (`|EaseFunction` "Linear" _updatecoeff_2 (`SpringArmComponent.SocketOffset` (`self.SpringArm`)) _socketoffset) (`|EaseFunction` "Linear" _updatecoeff_2 (`CameraComponent.FieldOfView` (`self.FPSCamera`)) _fov)))
              (:`Finished`
                ;;;[1 1 1] On Finish transition
                ;;;;[1 0 0.1437] TO PARENT CHARACTER FP
                (`self.ClientUpdateInChangingCameraMode` false)
                ;;;;[1 0.6824 0] TO PLAYER CAMERA FP
                (`/Game/CHARACTER_SYSTEM_V2/Blueprints/PlayerCameraTP/AC_PlayerCameraTP.ClientUpdateDOFOnChangeCameraMode` (`self.PlayerCameraTP`) (`self.GetInAimDownSight`))
                (`self.ClientDifineNewCameraPreset` (`self.GetMainCharacterState`)))))
          (:`then_1`
            (`/Engine/EditorBlueprintResources/StandardMacros.DoOnce` false
              (:`Completed`
                ;;;[1 1 1] Off owner no see
                (`PrimitiveComponent.SetOwnerNoSee` (`self.Mesh`) false)))))))))

(event `self.ServerChildHandleVehicleOn`
  ;[1 1 1] HANDLE VEHICLE
  ;;[1 1 1] Handle Vehicle on
  ;;;[0.1778 0 1] PARENT INPUT
  (switch `/Game/CHARACTER_SYSTEM_V2/Blueprints/DATA/E/E_CharacterCameraMode` (`self.GetCurrentCameraMode`)
    (:`NewEnumerator0`
      (`self.MulticastChildHandleVehicleOn`))
    (:`NewEnumerator1`
      ;;;[1 0 0.1451] TO PARENT CHARACTER COMMON
      (`self.MulticastHandleVehicleOn`))))

(event `MulticastChildHandleVehicleOn`
  ;[1 1 1] HANDLE VEHICLE
  ;;[1 1 1] Handle Vehicle on
  (`SceneComponent.SetVisibility` (`self.Backpack`) false false)
  (`SceneComponent.SetVisibility` (`self.Mesh`) false false))

(event `self.ServerChildHandleVehicleOff`
  ;[1 1 1] HANDLE VEHICLE
  ;;[1 1 1] Handle Vehicle off
  ;;;[0.1778 0 1] PARENT INPUT
  (switch `/Game/CHARACTER_SYSTEM_V2/Blueprints/DATA/E/E_CharacterCameraMode` (`self.GetCurrentCameraMode`)
    (:`NewEnumerator0`
      (`self.MulticastChildHandleVehicleOff`))
    (:`NewEnumerator1`
      ;;;[1 0 0.1451] TO PARENT CHARACTER COMMON
      (`self.MulticastHandleVehicleOff`))))

(event `MulticastChildHandleVehicleOff`
  ;[1 1 1] HANDLE VEHICLE
  ;;[1 1 1] Handle Vehicle off
  (`SceneComponent.SetVisibility` (`self.Backpack`) true false)
  (`SceneComponent.SetVisibility` (`self.Mesh`) true false))

(fn `DefineTPSCameraTransferPreset`
  (switch `/Game/CHARACTER_SYSTEM_V2/Blueprints/DATA/E/E_CharacterMainState` (`self.GetMainCharacterState`)
    (:`NewEnumerator0`
      (set `self.TransferTPSCameraName` "StandIdle"))
    (:`NewEnumerator12`
      (set `self.TransferTPSCameraName` "StandMove"))
    (:`NewEnumerator1`
      (set `self.TransferTPSCameraName` "StandAim" :!label _label))
    (:`NewEnumerator13`
      (goto _label))
    (:`NewEnumerator2`
      (set `self.TransferTPSCameraName` "CrouchIdle"))
    (:`NewEnumerator14`
      (set `self.TransferTPSCameraName` "CrouchMove"))
    (:`NewEnumerator3`
      (set `self.TransferTPSCameraName` "CrouchAim" :!label _label_2))
    (:`NewEnumerator15`
      (goto _label_2))
    (:`NewEnumerator4`
      (set `self.TransferTPSCameraName` "ProneIdle"))
    (:`NewEnumerator16`
      (set `self.TransferTPSCameraName` "ProneMove"))
    (:`NewEnumerator5`
      (set `self.TransferTPSCameraName` "ProneAim" :!label _label_3))
    (:`NewEnumerator17`
      (goto _label_3))
    (:`NewEnumerator6`
      (set `self.TransferTPSCameraName` "Sprint"))
    (:`NewEnumerator7`
      (set `self.TransferTPSCameraName` "HighCoverClimb" :!label _label_4))
    (:`NewEnumerator8`
      (goto _label_4))
    (:`NewEnumerator9`
      (goto _label_4))
    (:`NewEnumerator10`
      (goto _label_4))
    (:`NewEnumerator11`
      (set `self.TransferTPSCameraName` "Dead"))))

(fn `SetCameraPreset`
  (params (`Target Arm Length` :type "Float (single-precision)") (`Socket Offset` :type "Vector Structure") (`Field Of View` :type "Float (single-precision)"))
  (`/Engine/EditorBlueprintResources/StandardMacros.IsValid` (`self.SpringArm`)
    (:`Is Valid`
      (`/Engine/EditorBlueprintResources/StandardMacros.IsValid` (`self.FPSCamera`)
        (:`Is Valid`
          (set `SpringArmComponent.TargetArmLength` `Target Arm Length` (`self.SpringArm`))
          (set `SpringArmComponent.SocketOffset` `Socket Offset` (`self.SpringArm`))
          (set `CameraComponent.FieldOfView` `Field Of View` (`self.FPSCamera`)))))))

(fn `UserConstructionScript`
  (`parent.UserConstructionScript`))