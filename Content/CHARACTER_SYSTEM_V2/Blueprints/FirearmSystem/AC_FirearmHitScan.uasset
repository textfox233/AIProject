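; Actor component that performs client-side hitscan line traces for the firearm system.
; Single or multi-trace requests from AC_FirearmSystem run object-type traces, ignoring the owner and inventory actors of player 0's pawn.
; Each hit becomes a hitscan descriptor with location, normal, actor, bone and surface type.
; Results are stored for getters and passed back to the owner's AC_FirearmSystem.
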(event `ClientHandleCreateSingleLineTrace`
  (params (StartPoint :type "Vector Structure") (EndPoint :type "Vector Structure"))
  ;[1 1 1] MAIN
  ;;[1 0.1179 0] INPUT FROM FIREARMSYSTEM
  (bind _hitscandesc (`self.CreateLineTrace` StartPoint EndPoint))
  (bind _output_get (set `self.SingleHitScan` _hitscandesc))
  ;;[0.9739 1 0] BI OUTPUT TO FirearmSystem
  (`/Game/CHARACTER_SYSTEM_V2/Blueprints/FirearmSystem/AC_FirearmSystem.ClientSingleTraceCreated` (`self.GetFirearmSystem`) _output_get))

(event `ClientHandleCreateMultiLineTrace`
  (params (MultiTraceDesc :type "Array of /Game/CHARACTER_SYSTEM_V2/Blueprints/DATA/STR/STR_FirearmMultiTraceDesc Structure"))
  ;[1 1 1] MAIN
  ;;[1 0.1179 0] INPUT FROM FIREARMSYSTEM
  (`KismetArrayLibrary.Array_Clear` (`self.MultiHitScanArray`))
  (`KismetArrayLibrary.Array_Resize` (`self.MultiHitScanArray`) (`KismetArrayLibrary.Array_Length` MultiTraceDesc))
  (for _array_element MultiTraceDesc
    (bind (_startpoint _endpoint) (break `/Game/CHARACTER_SYSTEM_V2/Blueprints/DATA/STR/STR_FirearmMultiTraceDesc` _array_element))
    (bind _hitscandesc (`self.CreateLineTrace` _startpoint _endpoint))
    (`KismetArrayLibrary.Array_Add` (`self.MultiHitScanArray`) _hitscandesc))
  ;;[0.9739 1 0] BI OUTPUT TO FirearmSystem
  (`/Game/CHARACTER_SYSTEM_V2/Blueprints/FirearmSystem/AC_FirearmSystem.ClientMultiTraceCreated` (`self.GetFirearmSystem`) (`self.MultiHitScanArray`)))

(fn `CreateLineTrace`
  (params (Start :type "Vector Structure") (End :type "Vector Structure"))
  (returns (HitScanDesc :type "/Game/CHARACTER_SYSTEM_V2/Blueprints/DATA/STR/STR_FirearmHitScanDesc Structure"))
  (locals (loc_actors_for_ingnor :type "Array of Actor Object Reference"))
  (set `local.loc_actors_for_ingnor` (`/Game/CHARACTER_SYSTEM_V2/Blueprints/InventorySystem/AC_InventorySystem.GetAllInventoryActors` (`self.GetInventorySystem`)))
  (`KismetArrayLibrary.Array_AddUnique` (`local.loc_actors_for_ingnor`) (`self.GetOwner` self))
  (bind _outhit (`KismetSystemLibrary.LineTraceSingleForObjects` Start End (`self.Object Types`) false (`local.loc_actors_for_ingnor`) "None" true (struct :`R` 1.0 :`A` 1.0) (struct :`G` 1.0 :`A` 1.0) 2.0))
  (bind (_bblockinghit _binitialoverlap _time _distance _location _impactpoint _normal _impactnormal _physmat _hitactor _hitcomponent _hitbonename _bonename _hititem _elementindex _faceindex _tracestart _traceend) (`GameplayStatics.BreakHitResult` _outhit))
  (return (make `/Game/CHARACTER_SYSTEM_V2/Blueprints/DATA/STR/STR_FirearmHitScanDesc` _bblockinghit _distance _tracestart _traceend _location _normal _hitactor _hitbonename (`GameplayStatics.GetSurfaceType` _outhit))))

(fn `GetFirearmSystem`
  (returns (FirearmSystem :type "/Game/CHARACTER_SYSTEM_V2/Blueprints/FirearmSystem/AC_FirearmSystem Object Reference"))
  (bind _returnvalue (`Actor.GetComponentByClass` (`self.GetOwner` self) "/Game/CHARACTER_SYSTEM_V2/Blueprints/FirearmSystem/AC_FirearmSystem.AC_FirearmSystem_C"))
  (`/Engine/EditorBlueprintResources/StandardMacros.IsValid` _returnvalue
    (:`Is Valid`
      (return _returnvalue))))

(fn `GetInventorySystem`
  (returns (InventorySystem :type "/Game/CHARACTER_SYSTEM_V2/Blueprints/InventorySystem/AC_InventorySystem Object Reference"))
  (bind _returnvalue (`Actor.GetComponentByClass` (`Controller.K2_GetPawn` (`GameplayStatics.GetPlayerController` 0)) "/Game/CHARACTER_SYSTEM_V2/Blueprints/InventorySystem/AC_InventorySystem.AC_InventorySystem_C"))
  (`/Engine/EditorBlueprintResources/StandardMacros.IsValid` _returnvalue
    (:`Is Valid`
      (return _returnvalue))))

(fn `GetValueMultiHitScanDesc`
  (returns (MultiHitScanDesc :type "Array of /Game/CHARACTER_SYSTEM_V2/Blueprints/DATA/STR/STR_FirearmHitScanDesc Structure"))
  (return (`self.MultiHitScanArray`)))

(fn `GetValueSingleHitScanDesc`
  (returns (SingleHitScanDesc :type "/Game/CHARACTER_SYSTEM_V2/Blueprints/DATA/STR/STR_FirearmHitScanDesc Structure"))
  (return (`self.SingleHitScan`)))