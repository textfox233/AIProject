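; Firearm component that calculates bullet spread on the client and hands randomized camera-based trace points for single or multi-trace (shotgun) shots to AC_FirearmSystem.
; Spread angle blends the firearm's min and max angles by a spread energy level, scaled by an owner-state coefficient and a first-person mode multiplier.
; Each shot drains energy via a decrement curve, and a looping timer, gated by a DoOnce, regenerates it to max.
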(event `ClientHandleUpdateMinSpreadOnInitFirearm`
  ;[1 1 1] UPDATE ON INIT FIREARM
  ;;[1 0.1179 0] INPUT FROM FIREARMSYSTEM
  ;;[1 1 1] Init start spread angle
  (set `self.CurrentSpreadOwnerInfCoeff` (`/Game/CHARACTER_SYSTEM_V2/Blueprints/FirearmSystem/AC_FirearmOwnerStateHandler.GetCurrentSpreadCoeff` (`self.GetFirearmOwnerStateHandler`)))
  (set `self.CurrentSpreadAngle` (* (`self.GetMinRandomSpreadAngle`) (`self.CurrentSpreadOwnerInfCoeff`) (`self.Spread Scale in FP Mode`)))
  ;;[1 1 1] Initialize Array for Start / End Points for multi trace shot (shotgun)
  (if (`|EnumEquality` (`self.GetTraceType`) "NewEnumerator1")
    (`KismetArrayLibrary.Array_Clear` (`self.MultiTraceArray`))
    (`KismetArrayLibrary.Array_Resize` (`self.MultiTraceArray`) (`self.GetMultiTraceAmount`))))

(event `ClientHandleUpdateSpreadInfOnIteratationStep`
  ;[1 1 1] UPDATE OWNER INFLUENCE ON SPREAD
  ;;[1 0.1179 0] INPUT FROM FIREARMSYSTEM
  (set `self.CurrentSpreadOwnerInfCoeff` (`/Game/CHARACTER_SYSTEM_V2/Blueprints/FirearmSystem/AC_FirearmOwnerStateHandler.GetCurrentSpreadCoeff` (`self.GetFirearmOwnerStateHandler`)))
  (`self.ClientUpdateSpreadAngleOnUpdateInfluence`))

(event `ClientHandleToggleOnFPMode`
  (params (ToggleOn :type Boolean))
  ;[1 1 1] TOGGLE FP MODE
  ;;[1 0.1179 0] INPUT FROM FIREARMSYSTEM
  (if ToggleOn
    (set `self.Spread Scale in FP Mode` (`self.GetSpreadScaleInFPMode`))
    (else
      (set `self.Spread Scale in FP Mode` 1.0)))
  (`self.ClientUpdateSpreadAngleOnUpdateInfluence`))

(event `ClientHandleUpdateSpreadOnShot`
  ;[1 1 1] ON SHOT (SINGLE TRACE/ MULTI TRACE)
  ;;[1 0.1179 0] INPUT FROM FIREARMSYSTEM
  ;;[1 1 1] Step 1. Update Spread Angle
  (`self.ClientUpdateSpreadAngleAfterShot`)
  (switch `/Game/CHARACTER_SYSTEM_V2/Blueprints/DATA/E/E_FirearmTraceType` (`self.GetTraceType`)
    (:`NewEnumerator0`
      ;;[1 1 1] SingleTrace Shot
      (`self.ClientUpdateTraceStartEnd`)
      ;;;[1 0.6824 0] BI OUTPUT TO Firearm System
      (`/Game/CHARACTER_SYSTEM_V2/Blueprints/FirearmSystem/AC_FirearmSystem.ClientHandleReadyToSingleShot` (`self.GetFirearmSystem`) (`self.TraceStartPoint`) (`self.TraceEndPoint`))
      (`self.ClientReduceSpreadEnergyAfterShot`))
    (:`NewEnumerator1`
      ;;[1 1 1] MultiTrace Shot
      (`KismetArrayLibrary.Array_Clear` (`self.MultiTraceArray`))
      (for _index (range (`self.GetMultiTraceAmount`))
        (set `self.CurrentMutliTraceStepIndex` _index)
        (`self.ClientUpdateTraceStartEnd`))
      ;;;[1 0.6824 0] BI OUTPUT TO Firearm System
      (`/Game/CHARACTER_SYSTEM_V2/Blueprints/FirearmSystem/AC_FirearmSystem.ClientHandleReadyToMultiShot` (`self.GetFirearmSystem`) (`self.MultiTraceArray`))
      (`self.ClientReduceSpreadEnergyAfterShot`))))

(event `ClientUpdateSpreadAngleOnUpdateInfluence`
  ;[1 1 1] 1. UPDATE SPREAD ANGLE
  ;;[1 1 1] Calculate Current Spread Energy Coeff based on Current Spread Energy level
  (set `self.CurrentSpreadEnergyCoeff` (`KismetMathLibrary.Abs` (- (/ (`self.CurrentSpreadEnergy`) 100.0) 1.0)) :!label _label)
  ;;[1 1 1] Calculation Current Spread Angle based on Energy Coeff
  (set `self.CurrentSpreadAngle` (* (`KismetMathLibrary.Abs` (+ (* (`self.GetMaxRandomSpreadAngle`) (`self.CurrentSpreadEnergyCoeff`)) (* (`self.GetMinRandomSpreadAngle`) (`KismetMathLibrary.Abs` (- 1.0 (`self.CurrentSpreadEnergyCoeff`)))))) (`self.CurrentSpreadOwnerInfCoeff`) (`self.Spread Scale in FP Mode`))))

(event `ClientUpdateSpreadAngleAfterShot`
  ;[1 1 1] 1. UPDATE SPREAD ANGLE
  ;;[1 1 1] Check Main Seggins of Weapon System: Use Spread ?
  (if (`self.UseSpread ?`)
    (goto _label)
    (else
      ;;[1 1 1] If Spread is not use, current spread angle == 0
      (set `self.CurrentSpreadAngle` 0.0))))

(event `ClientUpdateTraceStartEnd`
  ;[1 1 1] 2. UPDATE TRACE START & END
  ;;[1 1 1] Start Point
  (set `self.TraceStartPoint` (`SceneComponent.K2_GetComponentLocation` (`self.GetMainPlayerCamera`)))
  ;;[1 1 1] End Point
  (set `self.TraceEndPoint` (+ (`SceneComponent.K2_GetComponentLocation` (`self.GetMainPlayerCamera`)) (* (`KismetMathLibrary.GetForwardVector` (`KismetMathLibrary.MakeRotator` (.roll (`SceneComponent.K2_GetComponentRotation` (`self.GetMainPlayerCamera`))) (+ (.pitch (`SceneComponent.K2_GetComponentRotation` (`self.GetMainPlayerCamera`))) (`KismetMathLibrary.RandomFloatInRange` (* (`self.CurrentSpreadAngle`) -1.0) (`self.CurrentSpreadAngle`))) (+ (.yaw (`SceneComponent.K2_GetComponentRotation` (`self.GetMainPlayerCamera`))) (`KismetMathLibrary.RandomFloatInRange` (* (`self.CurrentSpreadAngle`) -1.0) (`self.CurrentSpreadAngle`))))) (`self.ShootingMaxDistance`))))
  ;;[1 1 1] Form Trace Array for MultiTrace
  (if (`|EnumEquality` (`self.GetTraceType`) "NewEnumerator1")
    (`KismetArrayLibrary.Array_Add` (`self.MultiTraceArray`) (make `/Game/CHARACTER_SYSTEM_V2/Blueprints/DATA/STR/STR_FirearmMultiTraceDesc` (`self.TraceStartPoint`) (`self.TraceEndPoint`)))))

(event `ClientReduceSpreadEnergyAfterShot`
  ;[1 1 1] 4. RECALCULATION SPREAD ENERGY
  ;;[1 1 1] Requce Spread Enegry After Shot
  ;;;[1 1 1] Check Main Seggins of Weapon System: Use Spread ?
  (if (`self.UseSpread ?`)
    (`/Engine/EditorBlueprintResources/StandardMacros.IsValid` (`self.GetEnergyDecrementCurve`)
      (:`Is Valid`
        ;;;[1 1 1] Decrement Current Spread Energy base on Curent Spread Energy and Decrement Curve
        (set `self.CurrentSpreadEnergy` (`KismetMathLibrary.FClamp` (- (`self.CurrentSpreadEnergy`) (`CurveFloat.GetFloatValue` (`self.GetEnergyDecrementCurve`) (`self.CurrentSpreadEnergy`))) 0.0 100.0))
        ;;;[1 1 1] Save spread energy level after shot because berween shot work recevery spread energy logic
        (set `self.SpreadEnergyAfterShot` (`self.CurrentSpreadEnergy`))
        ;;;[1 1 1] Update Angle based on spread energy after reduse
        (`self.ClientUpdateSpreadAngleAfterShot`)
        ;;;[1 1 1] If Current Spread Energy < 100 (max value) , start Spread Energy Recovery
        (if (not (== (`self.CurrentSpreadEnergy`) (`self.MaxSpreadEnergy`)))
          (`/Engine/EditorBlueprintResources/StandardMacros.DoOnce` false :!label _label_2
            (:`Completed`
              (`self.ClientStartSpreadEnergyRecovery`))))))))

(event `ClientResetStartSpreadEnergyRecoveryGate`
  ;[1 1 1] 4. RECALCULATION SPREAD ENERGY
  ;;[1 1 1] Requce Spread Enegry After Shot
  ;;;[1 1 1] If Current Spread Energy < 100 (max value) , start Spread Energy Recovery
  (goto _label_2 :!via `Reset`))

(event `ClientStartSpreadEnergyRecovery`
  ;[1 1 1] 4. RECALCULATION SPREAD ENERGY
  ;;[1 1 1] Start Recovery Energy Spread
  ;;;[1 1 1] Initialize Reget Step Value. Energy Value per second / Step Regen Count. This value will be add to current spread energy on each step (spread regen time step)
  (set `self.SpreadRegenValueStep` (/ (`self.GetEnergyGeneratedPerSecond`) (`KismetMathLibrary.Conv_IntToDouble` (`self.SpreadRegenStepsCount`))))
  ;;;[1 1 1] Initialize Spread Regen Time Step.  1 sec / Regen Steps Count
  (set `self.SpreadRegenTimeStep` (/ 1.0 (`KismetMathLibrary.Conv_IntToDouble` (`self.SpreadRegenStepsCount`))))
  ;;;[1 1 1] Set Timer for ClientSpreadEnergyRecoveryStep
  (`KismetSystemLibrary.K2_SetTimer` null "ClientSpreadEnergyRecoveryStep" (`self.SpreadRegenTimeStep`) true))

(event `ClientSpreadEnergyRecoveryStep`
  ;[1 1 1] 4. RECALCULATION SPREAD ENERGY
  ;;[1 1 1] Recover Spread energy Step
  ;;;[1 1 1] Check before intialize new value of current spread energy.
  (if (>= (+ (`self.CurrentSpreadEnergy`) (`self.SpreadRegenValueStep`)) (`self.MaxSpreadEnergy`))
    ;;;[1 1 1] Current = Max = 100
    (set `self.CurrentSpreadEnergy` (`self.MaxSpreadEnergy`))
    ;;;[1 1 1] Update Current Spread angel on each reduce step
    (`self.ClientUpdateSpreadAngleAfterShot`)
    ;;;[1 1 1] Stop Regen Spread Enegry of Current = Max = 100
    (`KismetSystemLibrary.K2_ClearTimer` null "ClientSpreadEnergyRecoveryStep")
    (`self.ClientResetStartSpreadEnergyRecoveryGate`)
    (else
      ;;;[1 1 1] Add Step value to Current Spread Energy Value
      (set `self.CurrentSpreadEnergy` (+ (`self.CurrentSpreadEnergy`) (`self.SpreadRegenValueStep`)))
      ;;;[1 1 1] Update Current Spread angel on each reduce step
      (`self.ClientUpdateSpreadAngleAfterShot`))))

(fn `GetCurrentSpreadAngle`
  (returns (CurrentSpreadAngle :type "Float (double-precision)"))
  (return (`self.CurrentSpreadAngle`)))

(fn `GetCurrentSpreadEnergy`
  (returns (CurrentSpreadEnergy :type "Float (double-precision)"))
  (return (`self.CurrentSpreadEnergy`)))

(fn `GetEndPoint`
  (returns (EndPoint :type "Vector Structure"))
  (return (`self.TraceEndPoint`)))

(fn `GetEnergyDecrementCurve`
  (returns (`Energy Decrement Curve` :type "CurveFloat Object Reference"))
  (return (`.EnergyDecrementCurve_152_6109658A413516DE0E58809B14CFA540` (break `/Game/CHARACTER_SYSTEM_V2/Blueprints/DATA/STR/STR_FL_FirearmLibrarySpreadDesc` (`.Spread_36_97BCE5434EF20DF2D11FA689CD55AA5C` (break `/Game/CHARACTER_SYSTEM_V2/Blueprints/DATA/STR/STR_FL_FirearmLibraryDesc` (`/Game/CHARACTER_SYSTEM_V2/Blueprints/FirearmSystem/AC_FirearmSystem.GetFirearmLibraryDesc` (`self.GetFirearmSystem`))))))))

(fn `GetEnergyGeneratedPerSecond`
  (returns (`Energy Generated Per Second` :type "Float (double-precision)"))
  (return (`.EnergyGeneratedPerSecond_162_D5271980427476D8FB11A79169B485C0` (break `/Game/CHARACTER_SYSTEM_V2/Blueprints/DATA/STR/STR_FL_FirearmLibrarySpreadDesc` (`.Spread_36_97BCE5434EF20DF2D11FA689CD55AA5C` (break `/Game/CHARACTER_SYSTEM_V2/Blueprints/DATA/STR/STR_FL_FirearmLibraryDesc` (`/Game/CHARACTER_SYSTEM_V2/Blueprints/FirearmSystem/AC_FirearmSystem.GetFirearmLibraryDesc` (`self.GetFirearmSystem`))))))))

(fn `GetFirearmOwnerStateHandler`
  (returns (FirearmOwnerStateHandler :type "/Game/CHARACTER_SYSTEM_V2/Blueprints/FirearmSystem/AC_FirearmOwnerStateHandler Object Reference"))
  (bind _returnvalue (`Actor.GetComponentByClass` (`self.GetOwner` self) "/Game/CHARACTER_SYSTEM_V2/Blueprints/FirearmSystem/AC_FirearmOwnerStateHandler.AC_FirearmOwnerStateHandler_C"))
  (`/Engine/EditorBlueprintResources/StandardMacros.IsValid` _returnvalue
    (:`Is Valid`
      (return _returnvalue))))

(fn `GetFirearmSystem`
  (returns (FirearmSystem :type "/Game/CHARACTER_SYSTEM_V2/Blueprints/FirearmSystem/AC_FirearmSystem Object Reference"))
  (bind _returnvalue (`Actor.GetComponentByClass` (`self.GetOwner` self) "/Game/CHARACTER_SYSTEM_V2/Blueprints/FirearmSystem/AC_FirearmSystem.AC_FirearmSystem_C"))
  (`/Engine/EditorBlueprintResources/StandardMacros.IsValid` _returnvalue
    (:`Is Valid`
      (return _returnvalue))))

(fn `GetMainPlayerCamera`
  (returns (MainPlayerCamera :type "CameraComponent Object Reference"))
  (bind _output (`|GetArrayItem` (`Actor.GetComponentsByTag` (`self.GetOwner`) "/Script/Engine.CameraComponent" (`self.MainPlayerCameraTag`))))
  (`/Engine/EditorBlueprintResources/StandardMacros.IsValid` _output
    (:`Is Valid`
      (return _output))))

(fn `GetMaxRandomSpreadAngle`
  (returns (`Max Random Spread Angle` :type "Float (double-precision)"))
  (return (`.MaxRandomSpreadAngle_160_E04D91D247939037F6404B85178F653A` (break `/Game/CHARACTER_SYSTEM_V2/Blueprints/DATA/STR/STR_FL_FirearmLibrarySpreadDesc` (`.Spread_36_97BCE5434EF20DF2D11FA689CD55AA5C` (break `/Game/CHARACTER_SYSTEM_V2/Blueprints/DATA/STR/STR_FL_FirearmLibraryDesc` (`/Game/CHARACTER_SYSTEM_V2/Blueprints/FirearmSystem/AC_FirearmSystem.GetFirearmLibraryDesc` (`self.GetFirearmSystem`))))))))

(fn `GetMinRandomSpreadAngle`
  (returns (`Min Random Spread Angle` :type "Float (double-precision)"))
  (return (`.MinRandomSpreadAngle_159_8CEBA06C48C30A68BE5D9BBE1E7BE9BA` (break `/Game/CHARACTER_SYSTEM_V2/Blueprints/DATA/STR/STR_FL_FirearmLibrarySpreadDesc` (`.Spread_36_97BCE5434EF20DF2D11FA689CD55AA5C` (break `/Game/CHARACTER_SYSTEM_V2/Blueprints/DATA/STR/STR_FL_FirearmLibraryDesc` (`/Game/CHARACTER_SYSTEM_V2/Blueprints/FirearmSystem/AC_FirearmSystem.GetFirearmLibraryDesc` (`self.GetFirearmSystem`))))))))

(fn `GetMultiTraceAmount`
  (returns (`Multi Trace Amount` :type Integer))
  (return (`.MultiTraceAmount_24_0BD7BF06485D44A62BB3D59AFC24A936` (break `/Game/CHARACTER_SYSTEM_V2/Blueprints/DATA/STR/STR_FL_FirearmLibraryShootDesc` (`.Shoot_18_65E9D0144E92C7449C62968586480AD6` (break `/Game/CHARACTER_SYSTEM_V2/Blueprints/DATA/STR/STR_FL_FirearmLibraryDesc` (`/Game/CHARACTER_SYSTEM_V2/Blueprints/FirearmSystem/AC_FirearmSystem.GetFirearmLibraryDesc` (`self.GetFirearmSystem`))))))))

(fn `GetMultiTracePointsArray`
  (returns (PointsDesc :type "Array of /Game/CHARACTER_SYSTEM_V2/Blueprints/DATA/STR/STR_FirearmMultiTraceDesc Structure"))
  (return (`self.MultiTraceArray`)))

(fn `GetSpreadScaleInFPMode`
  (returns (`Spread Scale In FP Mode` :type "Float (double-precision)"))
  (return (`.SpreadScaleInFPMode_165_88B0357146933011EFAFF9BDF6D2B145` (break `/Game/CHARACTER_SYSTEM_V2/Blueprints/DATA/STR/STR_FL_FirearmLibrarySpreadDesc` (`.Spread_36_97BCE5434EF20DF2D11FA689CD55AA5C` (break `/Game/CHARACTER_SYSTEM_V2/Blueprints/DATA/STR/STR_FL_FirearmLibraryDesc` (`/Game/CHARACTER_SYSTEM_V2/Blueprints/FirearmSystem/AC_FirearmSystem.GetFirearmLibraryDesc` (`self.GetFirearmSystem`))))))))

(fn `GetStartPoint`
  (returns (StartPoint :type "Vector Structure"))
  (return (`self.TraceStartPoint`)))

(fn `GetTraceType`
  (returns (`Trace Type` :type "/Game/CHARACTER_SYSTEM_V2/Blueprints/DATA/E/E_FirearmTraceType Enum"))
  (return (`.TraceType_20_B15526C84A6C7A0A83FE548A654DB272` (break `/Game/CHARACTER_SYSTEM_V2/Blueprints/DATA/STR/STR_FL_FirearmLibraryShootDesc` (`.Shoot_18_65E9D0144E92C7449C62968586480AD6` (break `/Game/CHARACTER_SYSTEM_V2/Blueprints/DATA/STR/STR_FL_FirearmLibraryDesc` (`/Game/CHARACTER_SYSTEM_V2/Blueprints/FirearmSystem/AC_FirearmSystem.GetFirearmLibraryDesc` (`self.GetFirearmSystem`))))))))