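; Firearm component that plays client-side camera shakes on the player camera each time the weapon fires.
; Each shot stops and restarts separate low- and high-frequency shakes, with classes, powers and stop modes read from the firearm system's library description.
; Shake scale combines that power with an owner-state coefficient, refreshed on init and influence updates, plus an extra multiplier in first-person mode.
; The firearm system drives all its events.
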(event `ClientHandleUpdateOnFirearmInitialize`
  ;[1 1 1] UPDATE ON INIT FIREARM
  ;;[1 0.1179 0] INPUT FROM FIREARM SYSTEM
  (set `self.CharacterInfluenceCoeff` (`/Game/CHARACTER_SYSTEM_V2/Blueprints/FirearmSystem/AC_FirearmOwnerStateHandler.GetCurrentCameraShakeCoeff` (`self.GetFirearmOwnerStateHandler`))))

(event `ClientHandleInteratedCharacterInfluence`
  ;[1 1 1] UPDATE OWNER INFLUENCE ON SPREAD
  ;;[1 0.1179 0] INPUT FROM FIREARM SYSTEM
  (set `self.CharacterInfluenceCoeff` (`/Game/CHARACTER_SYSTEM_V2/Blueprints/FirearmSystem/AC_FirearmOwnerStateHandler.GetCurrentCameraShakeCoeff` (`self.GetFirearmOwnerStateHandler`))))

(event `ClientToggleFPMode`
  (params (ToggleOn :type Boolean))
  ;[1 1 1] TOGGLE FP MODE
  ;;[1 0.1179 0] INPUT FROM FIREARM SYSTEM
  (if ToggleOn
    (set `self.Use In FPS Character?` true)
    (else
      (set `self.Use In FPS Character?` false))))

(event `ClientHandlePlayerShakeOnShot`
  ;[1 1 1] PLAY LOW & HIQH FREQ CHAKES
  ;;[1 0.1179 0] INPUT FROM FIREARM SYSTEM
  ;;[1 1 1] Check use cam shakes
  (if (`self.Use Camera Shake?`)
    (`|ExecutionSequence`
      (:`then_0`
        ;;[1 1 1] LOW F CAM SHAKE
        ;;;[1 1 1] Stop Low F Shake on New shot
        (`PlayerCameraManager.StopCameraShake` (`GameplayStatics.GetPlayerCameraManager` 0) (`self.CurrentCamShakeLowF`) (`self.GetCamShakeLowFrequencyStopImmediately`))
        ;;;[1 1 1] Start Low F cam shaek on each shot
        (bind _returnvalue (`PlayerCameraManager.StartCameraShake` :`self` (`GameplayStatics.GetPlayerCameraManager` 0) :`ShakeClass` (`self.GetCamShakeLowFrequency`) :`Scale` (* (select `bool` (`self.Use In FPS Character?`) :`false` 1.0 :`true` (`self.GetCamShakeScaleInFPMode`)) (`self.CharacterInfluenceCoeff`) (`self.GetCamShakeLowFrequencyPower`))))
        (set `self.CurrentCamShakeLowF` _returnvalue))
      (:`then_1`
        ;;[1 1 1] HIGH F CAM SHAKE
        ;;;[1 1 1] Stop high F Shake on New shot
        (`PlayerCameraManager.StopCameraShake` (`GameplayStatics.GetPlayerCameraManager` 0) (`self.CurrentCamShakeHighF`) (`self.GetCamShakeHighFrequencyStopImmediately`))
        ;;;[1 1 1] Start high F cam shaek on each shot
        (bind _returnvalue_2 (`PlayerCameraManager.StartCameraShake` :`self` (`GameplayStatics.GetPlayerCameraManager` 0) :`ShakeClass` (`self.GetCamShakeHighFrequency`) :`Scale` (* (select `bool` (`self.Use In FPS Character?`) :`false` 1.0 :`true` (`self.GetCamShakeScaleInFPMode`)) (`self.CharacterInfluenceCoeff`) (`self.GetCamShakeHighFrequencyPower`))))
        (set `self.CurrentCamShakeHighF` _returnvalue_2)))))

(fn `GetCamShakeHighFrequency`
  (returns (`Cam Shake High Frequency` :type "CameraShakeBase Class Reference"))
  (return (`.CamShakeHighFrequency_4_49548EC41B47A9F0F05690A615C14FA7` (break `/Game/CHARACTER_SYSTEM_V2/Blueprints/DATA/STR/STR_FL_FirearmLibraryCamShakesDesc` (`.CameraShake_65_17AD6C6D40CE28DD67A6E5B7FC03C38F` (break `/Game/CHARACTER_SYSTEM_V2/Blueprints/DATA/STR/STR_FL_FirearmLibraryDesc` (`/Game/CHARACTER_SYSTEM_V2/Blueprints/FirearmSystem/AC_FirearmSystem.GetFirearmLibraryDesc` (`self.GetFirearmSystem`))))))))

(fn `GetCamShakeHighFrequencyPower`
  (returns (`Cam Shake High Frequency Power` :type "Float (double-precision)"))
  (return (`.CamShakeHighFrequencyPower_10_09F7CD77134B171751D0FF9848666E8A` (break `/Game/CHARACTER_SYSTEM_V2/Blueprints/DATA/STR/STR_FL_FirearmLibraryCamShakesDesc` (`.CameraShake_65_17AD6C6D40CE28DD67A6E5B7FC03C38F` (break `/Game/CHARACTER_SYSTEM_V2/Blueprints/DATA/STR/STR_FL_FirearmLibraryDesc` (`/Game/CHARACTER_SYSTEM_V2/Blueprints/FirearmSystem/AC_FirearmSystem.GetFirearmLibraryDesc` (`self.GetFirearmSystem`))))))))

(fn `GetCamShakeHighFrequencyStopImmediately`
  (returns (`Cam Shake High Frequency Stop Immediately` :type Boolean))
  (return (`.CamShakeHighFrequencyStopImmediately_18_1E0CD5455C4E14CC7491BDBF01EF1A68` (break `/Game/CHARACTER_SYSTEM_V2/Blueprints/DATA/STR/STR_FL_FirearmLibraryCamShakesDesc` (`.CameraShake_65_17AD6C6D40CE28DD67A6E5B7FC03C38F` (break `/Game/CHARACTER_SYSTEM_V2/Blueprints/DATA/STR/STR_FL_FirearmLibraryDesc` (`/Game/CHARACTER_SYSTEM_V2/Blueprints/FirearmSystem/AC_FirearmSystem.GetFirearmLibraryDesc` (`self.GetFirearmSystem`))))))))

(fn `GetCamShakeLowFrequency`
  (returns (`Cam Shake Low Frequency` :type "CameraShakeBase Class Reference"))
  (return (`.CamShakeLowFrequency_2_3DCA207D954FC9294616A08061A02799` (break `/Game/CHARACTER_SYSTEM_V2/Blueprints/DATA/STR/STR_FL_FirearmLibraryCamShakesDesc` (`.CameraShake_65_17AD6C6D40CE28DD67A6E5B7FC03C38F` (break `/Game/CHARACTER_SYSTEM_V2/Blueprints/DATA/STR/STR_FL_FirearmLibraryDesc` (`/Game/CHARACTER_SYSTEM_V2/Blueprints/FirearmSystem/AC_FirearmSystem.GetFirearmLibraryDesc` (`self.GetFirearmSystem`))))))))

(fn `GetCamShakeLowFrequencyPower`
  (returns (`Cam Shake Low Frequency Power` :type "Float (double-precision)"))
  (return (`.CamShakeLowFrequencyPower_9_D0791CB92641E92DE6E7E7B76A828644` (break `/Game/CHARACTER_SYSTEM_V2/Blueprints/DATA/STR/STR_FL_FirearmLibraryCamShakesDesc` (`.CameraShake_65_17AD6C6D40CE28DD67A6E5B7FC03C38F` (break `/Game/CHARACTER_SYSTEM_V2/Blueprints/DATA/STR/STR_FL_FirearmLibraryDesc` (`/Game/CHARACTER_SYSTEM_V2/Blueprints/FirearmSystem/AC_FirearmSystem.GetFirearmLibraryDesc` (`self.GetFirearmSystem`))))))))

(fn `GetCamShakeLowFrequencyStopImmediately`
  (returns (`Cam Shake Low Frequency Stop Immediately` :type Boolean))
  (return (`.CamShakeLowFrequencyStopImmediately_17_EDC5B3115A4D0E980F6E19A7193BF6B1` (break `/Game/CHARACTER_SYSTEM_V2/Blueprints/DATA/STR/STR_FL_FirearmLibraryCamShakesDesc` (`.CameraShake_65_17AD6C6D40CE28DD67A6E5B7FC03C38F` (break `/Game/CHARACTER_SYSTEM_V2/Blueprints/DATA/STR/STR_FL_FirearmLibraryDesc` (`/Game/CHARACTER_SYSTEM_V2/Blueprints/FirearmSystem/AC_FirearmSystem.GetFirearmLibraryDesc` (`self.GetFirearmSystem`))))))))

(fn `GetCamShakeScaleInFPMode`
  (returns (`Cam Shake Scale In FP Mode` :type "Float (double-precision)"))
  (return (`.CamShakeScaleInFPMode_24_F109079240C074D1DDDB0593D199A78A` (break `/Game/CHARACTER_SYSTEM_V2/Blueprints/DATA/STR/STR_FL_FirearmLibraryCamShakesDesc` (`.CameraShake_65_17AD6C6D40CE28DD67A6E5B7FC03C38F` (break `/Game/CHARACTER_SYSTEM_V2/Blueprints/DATA/STR/STR_FL_FirearmLibraryDesc` (`/Game/CHARACTER_SYSTEM_V2/Blueprints/FirearmSystem/AC_FirearmSystem.GetFirearmLibraryDesc` (`self.GetFirearmSystem`))))))))

(fn `GetFirearmOwnerStateHandler`
  (returns (FirearmOwnerStateHandler :type "/Game/CHARACTER_SYSTEM_V2/Blueprints/FirearmSystem/AC_FirearmOwnerStateHandler Object Reference"))
  (bind _returnvalue (`Actor.GetComponentByClass` (`self.GetOwner` self) "/Game/CHARACTER_SYSTEM_V2/Blueprints/FirearmSystem/AC_FirearmOwnerStateHandler.AC_FirearmOwnerStateHandler_C"))
  (`/Engine/EditorBlueprintResources/StandardMacros.IsValid` _returnvalue
    (:`Is Valid`
      (return _returnvalue))))

(fn `GetFirearmSystem`
  (returns (FirearmSystem :type "/Game/CHARACTER_SYSTEM_V2/Blueprints/FirearmSystem/AC_FirearmSystem Object Reference"))
  (bind _returnvalue (`Actor.GetComponentByClass` (`self.GetOwner` self) "/Game/CHARACTER_SYSTEM_V2/Blueprints/FirearmSystem/AC_FirearmSystem.AC_FirearmSystem_C"))
  (`/Engine/EditorBlueprintResources/StandardMacros.IsValid` _returnvalue
    (:`Is Valid`
      (return _returnvalue))))