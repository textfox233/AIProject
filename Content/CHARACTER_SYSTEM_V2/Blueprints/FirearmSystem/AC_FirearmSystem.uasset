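; Character component that acts as the central mediator of the modular firearm system.
; On authority it adds the shooting, spread, recoil, hit scan, damage and feedback sub-components, then initializes them for a firearm validated against DT_FirearmLibrary.
; It relays character input and stance to those components and returns firearm, reload and scope events to the character.
; Shots flow through spread into hit scan, whose traces feed character, sound and damage handling.
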(event `self.ReceiveBeginPlay`
  ;[1 1 1] EVENT BEGIN PLAY
  (`/Engine/EditorBlueprintResources/ActorComponentMacros.Switch Has Authority`
    (:`Authority`
      ;;[1 1 1] Create FirearmShootingController
      (`|AddComponentByClass` (`self.GetOwner` self) "/Game/CHARACTER_SYSTEM_V2/Blueprints/FirearmSystem/AC_FirearmShootingController.AC_FirearmShootingController_C")
      ;;[1 1 1] Create FirearmSpreadController
      (`|AddComponentByClass` (`self.GetOwner` self) "/Game/CHARACTER_SYSTEM_V2/Blueprints/FirearmSystem/AC_FirearmSpreadController.AC_FirearmSpreadController_C")
      ;;[1 1 1] Create FirearmOwnerStateHandler
      (`|AddComponentByClass` (`self.GetOwner` self) "/Game/CHARACTER_SYSTEM_V2/Blueprints/FirearmSystem/AC_FirearmOwnerStateHandler.AC_FirearmOwnerStateHandler_C")
      ;;[1 1 1] Create FirearmHitScan
      (`|AddComponentByClass` (`self.GetOwner` self) "/Game/CHARACTER_SYSTEM_V2/Blueprints/FirearmSystem/AC_FirearmHitScan.AC_FirearmHitScan_C")
      ;;[1 1 1] Create FirearmVFXController
      (`|AddComponentByClass` (`self.GetOwner` self) "/Game/CHARACTER_SYSTEM_V2/Blueprints/FirearmSystem/AC_FirearmVFXController.AC_FirearmVFXController_C")
      ;;[1 1 1] Create FirearmSoundController
      (`|AddComponentByClass` (`self.GetOwner` self) "/Game/CHARACTER_SYSTEM_V2/Blueprints/FirearmSystem/AC_FirearmSoundController.AC_FirearmSoundController_C")
      ;;[1 1 1] Create FirearmRecoilController
      (`|AddComponentByClass` (`self.GetOwner` self) "/Game/CHARACTER_SYSTEM_V2/Blueprints/FirearmSystem/AC_FirearmRecoilController.AC_FirearmRecoilController_C")
      ;;[1 1 1] Create CameraShakeController
      (`|AddComponentByClass` (`self.GetOwner` self) "/Game/CHARACTER_SYSTEM_V2/Blueprints/FirearmSystem/AC_FirearmCameraShakeController.AC_FirearmCameraShakeController_C")
      ;;[1 1 1] Create FirearmScopeController
      (`|AddComponentByClass` (`self.GetOwner` self) "/Game/CHARACTER_SYSTEM_V2/Blueprints/FirearmSystem/AC_FirearmScopeController.AC_FirearmScopeController_C")
      ;;[1 1 1] Create FirearmDamageHandler
      (`|AddComponentByClass` (`self.GetOwner` self) "/Game/CHARACTER_SYSTEM_V2/Blueprints/FirearmSystem/AC_FirearmDamageHandler.AC_FirearmDamageHandler_C"))))

(event `ServerInitializeFirearmItem`
  (params (FirearmActor :type "Actor Object Reference"))
  ;[1 1 1] INITIALIZE FIREARM
  ;;[1 0.1179 0] INPUT FROM CHARACTER
  ;;[1 1 1] Initialize & Check Valid Actor
  (bind _asbp_firearm_actor_common (cast `/Game/CHARACTER_SYSTEM_V2/Blueprints/FirearmSystem/BP_FirearmActorCommon` FirearmActor)
    (:`then`
      (bind _output_get (set `self.FirearmItemCommon` _asbp_firearm_actor_common))
      (set `self.FirearmTag` (`/Game/CHARACTER_SYSTEM_V2/Blueprints/FirearmSystem/BP_FirearmActorCommon.FirearmTag` _output_get))
      (bind _returnvalue (`DataTableFunctionLibrary.DoesDataTableRowExist` "/Game/CHARACTER_SYSTEM_V2/Blueprints/FirearmTP/DT_FirearmLibrary.DT_FirearmLibrary" (`self.FirearmTag`)))
      (if _returnvalue
        (`KismetSystemLibrary.Delay` 0.1)
        ;;[1 1 1] Initialize Firearm System Components
        (`/Game/CHARACTER_SYSTEM_V2/Blueprints/FirearmSystem/AC_FirearmOwnerStateHandler.ClientHandleInitFirearm` (`self.GetFirearmOwnerStateHandler`))
        (`/Game/CHARACTER_SYSTEM_V2/Blueprints/FirearmSystem/AC_FirearmSpreadController.ClientHandleUpdateMinSpreadOnInitFirearm` (`self.GetFirearmSpreadController`))
        (`/Game/CHARACTER_SYSTEM_V2/Blueprints/FirearmSystem/AC_FirearmRecoilController.ClientHandleFirearmInit` (`self.GetFirearmRecoilController`))
        (`/Game/CHARACTER_SYSTEM_V2/Blueprints/FirearmSystem/AC_FirearmCameraShakeController.ClientHandleUpdateOnFirearmInitialize` (`self.GetFirearmCameraShakeController`))
        (`/Game/CHARACTER_SYSTEM_V2/Blueprints/FirearmSystem/AC_FirearmScopeController.ClientHandleInitFirearm` (`self.GetFirearmScopeController`))
        ;;[1 1 1] Check condition for main reload / extra reload on init firearm
        (if (`/Game/CHARACTER_SYSTEM_V2/Blueprints/FirearmSystem/BP_FirearmActorCommon.GetInExtraReload` (`self.FirearmItemCommon`))
          (`/Game/CHARACTER_SYSTEM_V2/Blueprints/FirearmSystem/AC_FirearmShootingController.ClientRequestedExtraReload` (`self.GetFirearmShootingController`))
          (elif (== (`/Game/CHARACTER_SYSTEM_V2/Blueprints/FirearmSystem/BP_FirearmActorCommon.GetCurrentAmmoInClip` (`self.FirearmItemCommon`)) 0)
            (`/Game/CHARACTER_SYSTEM_V2/Blueprints/FirearmSystem/AC_FirearmShootingController.ClientRequestedMainReload` (`self.GetFirearmShootingController`))))
        (else
          (`self.DebugMessage` "Firearm Item Tag is not found in Firearm Library"))))
    (:`CastFailed`
      (`self.DebugMessage` "Actor on init is not child of FirearmItemCommon"))))

(event `ClientSingleTraceCreated`
  (params (SingleTraceDesc :type "/Game/CHARACTER_SYSTEM_V2/Blueprints/DATA/STR/STR_FirearmHitScanDesc Structure"))
  ;[1 1 1] INPUT FROM HIT SCAN
  ;;[1 0.1179 0] INPUT FROM FIREARM HIT SCAN
  ;;[1 0.6824 0] TO CHARACTER COMMON
  (`/Game/CHARACTER_SYSTEM_V2/Blueprints/CharacterCommon/BP_CharacterCommon.ClientHandleSingleTraceCreated` (`self.GetCharacterCommon`) SingleTraceDesc)
  ;;[1 0.6824 0] TO FIREARM SOUND CONTROLLER
  (`/Game/CHARACTER_SYSTEM_V2/Blueprints/FirearmSystem/AC_FirearmSoundController.ClientHandlePlayerSoundOnSingleHit` (`self.GetFirearmSoundController`) SingleTraceDesc)
  ;;[1 0.6824 0] TO FIREARM DAMAGE HANDLER
  (`/Game/CHARACTER_SYSTEM_V2/Blueprints/FirearmSystem/AC_FirearmDamageHandler.ServerHandleSingleHit` (`self.GetFirearmDamageHandler`) SingleTraceDesc))

(event `ClientShotHappened`
  ;[1 1 1] INPUTS FROM SHOOTING CONTROLLER
  ;;[1 1 1] Main
  ;;;[1 0.1179 0] INPUT FROM SHOOTING CONTROLLER
  ;;;[1 0.6824 0] TO FIREARM ACTOR
  (`/Game/CHARACTER_SYSTEM_V2/Blueprints/FirearmSystem/BP_FirearmActorCommon.ClientUpdateAmmoInClipOnShot` (`self.FirearmItemCommon`))
  (`/Game/CHARACTER_SYSTEM_V2/Blueprints/FirearmSystem/AC_FirearmSpreadController.ClientHandleUpdateSpreadOnShot` (`self.GetFirearmSpreadController`))
  (`/Game/CHARACTER_SYSTEM_V2/Blueprints/FirearmSystem/AC_FirearmRecoilController.ClientHandleShot` (`self.GetFirearmRecoilController`))
  (`/Game/CHARACTER_SYSTEM_V2/Blueprints/FirearmSystem/AC_FirearmSoundController.ClientHandlePlayerSoundOnShot` (`self.GetFirearmSoundController`))
  (`/Game/CHARACTER_SYSTEM_V2/Blueprints/FirearmSystem/AC_FirearmCameraShakeController.ClientHandlePlayerShakeOnShot` (`self.GetFirearmCameraShakeController`))
  (`self.ClientFirearmEvent` "NewEnumerator0"))

(event `ClientHandleReadyToSingleShot`
  (params (TraceStartPoint :type "Vector Structure") (TraceEndPoint :type "Vector Structure"))
  ;[1 1 1] INPUTS FROM SPREAD CONTROLLLER
  ;;[1 0.1179 0] INPUT FROM FIREARM SPREAD CONTROLLER
  ;;[1 0.6824 0] TO FIREARM HITSCAN
  (`/Game/CHARACTER_SYSTEM_V2/Blueprints/FirearmSystem/AC_FirearmHitScan.ClientHandleCreateSingleLineTrace` (`self.GetFirearmHitScan`) TraceStartPoint TraceEndPoint))

(event `ClientInputPressedShooting`
  ;[1 1 1] INPUTS FROM CHARACTER
  ;;[1 0.1179 0] INPUT FROM CHARACTER
  ;;[1 0.6824 0] TO FIREARM SHOOTING CONTROLLER
  (`/Game/CHARACTER_SYSTEM_V2/Blueprints/FirearmSystem/AC_FirearmShootingController.ClientShootPressed` (`self.GetFirearmShootingController`)))

(event `ClientShotDelayEnded`
  ;[1 1 1] INPUTS FROM SHOOTING CONTROLLER
  ;;[1 1 1] Main
  ;;;[1 0.1179 0] INPUT FROM SHOOTING CONTROLLER
  (`self.ClientFirearmEvent` "NewEnumerator1")
  (`/Game/CHARACTER_SYSTEM_V2/Blueprints/FirearmSystem/AC_FirearmRecoilController.ClientHandleShotDelayEnd` (`self.GetFirearmRecoilController`)))

(event `ClientInputReleasedShooting`
  ;[1 1 1] INPUTS FROM CHARACTER
  ;;[1 0.1179 0] INPUT FROM CHARACTER
  (`/Game/CHARACTER_SYSTEM_V2/Blueprints/FirearmSystem/AC_FirearmShootingController.ClientShootReleased` (`self.GetFirearmShootingController`))
  (`self.ClientFirearmEvent` "NewEnumerator12")
  (`/Game/CHARACTER_SYSTEM_V2/Blueprints/FirearmSystem/AC_FirearmRecoilController.ClientHandleShootingInputRealized` (`self.GetFirearmRecoilController`)))

(event `ClientMultiTraceCreated`
  (params (MultiTraceDesc :type "Array of /Game/CHARACTER_SYSTEM_V2/Blueprints/DATA/STR/STR_FirearmHitScanDesc Structure"))
  ;[1 1 1] INPUT FROM HIT SCAN
  ;;[1 0.1179 0] INPUT FROM FIREARM HIT SCAN
  ;;[1 0.6824 0] TO CHARACTER COMMON
  (`/Game/CHARACTER_SYSTEM_V2/Blueprints/CharacterCommon/BP_CharacterCommon.ClientHandleMultiTraceCreated` (`self.GetCharacterCommon`) MultiTraceDesc)
  ;;[1 0.6824 0] TO FIREARM SOUND CONTROLLER
  (`/Game/CHARACTER_SYSTEM_V2/Blueprints/FirearmSystem/AC_FirearmSoundController.ClientHandlePlayerSoundOnMultiHit` (`self.GetFirearmSoundController`) MultiTraceDesc)
  ;;[1 0.6824 0] TO FIREARM DAMAGE HANDLER
  (`/Game/CHARACTER_SYSTEM_V2/Blueprints/FirearmSystem/AC_FirearmDamageHandler.ServerHandleMultiHit` (`self.GetFirearmDamageHandler`) MultiTraceDesc))

(event `ClientHandleReadyToMultiShot`
  (params (MultiTraces :type "Array of /Game/CHARACTER_SYSTEM_V2/Blueprints/DATA/STR/STR_FirearmMultiTraceDesc Structure"))
  ;[1 1 1] INPUTS FROM SPREAD CONTROLLLER
  ;;[1 0.1179 0] INPUT FROM FIREAM SPREAD CONTROLLER
  ;;[1 0.6824 0] TO FIREARM HITSCAN
  (`/Game/CHARACTER_SYSTEM_V2/Blueprints/FirearmSystem/AC_FirearmHitScan.ClientHandleCreateMultiLineTrace` (`self.GetFirearmHitScan`) MultiTraces))

(event `ClientFirearmsAmmoEmpty`
  ;[1 1 1] INPUTS FROM SHOOTING CONTROLLER
  ;;[1 1 1] Main
  ;;;[1 0.1179 0] INPUT FROM SHOOTING CONTROLLER
  (`self.ClientFirearmEvent` "NewEnumerator11"))

(event `ClientInputReloadTrigger`
  ;[1 1 1] INPUTS FROM CHARACTER
  ;;[1 0.1179 0] INPUT FROM CHARACTER
  (`/Game/CHARACTER_SYSTEM_V2/Blueprints/FirearmSystem/AC_FirearmShootingController.ClientRequestedMainReload` (`self.GetFirearmShootingController`)))

(event `ClientMainReloadStart`
  ;[1 1 1] INPUTS FROM SHOOTING CONTROLLER
  ;;[1 1 1] Main Reload
  ;;;[1 0.1179 0] INPUT FROM SHOOTING CONTROLLER
  (`self.ClientFirearmEvent` "NewEnumerator2")
  ;;;[1 0.6824 0] TO CHARACTER COMMON
  (`/Game/CHARACTER_SYSTEM_V2/Blueprints/CharacterCommon/BP_CharacterCommon.ClientMainReloadOn` (`self.GetCharacterCommon`))
  (`/Game/CHARACTER_SYSTEM_V2/Blueprints/FirearmSystem/AC_FirearmRecoilController.ClientHandleStopRecoilAction` (`self.GetFirearmRecoilController`)))

(event `ServerMainReloadStart`
  ;[1 1 1] INPUTS FROM SHOOTING CONTROLLER
  ;;[1 1 1] Main Reload
)

(event `ClientFirearmEvent`
  (params (FirearmEventType :type "/Game/CHARACTER_SYSTEM_V2/Blueprints/DATA/E/E_GL_FirearmEventType Enum" :default "NewEnumerator0"))
  ;[1 1 1] OUTPUTS TO CHARACTER
  ;;[1 0.6824 0] TO CHARACTER COMMON
  (`/Game/CHARACTER_SYSTEM_V2/Blueprints/CharacterCommon/BP_CharacterCommon.ClientHandleFirearmEvent` (`self.GetCharacterCommon`) FirearmEventType))

(event `HandleSwitchFirearmsDown`
  (params (HalfSwitchTime :type "Float (double-precision)"))
  ;[1 1 1] SWITCH FIREARMS
  ;;[1 0.1179 0] BI INPUT FROM CHARACTER
  (`/Game/CHARACTER_SYSTEM_V2/Blueprints/FirearmSystem/AC_FirearmSoundController.ClientPlaySwitchDownSound` (`self.GetFirearmSoundController`)))

(event `ClientMainReloadFinish`
  ;[1 1 1] INPUTS FROM SHOOTING CONTROLLER
  ;;[1 1 1] Main Reload
  ;;;[1 0.1179 0] INPUT FROM SHOOTING CONTROLLER
  ;;;[1 0.6824 0] TO FIREARM ACTOR
  (`/Game/CHARACTER_SYSTEM_V2/Blueprints/FirearmSystem/BP_FirearmActorCommon.ClientUpdateAmmoOnMainReload` (`self.FirearmItemCommon`))
  ;;;[1 0.6824 0] TO CHARACTER COMMON
  (`/Game/CHARACTER_SYSTEM_V2/Blueprints/CharacterCommon/BP_CharacterCommon.ClientMainReloadOff` (`self.GetCharacterCommon`))
  (`self.ClientFirearmEvent` "NewEnumerator3"))

(event `ServerHandleOwnerADSOn`
  ;[1 1 1] INPUT OWNER STATE
  ;;[1 0.1179 0] INPUT FROM CHARACTER
  (`/Game/CHARACTER_SYSTEM_V2/Blueprints/FirearmSystem/AC_FirearmOwnerStateHandler.ServerHandleOwnerADSOn` (`self.GetFirearmOwnerStateHandler`))
  (`/Game/CHARACTER_SYSTEM_V2/Blueprints/FirearmSystem/AC_FirearmSoundController.ClientPlayZoomInSound` (`self.GetFirearmSoundController`)))

(event `HandleSwitchFirearmsUp`
  (params (HalfSwitchTime :type "Float (double-precision)"))
  ;[1 1 1] SWITCH FIREARMS
  ;;[1 0.1179 0] BI INPUT FROM CHARACTER
  (`/Game/CHARACTER_SYSTEM_V2/Blueprints/FirearmSystem/AC_FirearmSoundController.ClientPlaySwitchUpSound` (`self.GetFirearmSoundController`)))

(event `ClientMainReloadCanceled`
  ;[1 1 1] INPUTS FROM SHOOTING CONTROLLER
  ;;[1 1 1] Main Reload
  ;;;[1 0.1179 0] INPUT FROM SHOOTING CONTROLLER
  (`self.ClientFirearmEvent` "NewEnumerator4"))

(event `ServerHandleOwnerADSOff`
  ;[1 1 1] INPUT OWNER STATE
  ;;[1 0.1179 0] INPUT FROM CHARACTER
  (`/Game/CHARACTER_SYSTEM_V2/Blueprints/FirearmSystem/AC_FirearmOwnerStateHandler.ServerHandleOwnerADSOff` (`self.GetFirearmOwnerStateHandler`))
  (`/Game/CHARACTER_SYSTEM_V2/Blueprints/FirearmSystem/AC_FirearmSoundController.ClientPlayZoomOutSound` (`self.GetFirearmSoundController`)))

(event `ServerHandleSwitchFirearmFinish`
  ;[1 1 1] SWITCH FIREARMS
)

(event `ServerChildHandleSwitchFirearmFinish`
  ;[1 1 1] SWITCH FIREARMS
  ;;[0.1778 0 1] PARENT OUTPUT EVENT
)

(event `HandleSwitchFirearmsFinish`
  ;[1 1 1] SWITCH FIREARMS
  ;;[1 0.1179 0] BI INPUT FROM CHARACTER
  (`self.ServerHandleSwitchFirearmFinish`)
  (`self.ServerChildHandleSwitchFirearmFinish`))

(event `ServerHandleOwnerCrouchOff`
  ;[1 1 1] INPUT OWNER STATE
  ;;[1 0.1179 0] INPUT FROM CHARACTER
  (`/Game/CHARACTER_SYSTEM_V2/Blueprints/FirearmSystem/AC_FirearmOwnerStateHandler.ServerHandleOwnerCrouchOff` (`self.GetFirearmOwnerStateHandler`)))

(event `ServerHandleOwnerCrouchOn`
  ;[1 1 1] INPUT OWNER STATE
  ;;[1 0.1179 0] INPUT FROM CHARACTER
  (`/Game/CHARACTER_SYSTEM_V2/Blueprints/FirearmSystem/AC_FirearmOwnerStateHandler.ServerHandleOwnerCrouchOn` (`self.GetFirearmOwnerStateHandler`)))

(event `ClientMainReloadCyclicStartToPos`
  ;[1 1 1] INPUTS FROM SHOOTING CONTROLLER
  ;;[1 1 1] Cyclic Main Reload
  ;;;[1 0.1179 0] INPUT FROM SHOOTING CONTROLLER
  (`self.ClientFirearmEvent` "NewEnumerator5"))

(event `ServerHandleOwnerProneOff`
  ;[1 1 1] INPUT OWNER STATE
  ;;[1 0.1179 0] INPUT FROM CHARACTER
  (`/Game/CHARACTER_SYSTEM_V2/Blueprints/FirearmSystem/AC_FirearmOwnerStateHandler.ServerHandleOwnerProneOff` (`self.GetFirearmOwnerStateHandler`)))

(event `ServerHandleOwnerProneOn`
  ;[1 1 1] INPUT OWNER STATE
  ;;[1 0.1179 0] INPUT FROM CHARACTER
  (`/Game/CHARACTER_SYSTEM_V2/Blueprints/FirearmSystem/AC_FirearmOwnerStateHandler.ServerHandleOwnerProneOn` (`self.GetFirearmOwnerStateHandler`)))

(event `ClientMainReloadCyclicStart`
  ;[1 1 1] INPUTS FROM SHOOTING CONTROLLER
  ;;[1 1 1] Cyclic Main Reload
  ;;;[1 0.1179 0] INPUT FROM SHOOTING CONTROLLER
  (`self.ClientFirearmEvent` "NewEnumerator6"))

(event `ServerHandleOwnerMoveOff`
  ;[1 1 1] INPUT OWNER STATE
  ;;[1 0.1179 0] INPUT FROM CHARACTER
  (`/Game/CHARACTER_SYSTEM_V2/Blueprints/FirearmSystem/AC_FirearmOwnerStateHandler.ServerHadleMovementOff` (`self.GetFirearmOwnerStateHandler`)))

(event `ServerHandleOwnerMoveOn`
  ;[1 1 1] INPUT OWNER STATE
  ;;[1 0.1179 0] INPUT FROM CHARACTER
  (`/Game/CHARACTER_SYSTEM_V2/Blueprints/FirearmSystem/AC_FirearmOwnerStateHandler.ServerHadleMovementOn` (`self.GetFirearmOwnerStateHandler`)))

(event `ClientMainReloadCyclicStop`
  ;[1 1 1] INPUTS FROM SHOOTING CONTROLLER
  ;;[1 1 1] Cyclic Main Reload
  ;;;[1 0.1179 0] INPUT FROM SHOOTING CONTROLLER
  (`self.ClientFirearmEvent` "NewEnumerator7"))

(event `ServerHandleOwnerSprintOn`
  ;[1 1 1] INPUT OWNER STATE
  ;;[1 0.1179 0] INPUT FROM CHARACTER
)

(event `ServerHandleOwnerSprintOff`
  ;[1 1 1] INPUT OWNER STATE
  ;;[1 0.1179 0] INPUT FROM CHARACTER
)

(event `ClientMainReloadCyclicEndToPos`
  ;[1 1 1] INPUTS FROM SHOOTING CONTROLLER
  ;;[1 1 1] Cyclic Main Reload
  ;;;[1 0.1179 0] INPUT FROM SHOOTING CONTROLLER
  (`self.ClientFirearmEvent` "NewEnumerator8"))

(event `ClientToggleFPMode`
  (params (ToggleOn :type Boolean))
  ;[1 1 1] TOGGLE FP MODE
  ;;[1 0.1179 0] BI INPUT FROM CHARACTER
  (`/Game/CHARACTER_SYSTEM_V2/Blueprints/FirearmSystem/AC_FirearmSpreadController.ClientHandleToggleOnFPMode` (`self.GetFirearmSpreadController`) ToggleOn)
  (`/Game/CHARACTER_SYSTEM_V2/Blueprints/FirearmSystem/AC_FirearmOwnerStateHandler.ClientToggleFPModeOnOff` (`self.GetFirearmOwnerStateHandler`) ToggleOn)
  (`/Game/CHARACTER_SYSTEM_V2/Blueprints/FirearmSystem/AC_FirearmRecoilController.ClientHandleToggleFPMode` (`self.GetFirearmRecoilController`) ToggleOn)
  (`/Game/CHARACTER_SYSTEM_V2/Blueprints/FirearmSystem/AC_FirearmCameraShakeController.ClientToggleFPMode` (`self.GetFirearmCameraShakeController`) ToggleOn)
  (`/Game/CHARACTER_SYSTEM_V2/Blueprints/FirearmSystem/AC_FirearmVFXController.ClientHandleToggleFPMode` (`self.GetFirearmVFXController`) ToggleOn))

(event `ClientExtraReloadStart`
  ;[1 1 1] INPUTS FROM SHOOTING CONTROLLER
  ;;[1 1 1] Extra Reload
  ;;;[1 0.1179 0] INPUT FROM SHOOTING CONTROLLER
  (`self.ClientFirearmEvent` "NewEnumerator9")
  (`/Game/CHARACTER_SYSTEM_V2/Blueprints/FirearmSystem/AC_FirearmRecoilController.ClientHandleStopRecoilAction` (`self.GetFirearmRecoilController`))
  (`self.ServerExtraReloadStart`)
  ;;;[1 0.6824 0] TO CHARACTER COMMON
  (`/Game/CHARACTER_SYSTEM_V2/Blueprints/CharacterCommon/BP_CharacterCommon.ServerExtraReloadOn` (`self.GetCharacterCommon`)))

(event `ServerExtraReloadStart`
  ;[1 1 1] INPUTS FROM SHOOTING CONTROLLER
  ;;[1 1 1] Extra Reload
  (`/Game/CHARACTER_SYSTEM_V2/Blueprints/FirearmSystem/BP_FirearmActorCommon.ServerSetExtraReloadStateOn` (`self.FirearmItemCommon`)))

(event `ClientHandleScopeInOut`
  (params (InScope :type Boolean))
  ;[1 1 1] SCOPE IN / OUT [IRON SIGHT]
  ;;[1 1 1] ClientHandleScopeInOut
  ;;;[1 0.1179 0] BI INPUT FROM CHARACTER
  ;;;[1 0.6824 0] TO FIREARM OWNER STATE HANDLER
  (`/Game/CHARACTER_SYSTEM_V2/Blueprints/FirearmSystem/AC_FirearmOwnerStateHandler.ClientHandleScopeOnOff` (`self.GetFirearmOwnerStateHandler`) InScope)
  ;;;[1 0.6824 0] TO FIREARM VFX CONTROLLER
  (`/Game/CHARACTER_SYSTEM_V2/Blueprints/FirearmSystem/AC_FirearmVFXController.ClientHandleScopeInOut` (`self.GetFirearmVFXController`) InScope)
  ;;;[1 0.6824 0] TO FIREARM SCOPE CONTROLLER
  (`/Game/CHARACTER_SYSTEM_V2/Blueprints/FirearmSystem/AC_FirearmScopeController.ClientHandleScopeInOut` (`self.GetFirearmScopeController`) InScope))

(event `ClientExtraReloadFinish`
  ;[1 1 1] INPUTS FROM SHOOTING CONTROLLER
  ;;[1 1 1] Extra Reload
  ;;;[1 0.1179 0] INPUT FROM SHOOTING CONTROLLER
  (`self.ClientFirearmEvent` "NewEnumerator10")
  (`self.ServerExtraReloadFinish`)
  ;;;[1 0.6824 0] TO CHARACTER COMMON
  (`/Game/CHARACTER_SYSTEM_V2/Blueprints/CharacterCommon/BP_CharacterCommon.ServerExtraReloadOff` (`self.GetCharacterCommon`)))

(event `ServerExtraReloadFinish`
  ;[1 1 1] INPUTS FROM SHOOTING CONTROLLER
  ;;[1 1 1] Extra Reload
  (`/Game/CHARACTER_SYSTEM_V2/Blueprints/FirearmSystem/BP_FirearmActorCommon.ServerSetExtraReloadStateOff` (`self.FirearmItemCommon`)))

(event `ClientExtraReloadCanceled`
  ;[1 1 1] INPUTS FROM SHOOTING CONTROLLER
  ;;[1 1 1] Extra Reload
  ;;;[1 0.1179 0] INPUT FROM SHOOTING CONTROLLER
)

(event `ClientHandleScopeOnOff`
  (params (ScopeOn :type Boolean))
  ;[1 1 1] SCOPE IN / OUT [IRON SIGHT]
  ;;[1 1 1] ClientHandleScopeOnOff
  ;;;[1 0.1179 0] INPUT FROM SCOPE CONTROLLER
  ;;;[1 0.6824 0] TO CHARACTER COMMON
  (`/Game/CHARACTER_SYSTEM_V2/Blueprints/CharacterCommon/BP_CharacterCommon.ClientHandleScopeOnOff` (`self.GetCharacterCommon`) ScopeOn))

(event `ClientHandleAnimEventReloadAction`
  (params (Index :type Integer))
  ;[1 1 1] INPUT ON HANDLE RELOAD ANIM EVENT
  ;;[1 0.1179 0] INPUT FROM ABP CHARACTER BASE
  (`/Game/CHARACTER_SYSTEM_V2/Blueprints/FirearmSystem/AC_FirearmSoundController.ClientHandleAnimEventReloadAction` (`self.GetFirearmSoundController`) Index))

(event `ClientHandleShellOnExtraReload`
  ;[1 1 1] INPUT ON HANDLE RELOAD ANIM EVENT
  ;;[1 0.1179 0] INPUT FROM ABP CHARACTER BASE
  (`/Game/CHARACTER_SYSTEM_V2/Blueprints/FirearmSystem/AC_FirearmSoundController.ClientHandleAnimEventReloadAction` (`self.GetFirearmSoundController`) 0))

(event `ClientUpdateOwnerInfluencesIterated`
  ;[1 1 1] INPUT FROM OWNER STATE HANDLER
  ;;[1 0.1179 0] INPUT FROM OWNER STATE HANDLER
  (`/Game/CHARACTER_SYSTEM_V2/Blueprints/FirearmSystem/AC_FirearmSpreadController.ClientHandleUpdateSpreadInfOnIteratationStep` (`self.GetFirearmSpreadController`))
  (`/Game/CHARACTER_SYSTEM_V2/Blueprints/FirearmSystem/AC_FirearmRecoilController.ClientHandleInfRecoilInterated` (`self.GetFirearmRecoilController`))
  (`/Game/CHARACTER_SYSTEM_V2/Blueprints/FirearmSystem/AC_FirearmCameraShakeController.ClientHandleInteratedCharacterInfluence` (`self.GetFirearmCameraShakeController`)))

(event `ClientOwnerStateUpdated`
  ;[1 1 1] INPUT FROM OWNER STATE HANDLER
  ;;[1 0.1179 0] INPUT FROM OWNER STATE HANDLER
)

(fn `GetCharacterCommon`
  (returns (CharacterCommon :type "/Game/CHARACTER_SYSTEM_V2/Blueprints/CharacterCommon/BP_CharacterCommon Object Reference"))
  (`/Engine/EditorBlueprintResources/StandardMacros.IsValid` (`self.GetOwner` self)
    (:`Is Valid`
      (bind _asbp_character_common (cast `/Game/CHARACTER_SYSTEM_V2/Blueprints/CharacterCommon/BP_CharacterCommon` (`self.GetOwner` self)))
      (return _asbp_character_common))))

(fn `GetFirearmCameraShakeController`
  (returns (FirearmCameraShakeController :type "/Game/CHARACTER_SYSTEM_V2/Blueprints/FirearmSystem/AC_FirearmCameraShakeController Object Reference"))
  (bind _returnvalue (`Actor.GetComponentByClass` (`self.GetOwner` self) "/Game/CHARACTER_SYSTEM_V2/Blueprints/FirearmSystem/AC_FirearmCameraShakeController.AC_FirearmCameraShakeController_C"))
  (`/Engine/EditorBlueprintResources/StandardMacros.IsValid` _returnvalue
    (:`Is Valid`
      (return _returnvalue))))

(fn `GetFirearmDamageHandler`
  (returns (FirearmDamageHandler :type "/Game/CHARACTER_SYSTEM_V2/Blueprints/FirearmSystem/AC_FirearmDamageHandler Object Reference"))
  (bind _returnvalue (`Actor.GetComponentByClass` (`self.GetOwner` self) "/Game/CHARACTER_SYSTEM_V2/Blueprints/FirearmSystem/AC_FirearmDamageHandler.AC_FirearmDamageHandler_C"))
  (`/Engine/EditorBlueprintResources/StandardMacros.IsValid` _returnvalue
    (:`Is Valid`
      (return _returnvalue))))

(fn `GetFirearmHitScan`
  (returns (FirearmHitScan :type "/Game/CHARACTER_SYSTEM_V2/Blueprints/FirearmSystem/AC_FirearmHitScan Object Reference"))
  (bind _returnvalue (`Actor.GetComponentByClass` (`self.GetOwner` self) "/Game/CHARACTER_SYSTEM_V2/Blueprints/FirearmSystem/AC_FirearmHitScan.AC_FirearmHitScan_C"))
  (`/Engine/EditorBlueprintResources/StandardMacros.IsValid` _returnvalue
    (:`Is Valid`
      (return _returnvalue))))

(fn `GetFirearmItemCommon`
  (returns (FirearmItemCommon :type "/Game/CHARACTER_SYSTEM_V2/Blueprints/FirearmSystem/BP_FirearmActorCommon Object Reference"))
  (return (`self.FirearmItemCommon`)))

(fn `GetFirearmLibraryDesc`
  (returns (FirearmLibDesc :type "/Game/CHARACTER_SYSTEM_V2/Blueprints/DATA/STR/STR_FL_FirearmLibraryDesc Structure"))
  (bind _returnvalue (`|GetDataTableRow` "/Game/CHARACTER_SYSTEM_V2/Blueprints/FirearmTP/DT_FirearmLibrary.DT_FirearmLibrary" (`self.FirearmTag`))
    (:`then`
      (return _returnvalue))))

(fn `GetFirearmOwnerStateHandler`
  (returns (FirearmOwnerStateHandler :type "/Game/CHARACTER_SYSTEM_V2/Blueprints/FirearmSystem/AC_FirearmOwnerStateHandler Object Reference"))
  (bind _returnvalue (`Actor.GetComponentByClass` (`self.GetOwner` self) "/Game/CHARACTER_SYSTEM_V2/Blueprints/FirearmSystem/AC_FirearmOwnerStateHandler.AC_FirearmOwnerStateHandler_C"))
  (`/Engine/EditorBlueprintResources/StandardMacros.IsValid` _returnvalue
    (:`Is Valid`
      (return _returnvalue))))

(fn `GetFirearmRecoilController`
  (returns (FirearmRecoilController :type "/Game/CHARACTER_SYSTEM_V2/Blueprints/FirearmSystem/AC_FirearmRecoilController Object Reference"))
  (bind _returnvalue (`Actor.GetComponentByClass` (`self.GetOwner` self) "/Game/CHARACTER_SYSTEM_V2/Blueprints/FirearmSystem/AC_FirearmRecoilController.AC_FirearmRecoilController_C"))
  (`/Engine/EditorBlueprintResources/StandardMacros.IsValid` _returnvalue
    (:`Is Valid`
      (return _returnvalue))))

(fn `GetFirearmScopeController`
  (returns (FirearmScopeController :type "/Game/CHARACTER_SYSTEM_V2/Blueprints/FirearmSystem/AC_FirearmScopeController Object Reference"))
  (bind _returnvalue (`Actor.GetComponentByClass` (`self.GetOwner` self) "/Game/CHARACTER_SYSTEM_V2/Blueprints/FirearmSystem/AC_FirearmScopeController.AC_FirearmScopeController_C"))
  (`/Engine/EditorBlueprintResources/StandardMacros.IsValid` _returnvalue
    (:`Is Valid`
      (return _returnvalue))))

(fn `GetFirearmShootingController`
  (returns (FirearmShootingController :type "/Game/CHARACTER_SYSTEM_V2/Blueprints/FirearmSystem/AC_FirearmShootingController Object Reference"))
  (bind _returnvalue (`Actor.GetComponentByClass` (`self.GetOwner` self) "/Game/CHARACTER_SYSTEM_V2/Blueprints/FirearmSystem/AC_FirearmShootingController.AC_FirearmShootingController_C"))
  (`/Engine/EditorBlueprintResources/StandardMacros.IsValid` _returnvalue
    (:`Is Valid`
      (return _returnvalue))))

(fn `GetFirearmSoundController`
  (returns (FirearmSoundController :type "/Game/CHARACTER_SYSTEM_V2/Blueprints/FirearmSystem/AC_FirearmSoundController Object Reference"))
  (bind _returnvalue (`Actor.GetComponentByClass` (`self.GetOwner` self) "/Game/CHARACTER_SYSTEM_V2/Blueprints/FirearmSystem/AC_FirearmSoundController.AC_FirearmSoundController_C"))
  (`/Engine/EditorBlueprintResources/StandardMacros.IsValid` _returnvalue
    (:`Is Valid`
      (return _returnvalue))))

(fn `GetFirearmSpreadController`
  (returns (FirearmSpreadController :type "/Game/CHARACTER_SYSTEM_V2/Blueprints/FirearmSystem/AC_FirearmSpreadController Object Reference"))
  (bind _returnvalue (`Actor.GetComponentByClass` (`self.GetOwner` self) "/Game/CHARACTER_SYSTEM_V2/Blueprints/FirearmSystem/AC_FirearmSpreadController.AC_FirearmSpreadController_C"))
  (`/Engine/EditorBlueprintResources/StandardMacros.IsValid` _returnvalue
    (:`Is Valid`
      (return _returnvalue))))

(fn `GetFirearmVFXController`
  (returns (FirearmVFXController :type "/Game/CHARACTER_SYSTEM_V2/Blueprints/FirearmSystem/AC_FirearmVFXController Object Reference"))
  (bind _returnvalue (`Actor.GetComponentByClass` (`self.GetOwner` self) "/Game/CHARACTER_SYSTEM_V2/Blueprints/FirearmSystem/AC_FirearmVFXController.AC_FirearmVFXController_C"))
  (`/Engine/EditorBlueprintResources/StandardMacros.IsValid` _returnvalue
    (:`Is Valid`
      (return _returnvalue))))