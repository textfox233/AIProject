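; Client-side firearm component that turns fire input from AC_FirearmSystem into timed shots and reloads, reporting each phase back to it.
; Supports automatic, semi, burst, bolt-action and single-shot modes using weapon library data and inventory ammo.
; Shots run on timers and delays, with "dense compensation" buffering late-window presses for semi and burst fire.
; Main, extra (bolt-cycle) and cyclic reloads use retriggerable delays behind gates that cancellation closes.
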(event `ClientSetBlockAnyAction`
  (params (InBlockAnyAction :type Boolean))
  ;[1 1 1] HANDLE INPUT RELEASED  & OTHERS
  ;;[1 0.1179 0] INPUT FROM FIREARM SYSTEM
  (bind _output_get (set `self.InBlockAnyAction` InBlockAnyAction))
  (if _output_get
    (`self.ClientCancelMainReload`)
    (`self.ClientCancelExtraReload`)
    (`self.ClientCancelCyclicMainReload`)))

(event `ClientShootReleased`
  ;[1 1 1] HANDLE INPUT RELEASED  & OTHERS
  ;;[1 0.1179 0] INPUT FROM FIREARM SYSTEM
  (set `self.InputFireHold` false)
  (switch `/Game/CHARACTER_SYSTEM_V2/Blueprints/DATA/E/E_GL_FirearmFiringMode` (`self.GetFiringMode`)
    (:`NewEnumerator0`
      (`KismetSystemLibrary.K2_ClearTimer` null "ClientCreateShot"))))

(event `ClientShootPressed`
  (bind _firing_mode (`self.GetFiringMode`))
  ;[1 1 1] HANDLE INPUT PRESSED
  ;;[1 0.1179 0] INPUT FROM FIREARM SYSTEM
  ;;[0 1 0.2254] InputFireHold = True
  (set `self.InputFireHold` true)
  ;;[0 0.3159 1] CONDITION: InMainReload = true or InExtraReload = true
  (if (or (`self.InMainReload`) (`self.InExtraReload`))
    ;;[0 0.3159 1] CONDITION: GetCyclicMainReload = True and InMainReload = true
    (if (and (`self.GetCyclicMainReload`) (`self.InMainReload`))
      ;;[0 1 0.2254] RequestForCancelCyclicMainReload = true
      (set `self.RequestForCancelCyclicMainReload` true))
    (else
      ;;[0 0.3159 1] CONDITION: GetCurrentClipSize = 0
      (if (== (`self.GetCurrentClipSize`) 0)
        ;;[0 0.3159 1] CONDITION: GetCurrentAmmoPull = 0
        (if (== (`self.GetCurrentAmmoPull`) 0)
          ;;[1 0 0.008047] TRIGGER: ClientFirearmsAmmoEmpty
          (`self.ClientFirearmsAmmoEmpty`)
          (else
            ;;[1 0 0.008047] TRIGGER: ClientRequestedMainReload
            (`self.ClientRequestedMainReload`)))
        (else
          ;;[0 0.3159 1] CONDITION: WaitShotDelay = true
          (if (`self.WaitShotDelay`)
            ;;[0 0.3159 1] CONDITION: GetFiringMode = Burst or GetFiringMode = Semi
            (if (or (`|EnumEquality` _firing_mode "NewEnumerator2") (`|EnumEquality` _firing_mode "NewEnumerator1"))
              ;;[0 0.3159 1] CONDITION: CanUseDenseComp = true
              (if (`self.CanUseDenseComp`)
                ;;[0 1 0.2254] DenseCompInputStoring = true
                (set `self.DenseCompInputStoring` true)))
            (else
              ;;[0 0.3159 1] CONDITION: FiringMode
              (switch `/Game/CHARACTER_SYSTEM_V2/Blueprints/DATA/E/E_GL_FirearmFiringMode` (`self.GetFiringMode`)
                (:`NewEnumerator0`
                  ;;[1 0 0.008047] TRIGGER: ClientCreateShot
                  (`self.ClientCreateShot` :!label _label)
                  ;;[1 0 0.008047] TRIGGER TIMER: ClientCreateShot
                  (`KismetSystemLibrary.K2_SetTimer` null "ClientCreateShot" (`self.GetShotDelay`) true))
                (:`NewEnumerator1`
                  ;;[1 0 0.008047] TRIGGER: ClientCreateShot
                  (`self.ClientCreateShot` :!label _label_2))
                (:`NewEnumerator2`
                  (goto _label))
                (:`NewEnumerator3`
                  (goto _label_2))
                (:`NewEnumerator4`
                  (goto _label_2))))))))))

(event `ClientCreateShot`
  (bind _firing_mode (`self.GetFiringMode`))
  ;[1 1 1] CREATE SHOT
  ;;[0.2033 0.3085 1] LOCAL INPUT
  ;;[0 0.3159 1] CONDITION: GetCurrentClipSize = 0
  (if (== (`self.GetCurrentClipSize`) 0)
    ;;[0 0.3159 1] CONDITION: GetCurrentAmmoPull = 0
    (if (== (`self.GetCurrentAmmoPull`) 0)
      ;;[1 0 0.008047] TRIGGER: ClientFirearmsAmmoEmpty
      (`self.ClientFirearmsAmmoEmpty`)
      (else
        ;;[0 0.3159 1] CONDITION: FiringMode = Single
        (if (not (`|EnumEquality` (`self.GetFiringMode`) "NewEnumerator4"))
          ;;[1 0 0.008047] TRIGGER: ClientRequestedMainReload
          (`self.ClientRequestedMainReload`))))
    (else
      ;;[0 0.3159 1] CONDITION: FiringMode = Burst
      (if (`|EnumEquality` (`self.GetFiringMode`) "NewEnumerator2")
        ;;[0 1 0.2254] WaitShotDelay = true
        (set `self.WaitShotDelay` true)
        ;;[0 0.3159 1] CONDITION: GetBurstFireShotsBeforePause = CurrentBurstFireShootsCount
        (if (== (`self.GetBurstFireShotsBeforePause`) (`self.CurrentBurstFireShootsCount`))
          ;;[1 1 1] ClearTimer: ClientCreateShot
          (`KismetSystemLibrary.K2_ClearTimer` null "ClientCreateShot")
          ;;[0 1 0.2254] CurrentBurstFireShootsCount = 0
          (set `self.CurrentBurstFireShootsCount` 0)
          ;;[0 0.3159 1] SEQUENCE
          (`|ExecutionSequence`
            (:`then_0`
              ;;[0.1778 0 1] DELAY: GetBurstFirePause
              (`KismetSystemLibrary.Delay` (`self.GetBurstFirePause`))
              ;;[0 1 0.2254] WaitShotDelay = false & CanUseDenseComp = false
              (set `self.WaitShotDelay` false)
              (set `self.CanUseDenseComp` false)
              ;;[1 1 1] End shot logic
              ;;;[1 1 1] Check request for main reload
              (if (`self.RequestForMainReload`) :!label _label_3
                (set `self.RequestForMainReload` false)
                (`self.ClientRequestedMainReload`)
                (else
                  ;;;[1 1 1] Check clip == 0
                  (if (== (`self.GetCurrentClipSize`) 0)
                    (`self.ClientRequestedMainReload`)
                    (else
                      ;;;[1 1 1] Check bolt-action or single- shot firearm. Desce compensation work ONLY for semi, auto (if low fire rate) or for burs firearm types
                      (if (not (or (`|EnumEquality` _firing_mode "NewEnumerator3") (`|EnumEquality` _firing_mode "NewEnumerator4")))
                        ;;;[1 1 1] Handle DenseComp after shot delay
                        (if (`self.DenseCompInputStoring`)
                          (`self.ClientShootPressed`)
                          (set `self.DenseCompInputStoring` false))))))))
            (:`then_1`
              ;;[0.1778 0 1] DELAY: GetDenseCompensation * GetBurstFirePause
              (`KismetSystemLibrary.Delay` (* (`self.GetDenseCompensation`) (`self.GetBurstFirePause`)))
              ;;[0 1 0.2254] CanUseDenseComp = true
              (set `self.CanUseDenseComp` true)))
          (else
            ;;[1 0 0.008047] TRIGGER: ClientShotHappened
            (`self.ClientShotHappened`)
            ;;[0 1 0.2254] CurrentBurstFireShootsCount + 1
            (`/Engine/EditorBlueprintResources/StandardMacros.IncrementInt` (`self.CurrentBurstFireShootsCount`)
              (:`  `
                ;;[0.1778 0 1] DELAY: GetShotDelay
                (`KismetSystemLibrary.Delay` (`self.GetShotDelay`))
                ;;[1 0 0.008047] TRIGGER: ClientShotDelayEnded
                (`self.ClientShotDelayEnded`)))))
        (else
          ;;[0 1 0.2254] WaitShotDelay = true
          (set `self.WaitShotDelay` true)
          ;;[1 0 0.008047] TRIGGER: ClientShotHappened
          (`self.ClientShotHappened`)
          ;;[0 0.3159 1] SEQUENCE
          (`|ExecutionSequence`
            (:`then_0`
              (`|ExecutionSequence`
                (:`then_0`
                  (`KismetSystemLibrary.Delay` (`self.GetShotDelay`))
                  (set `self.WaitShotDelay` false)
                  (set `self.CanUseDenseComp` false)
                  ;;[1 0 0.008047] TRIGGER: ClientShotDelayEnded
                  (`self.ClientShotDelayEnded`)
                  (goto _label_3))
                (:`then_1`
                  (if (`|EnumEquality` (`self.GetFiringMode`) "NewEnumerator1")
                    ;;[1 1 1] Calculation time in shot delay period when dense compensation windows is closed
                    (`KismetSystemLibrary.Delay` (* (`self.GetDenseCompensation`) (`self.GetShotDelay`)))
                    (set `self.CanUseDenseComp` true)))))
            (:`then_1`
              ;;[0 0.3159 1] CONDITION: FiringMode
              (switch `/Game/CHARACTER_SYSTEM_V2/Blueprints/DATA/E/E_GL_FirearmFiringMode` (`self.GetFiringMode`)
                (:`NewEnumerator3`
                  ;;[0.1778 0 1] DELAY: GetShotTimePart
                  (`KismetSystemLibrary.Delay` (`self.GetShotTimePart`))
                  ;;[1 1 1] Check clip == 0
                  (if (== (`self.GetCurrentClipSize`) 0)
                    (`self.ClientRequestedMainReload`)
                    (else
                      (`self.ClientRequestedExtraReload`))))
                (:`NewEnumerator4`
                  ;;[1 1 1] Handle triggering main reload request after shot by single-shot firearm
                  (`KismetSystemLibrary.Delay` (`self.GetShotTimePart`))
                  (`self.ClientRequestedMainReload`))))))))))

(event `ClientShotHappened`
  ;[1 1 1] OUTPUTS & RELOAD
  ;;[1 1 1] Shot & Ammo is empty
  ;;;[0.9739 1 0] BI OUTPUT TO FirearmSystem
  (`/Game/CHARACTER_SYSTEM_V2/Blueprints/FirearmSystem/AC_FirearmSystem.ClientShotHappened` (`self.GetFirearmSystem`)))

(event `ClientFirearmsAmmoEmpty`
  ;[1 1 1] OUTPUTS & RELOAD
  ;;[1 1 1] Shot & Ammo is empty
  (`KismetSystemLibrary.K2_ClearTimer` null "ClientCreateShot")
  ;;;[0.9739 1 0] BI OUTPUT TO FirearmSystem
  (`/Game/CHARACTER_SYSTEM_V2/Blueprints/FirearmSystem/AC_FirearmSystem.ClientFirearmsAmmoEmpty` (`self.GetFirearmSystem`)))

(event `ClientShotDelayEnded`
  ;[1 1 1] OUTPUTS & RELOAD
  ;;[1 1 1] Shot & Ammo is empty
  ;;;[0.9739 1 0] BI OUTPUT TO FirearmSystem
  (`/Game/CHARACTER_SYSTEM_V2/Blueprints/FirearmSystem/AC_FirearmSystem.ClientShotDelayEnded` (`self.GetFirearmSystem`)))

(event `ClientRequestedMainReload`
  ;[1 1 1] OUTPUTS & RELOAD
  ;;[1 1 1] Main Reload
  ;;;[1 0.1179 0] INPUT FROM FIREARM SYSTEM
  (`/Engine/EditorBlueprintResources/StandardMacros.DoOnce` false :!label _label_4
    (:`Completed`
      (`KismetSystemLibrary.Delay` 0.2)
      (`self.ClientResetGateMainReload`)
      (if (not (`self.InBlockAnyAction`))
        ;;;[1 1 1] Check clip = full
        (if (not (== (`self.GetClipSize`) (`self.GetCurrentClipSize`)))
          ;;;[1 1 1] Check Extra Reload. If 1, Main reload cancels extra reload
          (if (not (`self.InExtraReload`))
            ;;;[1 1 1] Main reload conditions
            (if (and (not (`self.InMainReload`)) (not (== (`self.GetCurrentAmmoPull`) 0)) (not (`self.InBlockAnyAction`)))
              ;;;[1 1 1] Handle firearm types
              (set `self.DenseCompInputStoring` false)
              (switch `/Game/CHARACTER_SYSTEM_V2/Blueprints/DATA/E/E_GL_FirearmFiringMode` (`self.GetFiringMode`)
                (:`NewEnumerator0`
                  (`KismetSystemLibrary.K2_ClearTimer` null "ClientCreateShot")
                  ;;;[1 1 1] Check CylclicMainReload Principal.
                  (if (`self.GetCyclicMainReload`) :!label _label_5
                    (`self.ClientHandleCyclicMainReload`)
                    (else
                      (set `self.InMainReload` true)
                      ;;;[1 1 1] Main reload delay logic
                      ;;;;[0.9739 1 0] BI OUTPUT TO FirearmSystem
                      (`/Game/CHARACTER_SYSTEM_V2/Blueprints/FirearmSystem/AC_FirearmSystem.ClientMainReloadStart` (`self.GetFirearmSystem`))
                      (`|ExecutionSequence`
                        (:`then_0`
                          (`KismetSystemLibrary.RetriggerableDelay` (`self.GetMainReloadTime`))
                          (`/Engine/EditorBlueprintResources/StandardMacros.Gate` false :!label _label_6
                            (:`Exit`
                              ;;;;[0.9739 1 0] BI OUTPUT TO FirearmSystem
                              (`/Game/CHARACTER_SYSTEM_V2/Blueprints/FirearmSystem/AC_FirearmSystem.ClientMainReloadFinish` (`self.GetFirearmSystem`))
                              (set `self.InMainReload` false)
                              ;;;[1 1 1] Triggers shooting after main reload if input fire is holded
                              (if (`self.InputFireHold`)
                                (`self.ClientShootPressed`)))))
                        (:`then_1`
                          (goto _label_6 :!via `Open`))))))
                (:`NewEnumerator1`
                  (if (`self.WaitShotDelay`) :!label _label_7
                    (set `self.RequestForMainReload` true)
                    (else
                      (goto _label_5))))
                (:`NewEnumerator2`
                  (goto _label_5))
                (:`NewEnumerator3`
                  (goto _label_7))
                (:`NewEnumerator4`
                  (goto _label_7))))))))))

(event `ClientResetGateMainReload`
  ;[1 1 1] OUTPUTS & RELOAD
  ;;[1 1 1] Main Reload
  (goto _label_4 :!via `Reset`))

(event `ClientCancelMainReload`
  ;[1 1 1] OUTPUTS & RELOAD
  ;;[1 1 1] Main Reload
  ;;;[1 1 1] Main reload delay logic
  ;;;;[0.9739 1 0] BI OUTPUT TO FirearmSystem
  (`/Game/CHARACTER_SYSTEM_V2/Blueprints/FirearmSystem/AC_FirearmSystem.ClientMainReloadCanceled` (`self.GetFirearmSystem`))
  (goto _label_6 :!via `Close`))

(event `ClientRequestedExtraReload`
  ;[1 1 1] OUTPUTS & RELOAD
  ;;[1 1 1] Extra Reload
  ;;;[1 0.1179 0] INPUT FROM FIREARM SYSTEM
  (if (not (`self.InBlockAnyAction`))
    (set `self.InExtraReload` true)
    ;;;[0.9739 1 0] BI OUTPUT TO FirearmSystem
    (`/Game/CHARACTER_SYSTEM_V2/Blueprints/FirearmSystem/AC_FirearmSystem.ClientExtraReloadStart` (`self.GetFirearmSystem`))
    ;;;[1 1 1] Extra  reload delay logic
    (`|ExecutionSequence`
      (:`then_0`
        (`KismetSystemLibrary.RetriggerableDelay` (- (`self.GetShotDelay`) (`self.GetShotTimePart`)))
        (`/Engine/EditorBlueprintResources/StandardMacros.Gate` false :!label _label_8
          (:`Exit`
            ;;;;[0.9739 1 0] BI OUTPUT TO FirearmSystem
            (`/Game/CHARACTER_SYSTEM_V2/Blueprints/FirearmSystem/AC_FirearmSystem.ClientExtraReloadFinish` (`self.GetFirearmSystem`))
            (set `self.InExtraReload` false))))
      (:`then_1`
        (goto _label_8 :!via `Open`)))))

(event `ClientCancelExtraReload`
  ;[1 1 1] OUTPUTS & RELOAD
  ;;[1 1 1] Extra Reload
  ;;;[1 1 1] Extra  reload delay logic
  ;;;;[0.9739 1 0] BI OUTPUT TO FirearmSystem
  (`/Game/CHARACTER_SYSTEM_V2/Blueprints/FirearmSystem/AC_FirearmSystem.ClientExtraReloadCanceled` (`self.GetFirearmSystem`))
  (goto _label_8 :!via `Close`))

(event `ClientHandleCyclicMainReload`
  ;[1 1 1] OUTPUTS & RELOAD
  ;;[1 1 1] Cyclic Main Reload
  (set `self.InMainReload` true)
  ;;;[1 1 1] Starting
  ;;;;[0.9739 1 0] BI OUTPUT TO FirearmSystem
  (`/Game/CHARACTER_SYSTEM_V2/Blueprints/FirearmSystem/AC_FirearmSystem.ClientMainReloadCyclicStartToPos` (`self.GetFirearmSystem`))
  (`|ExecutionSequence`
    (:`then_0`
      (`KismetSystemLibrary.RetriggerableDelay` (`self.GetCyclicMainReloadStartingTime`))
      (`/Engine/EditorBlueprintResources/StandardMacros.Gate` false :!label _label_9
        (:`Exit`
          ;;;[1 1 1] Cyclic Main reload time
          ;;;;[0.9739 1 0] BI OUTPUT TO FirearmSystem
          (`/Game/CHARACTER_SYSTEM_V2/Blueprints/FirearmSystem/AC_FirearmSystem.ClientMainReloadCyclicStart` (`self.GetFirearmSystem`) :!label _label_10)
          (`|ExecutionSequence`
            (:`then_0`
              (`KismetSystemLibrary.RetriggerableDelay` (`self.GetMainReloadTime`))
              (`/Engine/EditorBlueprintResources/StandardMacros.Gate` false :!label _label_11
                (:`Exit`
                  ;;;;[0.9739 1 0] BI OUTPUT TO FirearmSystem
                  (`/Game/CHARACTER_SYSTEM_V2/Blueprints/FirearmSystem/AC_FirearmSystem.ClientMainReloadCyclicStop` (`self.GetFirearmSystem`))
                  ;;;[1 1 1] Check condition to finish cyclic main reload
                  (if (== (`self.GetCurrentClipSize`) (`self.GetClipSize`))
                    ;;;[1 1 1] Transfer to default pos
                    ;;;;[0.9739 1 0] BI OUTPUT TO FirearmSystem
                    (`/Game/CHARACTER_SYSTEM_V2/Blueprints/FirearmSystem/AC_FirearmSystem.ClientMainReloadCyclicEndToPos` (`self.GetFirearmSystem`) :!label _label_12)
                    (`|ExecutionSequence`
                      (:`then_0`
                        (`KismetSystemLibrary.RetriggerableDelay` (`self.GetCyclicMainReloadEndingTime`))
                        (`/Engine/EditorBlueprintResources/StandardMacros.Gate` false :!label _label_13
                          (:`Exit`
                            ;;;;[0.9739 1 0] BI OUTPUT TO FirearmSystem
                            (`/Game/CHARACTER_SYSTEM_V2/Blueprints/FirearmSystem/AC_FirearmSystem.ClientMainReloadStart` (`self.GetFirearmSystem`))
                            (set `self.InMainReload` false))))
                      (:`then_1`
                        (goto _label_13 :!via `Open`)))
                    (else
                      ;;;[1 1 1] Check Input storing in main reload state by input pressed
                      (if (`self.RequestForCancelCyclicMainReload`)
                        (set `self.RequestForCancelCyclicMainReload` false)
                        (goto _label_12)
                        (else
                          (`self.ClientTriggerNewCyclicMainReload`))))))))
            (:`then_1`
              (goto _label_11 :!via `Open`))))))
    (:`then_1`
      (goto _label_9 :!via `Open`))))

(event `ClientTriggerNewCyclicMainReload`
  ;[1 1 1] OUTPUTS & RELOAD
  ;;[1 1 1] Cyclic Main Reload
  ;;;[1 1 1] Cyclic Main reload time
  (goto _label_10))

(event `ClientCancelCyclicMainReload`
  ;[1 1 1] OUTPUTS & RELOAD
  ;;[1 1 1] Cyclic Main Reload
  ;;;[1 1 1] Starting
  ;;;;[0.9739 1 0] BI OUTPUT TO FirearmSystem
  (`/Game/CHARACTER_SYSTEM_V2/Blueprints/FirearmSystem/AC_FirearmSystem.ClientMainReloadCanceled` (`self.GetFirearmSystem`))
  (`|ExecutionSequence`
    (:`then_0`
      (goto _label_9 :!via `Close`))
    (:`then_1`
      ;;;[1 1 1] Cyclic Main reload time
      ;;;;[0.9739 1 0] BI OUTPUT TO FirearmSystem
      (`/Game/CHARACTER_SYSTEM_V2/Blueprints/FirearmSystem/AC_FirearmSystem.ClientMainReloadCanceled` (`self.GetFirearmSystem`))
      (`|ExecutionSequence`
        (:`then_0`
          (goto _label_11 :!via `Close`))
        (:`then_1`
          ;;;[1 1 1] Transfer to default pos
          ;;;;[0.9739 1 0] BI OUTPUT TO FirearmSystem
          (`/Game/CHARACTER_SYSTEM_V2/Blueprints/FirearmSystem/AC_FirearmSystem.ClientMainReloadCanceled` (`self.GetFirearmSystem`))
          (goto _label_13 :!via `Close`))))))

(fn `GetBurstFirePause`
  (returns (`Burst Fire Pause` :type "Float (double-precision)"))
  (return (`.BurstFirePause_14_2DAB4AF94B87AAE531EC65AC66AEE5F8` (break `/Game/CHARACTER_SYSTEM_V2/Blueprints/DATA/STR/STR_FL_FirearmLibraryShootDesc` (`.Shoot_18_65E9D0144E92C7449C62968586480AD6` (break `/Game/CHARACTER_SYSTEM_V2/Blueprints/DATA/STR/STR_FL_FirearmLibraryDesc` (`/Game/CHARACTER_SYSTEM_V2/Blueprints/FirearmSystem/AC_FirearmSystem.GetFirearmLibraryDesc` (`self.GetFirearmSystem`))))))))

(fn `GetBurstFireShotsBeforePause`
  (returns (`Burst Fire Shots Before Pause` :type Integer))
  (return (`.BurstFireShotsBeforePause_11_B8C8CFC546C76B61E822088D0D15C689` (break `/Game/CHARACTER_SYSTEM_V2/Blueprints/DATA/STR/STR_FL_FirearmLibraryShootDesc` (`.Shoot_18_65E9D0144E92C7449C62968586480AD6` (break `/Game/CHARACTER_SYSTEM_V2/Blueprints/DATA/STR/STR_FL_FirearmLibraryDesc` (`/Game/CHARACTER_SYSTEM_V2/Blueprints/FirearmSystem/AC_FirearmSystem.GetFirearmLibraryDesc` (`self.GetFirearmSystem`))))))))

(fn `GetClipSize`
  (returns (ClipSize :type Integer))
  (return (`.MagazinSize_5_6D00165A43D81D5CEB72B483C72957EB` (break `/Game/CHARACTER_SYSTEM_V2/Blueprints/DATA/STR/STR_FL_FirearmLibraryAmmoDesc` (`.AmmoClip_11_4295B10E4993B4A5AED7F4AFCF05742F` (break `/Game/CHARACTER_SYSTEM_V2/Blueprints/DATA/STR/STR_FL_FirearmLibraryDesc` (`/Game/CHARACTER_SYSTEM_V2/Blueprints/FirearmSystem/AC_FirearmSystem.GetFirearmLibraryDesc` (`self.GetFirearmSystem`))))))))

(fn `GetCurrentAmmoPull`
  (returns (CurrentAmmoPull :type Integer))
  (locals (loc_ammo_type :type "/Game/CHARACTER_SYSTEM_V2/Blueprints/DATA/E/E_FirearmAmmoType Enum") (loc_ammo_res_current :type Integer :default 0) (loc_res_type :type "/Game/CHARACTER_SYSTEM_V2/Blueprints/DATA/E/Inventory/E_ResourceType Enum") (loc_spet_ammo :type Integer))
  (set `local.loc_ammo_type` (`.AmmoType_8_DEB67CD040AC5D3A9810B6918756DE73` (break `/Game/CHARACTER_SYSTEM_V2/Blueprints/DATA/STR/STR_FL_FirearmLibraryAmmoDesc` (`.AmmoClip_11_4295B10E4993B4A5AED7F4AFCF05742F` (break `/Game/CHARACTER_SYSTEM_V2/Blueprints/DATA/STR/STR_FL_FirearmLibraryDesc` (`/Game/CHARACTER_SYSTEM_V2/Blueprints/FirearmSystem/AC_FirearmSystem.GetFirearmLibraryDesc` (`self.GetFirearmSystem`)))))))
  (for _array_element (`/Game/CHARACTER_SYSTEM_V2/Blueprints/InventorySystem/AC_InventorySystem.GetInventoryResources` (`self.GetInventorySystem`))
    (bind (_resourcetype _amount) (break `/Game/CHARACTER_SYSTEM_V2/Blueprints/DATA/STR/STR_GL_InventoryResourceDesc` _array_element))
    (if (and (`|EnumEquality` _resourcetype (select `/Game/CHARACTER_SYSTEM_V2/Blueprints/DATA/E/E_FirearmAmmoType` (`local.loc_ammo_type`) :`NewEnumerator0` "NewEnumerator0" :`NewEnumerator1` "NewEnumerator1" :`NewEnumerator2` "NewEnumerator2" :`NewEnumerator3` "NewEnumerator3" :`NewEnumerator4` "NewEnumerator4" :`NewEnumerator5` "NewEnumerator5" :!type "/Game/CHARACTER_SYSTEM_V2/Blueprints/DATA/E/Inventory/E_ResourceType Enum")) (> _amount 0))
      (`/Engine/EditorBlueprintResources/StandardMacros.DoOnce` false
        (:`Completed`
          (set `local.loc_ammo_res_current` _amount)))))
  (return (`local.loc_ammo_res_current`)))

(fn `GetCurrentClipSize`
  (returns (`Clip Size` :type Integer))
  (`/Engine/EditorBlueprintResources/StandardMacros.IsValid` (`/Game/CHARACTER_SYSTEM_V2/Blueprints/FirearmSystem/AC_FirearmSystem.GetFirearmItemCommon` (`self.GetFirearmSystem`))
    (:`Is Valid`
      (return (`/Game/CHARACTER_SYSTEM_V2/Blueprints/FirearmSystem/BP_FirearmActorCommon.GetCurrentAmmoInClip` (`/Game/CHARACTER_SYSTEM_V2/Blueprints/FirearmSystem/AC_FirearmSystem.GetFirearmItemCommon` (`self.GetFirearmSystem`)))))))

(fn `GetCyclicMainReload`
  (returns (`Cyclic Main Reload` :type Boolean))
  (return (`.CyclicMainReload_15_E58FA21E4709F8476AE304B8796EFE4E` (break `/Game/CHARACTER_SYSTEM_V2/Blueprints/DATA/STR/STR_FL_FirearmLibraryCommonDesc` (`.Common_33_E987A8D34646F0BCC18DB4954EA3FE73` (break `/Game/CHARACTER_SYSTEM_V2/Blueprints/DATA/STR/STR_FL_FirearmLibraryDesc` (`/Game/CHARACTER_SYSTEM_V2/Blueprints/FirearmSystem/AC_FirearmSystem.GetFirearmLibraryDesc` (`self.GetFirearmSystem`))))))))

(fn `GetCyclicMainReloadEndingTime`
  (returns (`Cyclic Main Reload Ending Time` :type "Float (double-precision)"))
  (return (`.CyclicMainReloadEndingTime_13_5E0951E04D9946D356AED897DAFFA9C7` (break `/Game/CHARACTER_SYSTEM_V2/Blueprints/DATA/STR/STR_FL_FirearmLibraryActionDesc` (`.Action_24_DE5AE7C74EB74C14A91C7B8E58A8C5D7` (break `/Game/CHARACTER_SYSTEM_V2/Blueprints/DATA/STR/STR_FL_FirearmLibraryDesc` (`/Game/CHARACTER_SYSTEM_V2/Blueprints/FirearmSystem/AC_FirearmSystem.GetFirearmLibraryDesc` (`self.GetFirearmSystem`))))))))

(fn `GetCyclicMainReloadStartingTime`
  (returns (`Cyclic Main Reload Starting Time` :type "Float (double-precision)"))
  (return (`.CyclicMainReloadStartingTime_11_66DAACC94B072C5FD2ECCCAB9854B894` (break `/Game/CHARACTER_SYSTEM_V2/Blueprints/DATA/STR/STR_FL_FirearmLibraryActionDesc` (`.Action_24_DE5AE7C74EB74C14A91C7B8E58A8C5D7` (break `/Game/CHARACTER_SYSTEM_V2/Blueprints/DATA/STR/STR_FL_FirearmLibraryDesc` (`/Game/CHARACTER_SYSTEM_V2/Blueprints/FirearmSystem/AC_FirearmSystem.GetFirearmLibraryDesc` (`self.GetFirearmSystem`))))))))

(fn `GetDenseCompensation`
  (returns (`Dense Compensation` :type "Float (double-precision)"))
  (return (`.DenseCompensation_8_8CF51F9F45197394D64005A54377B135` (break `/Game/CHARACTER_SYSTEM_V2/Blueprints/DATA/STR/STR_FL_FirearmLibraryShootDesc` (`.Shoot_18_65E9D0144E92C7449C62968586480AD6` (break `/Game/CHARACTER_SYSTEM_V2/Blueprints/DATA/STR/STR_FL_FirearmLibraryDesc` (`/Game/CHARACTER_SYSTEM_V2/Blueprints/FirearmSystem/AC_FirearmSystem.GetFirearmLibraryDesc` (`self.GetFirearmSystem`))))))))

(fn `GetFirearmSystem`
  (returns (FirearmSystem :type "/Game/CHARACTER_SYSTEM_V2/Blueprints/FirearmSystem/AC_FirearmSystem Object Reference"))
  (bind _returnvalue (`Actor.GetComponentByClass` (`self.GetOwner` self) "/Game/CHARACTER_SYSTEM_V2/Blueprints/FirearmSystem/AC_FirearmSystem.AC_FirearmSystem_C"))
  (`/Engine/EditorBlueprintResources/StandardMacros.IsValid` _returnvalue
    (:`Is Valid`
      (return _returnvalue))))

(fn `GetFiringMode`
  (returns (`Firing Mode` :type "/Game/CHARACTER_SYSTEM_V2/Blueprints/DATA/E/E_GL_FirearmFiringMode Enum"))
  (return (`.FiringMode_5_E5EF19BC42FD9D9388B2C0A2CEF5A755` (break `/Game/CHARACTER_SYSTEM_V2/Blueprints/DATA/STR/STR_FL_FirearmLibraryShootDesc` (`.Shoot_18_65E9D0144E92C7449C62968586480AD6` (break `/Game/CHARACTER_SYSTEM_V2/Blueprints/DATA/STR/STR_FL_FirearmLibraryDesc` (`/Game/CHARACTER_SYSTEM_V2/Blueprints/FirearmSystem/AC_FirearmSystem.GetFirearmLibraryDesc` (`self.GetFirearmSystem`))))))))

(fn `GetInventorySystem`
  (returns (InventorySystem :type "/Game/CHARACTER_SYSTEM_V2/Blueprints/InventorySystem/AC_InventorySystem Object Reference"))
  (bind _returnvalue (`Actor.GetComponentByClass` (`Controller.K2_GetPawn` (`GameplayStatics.GetPlayerController` 0)) "/Game/CHARACTER_SYSTEM_V2/Blueprints/InventorySystem/AC_InventorySystem.AC_InventorySystem_C"))
  (`/Engine/EditorBlueprintResources/StandardMacros.IsValid` _returnvalue
    (:`Is Valid`
      (return _returnvalue))))

(fn `GetMainReloadTime`
  (returns (`Main Reload Time` :type "Float (double-precision)"))
  (return (`.MainReloadTime_6_9EFCD44C48E22AE5F1D4A784284B98A6` (break `/Game/CHARACTER_SYSTEM_V2/Blueprints/DATA/STR/STR_FL_FirearmLibraryActionDesc` (`.Action_24_DE5AE7C74EB74C14A91C7B8E58A8C5D7` (break `/Game/CHARACTER_SYSTEM_V2/Blueprints/DATA/STR/STR_FL_FirearmLibraryDesc` (`/Game/CHARACTER_SYSTEM_V2/Blueprints/FirearmSystem/AC_FirearmSystem.GetFirearmLibraryDesc` (`self.GetFirearmSystem`))))))))

(fn `GetShotDelay`
  (returns (ShotDelay :type "Float (double-precision)"))
  (return (/ 1.0 (/ (`KismetMathLibrary.Conv_IntToDouble` (`.FireRate_2_52A27DD94EACF209306230AB91D8A62F` (break `/Game/CHARACTER_SYSTEM_V2/Blueprints/DATA/STR/STR_FL_FirearmLibraryShootDesc` (`.Shoot_18_65E9D0144E92C7449C62968586480AD6` (break `/Game/CHARACTER_SYSTEM_V2/Blueprints/DATA/STR/STR_FL_FirearmLibraryDesc` (`/Game/CHARACTER_SYSTEM_V2/Blueprints/FirearmSystem/AC_FirearmSystem.GetFirearmLibraryDesc` (`self.GetFirearmSystem`))))))) 60.0))))

(fn `GetShotTimePart`
  (returns (`Shot Time Part` :type "Float (double-precision)"))
  (return (`.ShotTimePart_17_31A3B65D4441C3BF29B6CAB40492A6FD` (break `/Game/CHARACTER_SYSTEM_V2/Blueprints/DATA/STR/STR_FL_FirearmLibraryShootDesc` (`.Shoot_18_65E9D0144E92C7449C62968586480AD6` (break `/Game/CHARACTER_SYSTEM_V2/Blueprints/DATA/STR/STR_FL_FirearmLibraryDesc` (`/Game/CHARACTER_SYSTEM_V2/Blueprints/FirearmSystem/AC_FirearmSystem.GetFirearmLibraryDesc` (`self.GetFirearmSystem`))))))))