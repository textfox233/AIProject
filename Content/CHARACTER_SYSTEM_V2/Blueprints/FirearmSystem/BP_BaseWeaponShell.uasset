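; Base actor for an ejected weapon shell casing, with physics impulse and a landing sound.
; Multicast events set its mesh and sound properties and apply the impulse as a velocity change.
; Shortly after spawn it plays the fall sound once on hitting a non-character, then destroys itself after a few seconds.
; A client event closes a second gate to silence that sound for the first-person owner.
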(event `self.StaticMesh.OnComponentHit`
  (params (HitComponent :type "PrimitiveComponent Object Reference") (OtherActor :type "Actor Object Reference") (OtherComp :type "PrimitiveComponent Object Reference") (NormalImpulse :type "Vector Structure") (Hit :type "HitResult Structure (by ref)"))
  ;[1 1 1] EVENT BEGIN PLAY & ON HIT (END FALLING - PLAY SOUND)
  (cast `Character` OtherActor
    (:`CastFailed`
      (`/Engine/EditorBlueprintResources/StandardMacros.Gate` true :!label _label
        (:`Exit`
          (`/Engine/EditorBlueprintResources/StandardMacros.DoOnce` false
            (:`Completed`
              (`/Engine/EditorBlueprintResources/StandardMacros.Gate` false :!label _label_2
                (:`Exit`
                  (`GameplayStatics.PlaySoundAtLocation` (`self.FallSound`) (`self.K2_GetActorLocation`) (struct) (`self.VolumeMultiplier`) (`self.PitchMultiplier`) 0.0 null null null null))))))))))

(event `ClientOffSoundesForFPOwner`
  ;[1 1 1] EVENT BEGIN PLAY & ON HIT (END FALLING - PLAY SOUND)
  (goto _label_2 :!via `Close`))

(event `self.ReceiveBeginPlay`
  ;[1 1 1] EVENT BEGIN PLAY & ON HIT (END FALLING - PLAY SOUND)
  (`|ExecutionSequence`
    (:`then_0`
      (`KismetSystemLibrary.Delay` 5.0)
      (`self.K2_DestroyActor`))
    (:`then_1`
      (`KismetSystemLibrary.Delay` 0.2)
      (goto _label :!via `Open`))))

(event `MulticastImpulse`
  (params (Impulse :type "Vector Structure"))
  ;[1 1 1] INITIALIZE ON SPAWN FROM WS
  ;;[1 1 1] MulticastImpulse
  (`PrimitiveComponent.AddImpulse` (`self.StaticMesh`) Impulse "None" true))

(event `MulticastInitializeStaticMesh`
  (params (NewMesh :type "StaticMesh Object Reference"))
  ;[1 1 1] INITIALIZE ON SPAWN FROM WS
  ;;[1 1 1] MulticastInitializeStaticMesh
  (`StaticMeshComponent.SetStaticMesh` (`self.StaticMesh`) NewMesh))

(event `MulticastInitializeSoundProperties`
  (params (FallSound :type "SoundBase Object Reference") (`Volume Multiplier` :type "Float (double-precision)" :default 1.0) (`Pitch Multiplier` :type "Float (double-precision)" :default 1.0))
  ;[1 1 1] INITIALIZE ON SPAWN FROM WS
  ;;[1 1 1] MulticastInitializeSoundProperties
  (set `self.FallSound` FallSound)
  (set `self.VolumeMultiplier` `Volume Multiplier`)
  (set `self.PitchMultiplier` `Pitch Multiplier`))

(fn `UserConstructionScript`)