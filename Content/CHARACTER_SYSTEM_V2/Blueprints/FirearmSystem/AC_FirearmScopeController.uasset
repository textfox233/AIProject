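; Actor component that manages a firearm's scope overlay and aim zoom for the owning character.
; On firearm init it creates a hidden scope widget from AC_FirearmSystem's library data and caches the tagged main camera's FOV, or removes the widget for scopeless firearms.
; Aim events toggle the widget and notify the firearm system.
; Scope-in applies the scope FOV, but scope-out never calls the FOV restore.
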(event `ClientHandleInitFirearm`
  (bind (_ascharacter _bsuccess) (cast `Character` (`self.GetOwner`) :!pure true))
  (bind (_asplayer_controller _bsuccess_2) (cast `PlayerController` (`Pawn.GetController` _ascharacter) :!pure true))
  ;[1 1 1] HADNLE INIT FIREARM
  ;;[1 0.1179 0] INPUT FROM FIREARM SYSTEM
  (if (`self.GetUseScope`)
    ;;[1 1 1] Create Firearm Scope Common Ref if use scope with a current firearm
    (if _bsuccess
      (if _bsuccess_2
        (bind _returnvalue (`|CreateWidget` (`self.GetScoreWidgetClass`) _asplayer_controller))
        (set `self.ScopeWidjet` _returnvalue)
        (`/Engine/EditorBlueprintResources/StandardMacros.IsValid` (`self.ScopeWidjet`)
          (:`Is Valid`
            (`UserWidget.AddToPlayerScreen` (`self.ScopeWidjet`) 5)
            (`Widget.SetVisibility` (`self.ScopeWidjet`) "Hidden")
            ;;[1 1 1] Save Default camera fov for change FOV to this value after out from scope
            (set `self.DefaultCameraFOV` (`CameraComponent.FieldOfView` (`self.GetMainPlayerCameraByTag`)))))))
    (else
      ;;[1 1 1] Remove Scope widjet if inited firearm not use scope
      (`/Engine/EditorBlueprintResources/StandardMacros.IsValid` (`self.ScopeWidjet`)
        (:`Is Valid`
          (`Widget.RemoveFromParent` (`self.ScopeWidjet`)))))))

(event `ClientHandleScopeInOut`
  (params (InScope :type Boolean))
  ;[1 1 1] HADNLE AIM ON / OFF
  ;;[1 1 1] HandleScopeInOut
  ;;;[1 0.1179 0] INPUT FROM FIREARM SYSTEM
  (if InScope
    (if (not (`self.In Scope`))
      (`self.ClientHandleAimON`))
    (elif (`self.In Scope`)
      (`self.ClientHandleAimOFF`))))

(event `ClientHandleAimON`
  ;[1 1 1] HADNLE AIM ON / OFF
  ;;[1 1 1] ClientHandleAimON
  (if (`self.GetUseScope`)
    (set `self.In Scope` true)
    ;;;[1 0.6824 0] TO FIREARM SYSTEM
    (`/Game/CHARACTER_SYSTEM_V2/Blueprints/FirearmSystem/AC_FirearmSystem.ClientHandleScopeOnOff` (`self.GetFirearmSystem`) true)
    (`/Engine/EditorBlueprintResources/StandardMacros.IsValid` (`self.ScopeWidjet`)
      (:`Is Valid`
        (`self.UpdateFOVOnMainCamera` true)
        (`Widget.SetVisibility` (`self.ScopeWidjet`) "Visible")))))

(event `ClientHandleAimOFF`
  ;[1 1 1] HADNLE AIM ON / OFF
  ;;[1 1 1] ClientHandleAimOFF
  (if (`self.GetUseScope`)
    (set `self.In Scope` false)
    ;;;[1 0.6824 0] TO FIREARM SYSTEM
    (`/Game/CHARACTER_SYSTEM_V2/Blueprints/FirearmSystem/AC_FirearmSystem.ClientHandleScopeOnOff` (`self.GetFirearmSystem`) false)
    (`/Engine/EditorBlueprintResources/StandardMacros.IsValid` (`self.ScopeWidjet`)
      (:`Is Valid`
        (`Widget.SetVisibility` (`self.ScopeWidjet`) "Hidden")))))

(fn `DEP_UpdateVisibleCharacterParts`
  (params (HideInScope :type Boolean))
  (if HideInScope
    (for _array_element (`self.GetCharacterMeshesForHideByTag`)
      (`/Engine/EditorBlueprintResources/StandardMacros.IsValid` _array_element
        (:`Is Valid`
          (`SceneComponent.SetHiddenInGame` _array_element true false))))
    (else
      (for _array_element_2 (`self.GetCharacterMeshesForHideByTag`)
        (`/Engine/EditorBlueprintResources/StandardMacros.IsValid` _array_element_2
          (:`Is Valid`
            (`SceneComponent.SetHiddenInGame` _array_element_2 false false)))))))

(fn `GetADSTime`
  (returns (`Aim Down Sight time` :type "Float (double-precision)"))
  (return (`.AimDownSighttime_7_7B91AA3046DAEF80A864E9BF85DB793A` (break `/Game/CHARACTER_SYSTEM_V2/Blueprints/DATA/STR/STR_FL_FirearmLibraryActionDesc` (`.Action_24_DE5AE7C74EB74C14A91C7B8E58A8C5D7` (break `/Game/CHARACTER_SYSTEM_V2/Blueprints/DATA/STR/STR_FL_FirearmLibraryDesc` (`/Game/CHARACTER_SYSTEM_V2/Blueprints/FirearmSystem/AC_FirearmSystem.GetFirearmLibraryDesc` (`self.GetFirearmSystem`))))))))

(fn `GetCharacterMeshesForHideByTag`
  (returns (SkeletalMeshes :type "Array of SkeletalMeshComponent Object Reference"))
  (`/Engine/EditorBlueprintResources/StandardMacros.IsValid` (`self.GetOwner`)
    (:`Is Valid`
      (return (`Actor.GetComponentsByTag` (`self.GetOwner`) "/Script/Engine.SkeletalMeshComponent" (`self.CharacterMeshTag`))))))

(fn `GetFirearmSystem`
  (returns (FirearmSystem :type "/Game/CHARACTER_SYSTEM_V2/Blueprints/FirearmSystem/AC_FirearmSystem Object Reference"))
  (bind _returnvalue (`Actor.GetComponentByClass` (`self.GetOwner` self) "/Game/CHARACTER_SYSTEM_V2/Blueprints/FirearmSystem/AC_FirearmSystem.AC_FirearmSystem_C"))
  (`/Engine/EditorBlueprintResources/StandardMacros.IsValid` _returnvalue
    (:`Is Valid`
      (return _returnvalue))))

(fn `GetFOVDefault`
  (returns (`FOV Default` :type "Float (double-precision)"))
  (return (`.FOVinScope_14_185FC5C04280520F6841C09CD458A864` (break `/Game/CHARACTER_SYSTEM_V2/Blueprints/DATA/STR/STR_FirearmScopeDesc` (`.Scope_68_C85005354340C93D2FECEDAE82C1FC15` (break `/Game/CHARACTER_SYSTEM_V2/Blueprints/DATA/STR/STR_FL_FirearmLibraryDesc` (`/Game/CHARACTER_SYSTEM_V2/Blueprints/FirearmSystem/AC_FirearmSystem.GetFirearmLibraryDesc` (`self.GetFirearmSystem`))))))))

(fn `GetFOVZoomed`
  (returns (`FOV Zoomed` :type "Float (double-precision)"))
  (return (`.FOVinScope_14_185FC5C04280520F6841C09CD458A864` (break `/Game/CHARACTER_SYSTEM_V2/Blueprints/DATA/STR/STR_FirearmScopeDesc` (`.Scope_68_C85005354340C93D2FECEDAE82C1FC15` (break `/Game/CHARACTER_SYSTEM_V2/Blueprints/DATA/STR/STR_FL_FirearmLibraryDesc` (`/Game/CHARACTER_SYSTEM_V2/Blueprints/FirearmSystem/AC_FirearmSystem.GetFirearmLibraryDesc` (`self.GetFirearmSystem`))))))))

(fn `GetInScope`
  (returns (`In Scope` :type Boolean))
  (return (`self.In Scope`)))

(fn `GetMainPlayerCameraByTag`
  (returns (MainCamera :type "CameraComponent Object Reference"))
  (bind _output (`|GetArrayItem` (`Actor.GetComponentsByTag` (`self.GetOwner`) "/Script/Engine.CameraComponent" (`self.MainPlayerCameraTag`))))
  (`/Engine/EditorBlueprintResources/StandardMacros.IsValid` _output
    (:`Is Valid`
      (return _output))))

(fn `GetScoreWidgetClass`
  (returns (`Score Widget Class` :type "UserWidget Class Reference"))
  (return (`.ScoreWidgetClass_2_E3944B4746E51E39F3F03498D0D7ABF6` (break `/Game/CHARACTER_SYSTEM_V2/Blueprints/DATA/STR/STR_FirearmScopeDesc` (`.Scope_68_C85005354340C93D2FECEDAE82C1FC15` (break `/Game/CHARACTER_SYSTEM_V2/Blueprints/DATA/STR/STR_FL_FirearmLibraryDesc` (`/Game/CHARACTER_SYSTEM_V2/Blueprints/FirearmSystem/AC_FirearmSystem.GetFirearmLibraryDesc` (`self.GetFirearmSystem`))))))))

(fn `GetUseScope`
  (returns (`Use Scope` :type Boolean))
  (return (`.UseScope_12_9EA2953140520D41D3F91884DE4CB0D1` (break `/Game/CHARACTER_SYSTEM_V2/Blueprints/DATA/STR/STR_FirearmScopeDesc` (`.Scope_68_C85005354340C93D2FECEDAE82C1FC15` (break `/Game/CHARACTER_SYSTEM_V2/Blueprints/DATA/STR/STR_FL_FirearmLibraryDesc` (`/Game/CHARACTER_SYSTEM_V2/Blueprints/FirearmSystem/AC_FirearmSystem.GetFirearmLibraryDesc` (`self.GetFirearmSystem`))))))))

(fn `UpdateFOVOnMainCamera`
  (params (ScopeOn :type Boolean))
  (if ScopeOn
    (set `CameraComponent.FieldOfView` (`self.GetFOVDefault`) (`self.GetMainPlayerCameraByTag`))
    (else
      (set `CameraComponent.FieldOfView` (`self.DefaultCameraFOV`) (`self.GetMainPlayerCameraByTag`)))))